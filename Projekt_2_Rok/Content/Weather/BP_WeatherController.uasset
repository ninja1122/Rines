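; Weather controller that runs a day/night cycle by rotating the sun, faster at night, and blends between weather presets.
; Optional random weather picks between two types as sun pitch crosses phase thresholds.
; Each tick it interpolates values toward the target preset using day-phase value and speed overrides, with a timed transition multiplier.
; Results drive MPC_Weather, the player pawn's rain particles, sky clouds, fog, skylight and lights.
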(event `self.ReceiveBeginPlay`
  (set `self.RainParticleSystem` (`self.GetComponentByClass` (`GameplayStatics.GetPlayerPawn` 0) "/Script/Engine.ParticleSystemComponent"))
  (bind _params (`self.GetWeatherParamsForType` (`self.StartingWeatherType`)))
  (bind _output_get (set `self.CurrentWeather` _params))
  (set `self.NewWeather` _output_get)
  (`self.SetWeatherParams` (struct))
  (set `self.startSunRotation` (`self.K2_GetActorRotation` (`self.SunLight`))))

(event `self.ReceiveTick`
  (params (DeltaSeconds :type "Float (single-precision)"))
  (`self.UpdateDayPhase` (`GameplayStatics.GetWorldDeltaSeconds`))
  (if (`self.EnableRandomWeather`)
    (`self.RandomWeather`))
  (`self.InterpolateParams`)
  (`self.SetWeatherParams` (`self.CurrentWeather`))
  (set `self.GlobalWeatherTransitionTimeLeft` (- (`self.GlobalWeatherTransitionTimeLeft`) (`GameplayStatics.GetWorldDeltaSeconds`))))

(event `UpdateDayPhase`
  (params (delta :type "Float (double-precision)"))
  (bind _sunlight (`self.SunLight`))
  (bind (_returnvalue_roll _returnvalue_pitch) (`KismetMathLibrary.BreakRotator` (`self.K2_GetActorRotation` _sunlight)))
  (`/Engine/EditorBlueprintResources/StandardMacros.IsValid` _sunlight
    (:`Is Valid`
      (`self.K2_AddActorLocalRotation` _sunlight (`KismetMathLibrary.MakeRotator` 0.0 (* (/ 360.0 (`self.DayLength`)) (* delta (select `/Game/Weather/BP_DayPhase` (`self.DayPhase`) :`NewEnumerator0` 1.0 :`NewEnumerator1` 1.6 :!type "Float (single-precision)")))) false false)
      (set `self.DayPhase` (select `bool` (`KismetMathLibrary.InRange_FloatFloat` _returnvalue_pitch 0.0 100.0) :`false` "NewEnumerator0" :`true` "NewEnumerator1" :!type "/Game/Weather/BP_DayPhase Enum")))))

(event `RandomWeather`
  (bind _sunrotation (`self.sunRotation`))
  (bind _sunlight (`self.SunLight`))
  (bind (_returnvalue_roll _returnvalue_pitch) (`KismetMathLibrary.BreakRotator` (`self.K2_GetActorRotation` _sunlight)))
  (`/Engine/EditorBlueprintResources/StandardMacros.IsValid` _sunlight
    (:`Is Valid`
      (`|ExecutionSequence`
        (:`then_0`
          (set `self.sunRotation` _returnvalue_pitch)
          (switch `int` (`self.RandomPhase`)
            (:`0`
              (if (`KismetMathLibrary.InRange_FloatFloat` _sunrotation -40.0 0.0)
                (set `self.RandomPhase` 1)))
            (:`1`
              (if (`KismetMathLibrary.InRange_FloatFloat` _sunrotation 0.0 100.0)
                (set `self.RandomPhase` 2)))
            (:`2`
              (if (`KismetMathLibrary.InRange_FloatFloat` _sunrotation -40.0 -10.0)
                (set `self.RandomPhase` 3)))
            (:`3`
              (if (`KismetMathLibrary.InRange_FloatFloat` _sunrotation -80.0 -40.0)
                (set `self.RandomPhase` 0)))))
        (:`then_1`
          (if (!= (`self.RandomPhase`) (`self.CurrentRandomPhase`))
            (set `self.CurrentRandomPhase` (`self.RandomPhase`))
            (`self.SetWeatherType` (select `bool` (== (`KismetMathLibrary.RandomInteger` 3) 0) :`false` "NewEnumerator1" :`true` "NewEnumerator0" :!type "/Game/Weather/BP_WeatherType Enum"))))))))

(fn `Editor_SetTime`
  (`self.SetTime` (`self.Editor_Time`)))

(fn `Editor_SetWeatherType`
  (`self.SetWeatherType` (`self.Editor_WeatherType`)))

(fn `GetWeatherParamsForType`
  (params (Type :type "/Game/Weather/BP_WeatherType Enum" :default "NewEnumerator0"))
  (returns (Params :type "/Game/Weather/BP_WeatherPhaseParams Structure"))
  (bind _array (`|MakeArray` (struct) :!type "/Game/Weather/BP_DayPhaseFloat Structure"))
  (bind (_value _returnvalue) (`BlueprintMapLibrary.Map_Find` (`self.WeatherPresets`) Type))
  (`KismetArrayLibrary.Array_Resize` _array (`KismetArrayLibrary.Array_Length` (`self.Lights`)))
  (return (select `bool` _returnvalue :`false` (make `/Game/Weather/BP_WeatherPhaseParams` (struct :`DefaultInterpSpeed` 1.0) (struct :`DefaultInterpSpeed` 1.0) (struct :`DefaultInterpSpeed` 1.0) null _array) :`true` _value)))

(fn `InterpolateParams`
  (bind _currentweather_puddles (break `/Game/Weather/BP_WeatherPhaseParams` (`self.CurrentWeather`)))
  (bind _newweather_puddles (break `/Game/Weather/BP_WeatherPhaseParams` (`self.NewWeather`)))
  (bind (_currentweather_puddles_2 _currentweather_rain) (break `/Game/Weather/BP_WeatherPhaseParams` (`self.CurrentWeather`)))
  (bind (_newweather_puddles_2 _newweather_rain) (break `/Game/Weather/BP_WeatherPhaseParams` (`self.NewWeather`)))
  (bind (_currentweather_puddles_3 _currentweather_rain_2 _currentweather_cloudopacity) (break `/Game/Weather/BP_WeatherPhaseParams` (`self.CurrentWeather`)))
  (bind (_newweather_puddles_3 _newweather_rain_2 _newweather_cloudopacity) (break `/Game/Weather/BP_WeatherPhaseParams` (`self.NewWeather`)))
  (bind (_currentweather_puddles_4 _currentweather_rain_3 _currentweather_cloudopacity_2 _currentweather_cloudcolors _currentweather_lightintensity) (break `/Game/Weather/BP_WeatherPhaseParams` (`self.CurrentWeather`)))
  (bind (_newweather_puddles_4 _newweather_rain_3 _newweather_cloudopacity_2 _newweather_cloudcolors _newweather_lightintensity) (break `/Game/Weather/BP_WeatherPhaseParams` (`self.NewWeather`)))
  (bind (_currentweather_puddles_5 _currentweather_rain_4 _currentweather_cloudopacity_3 _currentweather_cloudcolors_2 _currentweather_lightintensity_2 _currentweather_skylightintensity) (break `/Game/Weather/BP_WeatherPhaseParams` (`self.CurrentWeather`)))
  (bind (_newweather_puddles_5 _newweather_rain_4 _newweather_cloudopacity_3 _newweather_cloudcolors_2 _newweather_lightintensity_2 _newweather_skylightintensity) (break `/Game/Weather/BP_WeatherPhaseParams` (`self.NewWeather`)))
  (bind (_currentweather_puddles_6 _currentweather_rain_5 _currentweather_cloudopacity_4 _currentweather_cloudcolors_3 _currentweather_lightintensity_3 _currentweather_skylightintensity_2 _currentweather_fogmultiplier) (break `/Game/Weather/BP_WeatherPhaseParams` (`self.CurrentWeather`)))
  (bind (_newweather_puddles_6 _newweather_rain_5 _newweather_cloudopacity_4 _newweather_cloudcolors_3 _newweather_lightintensity_3 _newweather_skylightintensity_2 _newweather_fogmultiplier) (break `/Game/Weather/BP_WeatherPhaseParams` (`self.NewWeather`)))
  (bind (_currentweather_puddles_7 _currentweather_rain_6 _currentweather_cloudopacity_5 _currentweather_cloudcolors_4 _currentweather_lightintensity_4 _currentweather_skylightintensity_3 _currentweather_fogmultiplier_2 _currentweather_darkcloudsblend) (break `/Game/Weather/BP_WeatherPhaseParams` (`self.CurrentWeather`)))
  (bind (_newweather_puddles_7 _newweather_rain_6 _newweather_cloudopacity_5 _newweather_cloudcolors_4 _newweather_lightintensity_4 _newweather_skylightintensity_3 _newweather_fogmultiplier_2 _newweather_darkcloudsblend) (break `/Game/Weather/BP_WeatherPhaseParams` (`self.NewWeather`)))
  (set `self.CurrentWeather` (make `/Game/Weather/BP_WeatherPhaseParams` (`self.InterpolatePerPhaseFloat` _currentweather_puddles _newweather_puddles) (`self.InterpolatePerPhaseFloat` _currentweather_rain _newweather_rain) (`self.InterpolatePerPhaseFloat` _currentweather_cloudopacity _newweather_cloudopacity) null (`self.InterpolatePerPhaseFloatArray` _currentweather_lightintensity _newweather_lightintensity) (`self.InterpolatePerPhaseFloat` _currentweather_skylightintensity _newweather_skylightintensity) (`self.InterpolatePerPhaseFloat` _currentweather_fogmultiplier _newweather_fogmultiplier) (`self.InterpolatePerPhaseFloat` _currentweather_darkcloudsblend _newweather_darkcloudsblend))))

(fn `InterpolatePerPhaseFloat`
  (params (a :type "/Game/Weather/BP_DayPhaseFloat Structure") (b :type "/Game/Weather/BP_DayPhaseFloat Structure"))
  (returns (result :type "/Game/Weather/BP_DayPhaseFloat Structure"))
  (locals (Value_ :type "Float (double-precision)") (InterpSpeed_ :type "Float (double-precision)"))
  (bind (_defaultvalue _defaultinterpspeed _phasevalueoverride _phaseinterpspeedoverride) (break `/Game/Weather/BP_DayPhaseFloat` b))
  (bind _dayphase (`self.DayPhase`))
  (bind (_value _returnvalue) (`BlueprintMapLibrary.Map_Find` _phasevalueoverride _dayphase))
  (bind (_value_2 _returnvalue_2) (`BlueprintMapLibrary.Map_Find` _phaseinterpspeedoverride _dayphase))
  (set `local.Value_` _defaultvalue)
  (set `local.InterpSpeed_` _defaultinterpspeed)
  (if _returnvalue
    (set `local.Value_` _value))
  (if _returnvalue_2
    (set `local.InterpSpeed_` _value_2))
  (return (make `/Game/Weather/BP_DayPhaseFloat` (`KismetMathLibrary.FInterpTo` (`.DefaultValue_21_1CE86CB24D7A181B13EE889B0EA75A50` (break `/Game/Weather/BP_DayPhaseFloat` a)) (`local.Value_`) (`GameplayStatics.GetWorldDeltaSeconds`) (* (`local.InterpSpeed_`) (`self.GlobalTransitionSpeed`) (select `bool` (>= (`self.GlobalWeatherTransitionTimeLeft`) 0.0) :`false` 1.0 :`true` (`self.GlobalWeatherTransitionMultiplier`)))) 1.0 (`|MakeMap`) (`|MakeMap`))))

(fn `InterpolatePerPhaseFloatArray`
  (params (a :type "Array of /Game/Weather/BP_DayPhaseFloat Structure") (b :type "Array of /Game/Weather/BP_DayPhaseFloat Structure"))
  (returns (result :type "Array of /Game/Weather/BP_DayPhaseFloat Structure"))
  (locals (Result_ :type "Array of /Game/Weather/BP_DayPhaseFloat Structure"))
  (for (_array_element _array_index) a
    (`KismetArrayLibrary.Array_Add` (`local.Result_`) (`self.InterpolatePerPhaseFloat` _array_element (`|GetArrayItem` b _array_index))))
  (return (`local.Result_`)))

(fn `SetTime`
  (params (Time :type "Float (double-precision)"))
  (bind _sunlight (`self.SunLight`))
  (`self.K2_SetActorRotation` _sunlight (`self.startSunRotation`) false)
  (`self.K2_AddActorLocalRotation` _sunlight (`KismetMathLibrary.MakeRotator` 0.0 (* (/ (- Time 14.0) 24.0) 360.0)) false false))

(fn `SetWeatherParams`
  (params (Current :type "/Game/Weather/BP_WeatherPhaseParams Structure"))
  (locals (Current_ :type "/Game/Weather/BP_WeatherParams Structure") (LightIntensities :type "Array of Float (double-precision)"))
  (bind _sky (`self.Sky`))
  (bind _fog (`self.Fog`))
  (bind _skylight (`self.SkyLight`))
  (bind (_puddles _rain _cloudopacity _cloudcolors _lightintensity _skylightintensity _fogmultiplier _darkcloudsblend) (break `/Game/Weather/BP_WeatherParams` (`local.Current_`)))
  (for _array_element Current_LightIntensity_23_621631674895AEDCAE40A9A9344B2C9D
    (`KismetArrayLibrary.Array_Add` (`local.LightIntensities`) (break `/Game/Weather/BP_DayPhaseFloat` _array_element)))
  (bind _output_get (set `local.Current_` (make `/Game/Weather/BP_WeatherParams` (break `/Game/Weather/BP_DayPhaseFloat` (break `/Game/Weather/BP_WeatherPhaseParams` Current)) (break `/Game/Weather/BP_DayPhaseFloat` (`.Rain_21_32946BD546D3F5FD59A73EAB56A0BC8F` (break `/Game/Weather/BP_WeatherPhaseParams` Current))) (break `/Game/Weather/BP_DayPhaseFloat` (`.CloudOpacity_22_4D2994E54F8701DCED0D608AAA42E979` (break `/Game/Weather/BP_WeatherPhaseParams` Current))) null (`local.LightIntensities`) (break `/Game/Weather/BP_DayPhaseFloat` (`.SkyLightIntensity_24_EB64537749B28F39BDE8F4859FD41F2F` (break `/Game/Weather/BP_WeatherPhaseParams` Current))) (break `/Game/Weather/BP_DayPhaseFloat` (`.FogMultiplier_27_1ED01AB743DE8687E394EAB7DDCE99BE` (break `/Game/Weather/BP_WeatherPhaseParams` Current))) (break `/Game/Weather/BP_DayPhaseFloat` (`.DarkCloudsBlend_29_438518A44D19E06A8608ED96A9EAAC50` (break `/Game/Weather/BP_WeatherPhaseParams` Current))))))
  (set `self.Editor_PreviewCurrentWeather` _output_get)
  (`KismetMaterialLibrary.SetScalarParameterValue` "/Game/Weather/MPC_Weather.MPC_Weather" "Rain Amount Multiplier" (`.Puddles_5_B84AF9D941C30BFC9EEC24B86E7EAD12` (break `/Game/Weather/BP_WeatherParams` (`local.Current_`))))
  (`KismetMaterialLibrary.SetScalarParameterValue` "/Game/Weather/MPC_Weather.MPC_Weather" "RainAmount" (`KismetMathLibrary.Square` (/ (`.Rain_4_32946BD546D3F5FD59A73EAB56A0BC8F` (break `/Game/Weather/BP_WeatherParams` (`local.Current_`))) 6000.0)))
  (`ParticleSystemComponent.SetFloatParameter` (`self.RainParticleSystem`) "Rain Rate" (`.Rain_4_32946BD546D3F5FD59A73EAB56A0BC8F` (break `/Game/Weather/BP_WeatherParams` (`local.Current_`))))
  (set `/Game/Weather/Sky/BP_DynamicSkySphere.Cloud opacity` _cloudopacity _sky)
  (set `/Game/Weather/Sky/BP_DynamicSkySphere.DarkCloudsBlend` _darkcloudsblend _sky)
  (`/Game/Weather/Sky/BP_DynamicSkySphere.Update` _sky)
  (`/Engine/EditorBlueprintResources/StandardMacros.IsValid` _fog
    (:`Is Valid`
      (`AtmosphericFogComponent.SetFogMultiplier` (`AtmosphericFog.AtmosphericFogComponent` _fog) (`.FogMultiplier_24_DAF06EDA40192C8FA844B1806912D07D` (break `/Game/Weather/BP_WeatherParams` (`local.Current_`)))))
    (:`Is Not Valid`
      _))
  (`/Engine/EditorBlueprintResources/StandardMacros.IsValid` _skylight
    (:`Is Valid`
      (`SkyLightComponent.SetIntensity` (`SkyLight.LightComponent` _skylight) (`.SkyLightIntensity_19_EB64537749B28F39BDE8F4859FD41F2F` (break `/Game/Weather/BP_WeatherParams` (`local.Current_`)))))
    (:`Is Not Valid`
      _))
  (for (_array_element_2 _array_index) (`self.Lights`)
    (`LightComponent.SetIntensity` (`Light.LightComponent` _array_element_2) (`|GetArrayItem` (`.LightIntensity_16_621631674895AEDCAE40A9A9344B2C9D` (break `/Game/Weather/BP_WeatherParams` (`local.Current_`))) _array_index))))

(fn `SetWeatherType`
  (params (Type :type "/Game/Weather/BP_WeatherType Enum" :default "NewEnumerator0"))
  (set `self.CurrentType` Type)
  (bind _params (`self.GetWeatherParamsForType` Type))
  (set `self.NewWeather` _params)
  (set `self.GlobalWeatherTransitionTimeLeft` (`self.GlobalWeatherTransitionTime`)))

(fn `UserConstructionScript`)