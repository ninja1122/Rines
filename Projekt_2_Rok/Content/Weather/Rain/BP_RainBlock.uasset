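; BP_RainBlock is a placeable volume that registers as a rain kill volume with the player pawn's BP_Rain component.
; Its construction script sizes FindBox to BlockBox's extent plus a horizontal margin, forming a larger detection zone.
; Any overlap entering or leaving FindBox adds or removes the actor from the component's KillVolumes and calls RefreshBoxes.
; The rain reference is cached at BeginPlay, with a one-frame delayed retry on overlap if missing.
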(event `self.ReceiveBeginPlay`
  (`self.AddRainRef`))

(event `self.FindBox.OnComponentBeginOverlap`
  (params (OverlappedComponent :type "PrimitiveComponent Object Reference") (OtherActor :type "Actor Object Reference") (OtherComp :type "PrimitiveComponent Object Reference") (OtherBodyIndex :type Integer) (bFromSweep :type Boolean) (SweepResult :type "HitResult Structure (by ref)"))
  (`self.EnsureRainRef`))

(event `self.FindBox.OnComponentEndOverlap`
  (params (OverlappedComponent :type "PrimitiveComponent Object Reference") (OtherActor :type "Actor Object Reference") (OtherComp :type "PrimitiveComponent Object Reference") (OtherBodyIndex :type Integer))
  (bind _rain (`self.Rain`))
  (`KismetArrayLibrary.Array_RemoveItem` (`/Game/Weather/Rain/BP_Rain.KillVolumes` _rain) self)
  (`/Game/Weather/Rain/BP_Rain.RefreshBoxes` _rain :!label _label))

(event `EnsureRainRef`
  (if (== (`self.Rain`) null)
    (`KismetSystemLibrary.Delay` 0.0)
    (`self.AddRainRef`))
  (`KismetArrayLibrary.Array_Add` (`/Game/Weather/Rain/BP_Rain.KillVolumes` (`self.Rain`)) self)
  (goto _label))

(event `AddRainRef`
  (set `self.Rain` (`self.GetComponentByClass` (`GameplayStatics.GetPlayerPawn` 0) "/Game/Weather/Rain/BP_Rain.BP_Rain_C")))

(fn `UserConstructionScript`
  (`BoxComponent.SetBoxExtent` (`self.FindBox`) (+ (`BoxComponent.GetScaledBoxExtent` (`self.BlockBox`)) (1000.0 1000.0 0.0)) true))