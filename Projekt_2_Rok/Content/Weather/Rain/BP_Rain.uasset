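; Rain helper that feeds kill volume bounds to the particle system on its owner, marking boxes for the effect.
; BeginPlay caches the particle component and prebuilds indexed min/max parameter names up to MaxBoxes.
; RefreshBoxes turns each volume's location and scale into axis-aligned corners, ignoring rotation, and writes them as vector parameters through SetBox.
; Unused slots are zeroed, and volumes beyond MaxBoxes are ignored.
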(event `self.ReceiveBeginPlay`
  (set `self.ParticleSystem` (`Actor.GetComponentByClass` (`self.GetOwner`) "/Script/Engine.ParticleSystemComponent"))
  (for _index (range (`self.maxBoxes`))
    (`KismetArrayLibrary.Array_Add` (`self.ParamNames`) (`KismetStringLibrary.Conv_StringToName` (`KismetStringLibrary.Concat_StrStr` "min" (`KismetStringLibrary.Conv_IntToString` _index))))
    (`KismetArrayLibrary.Array_Add` (`self.ParamNames`) (`KismetStringLibrary.Conv_StringToName` (`KismetStringLibrary.Concat_StrStr` "max" (`KismetStringLibrary.Conv_IntToString` _index))))))

(event `RefreshBoxes`
  (for (_array_element _array_index) (`self.KillVolumes`)
    (bind _returnvalue (`Actor.K2_GetActorLocation` _array_element))
    (bind _returnvalue_2 (* (`Actor.GetActorScale3D` _array_element) 100.0))
    (`self.SetBox` (- _returnvalue _returnvalue_2) (+ _returnvalue _returnvalue_2) _array_index))
  (for _index (range (`KismetArrayLibrary.Array_Length` (`self.KillVolumes`)) (`self.maxBoxes`))
    (`self.SetBox` (0.0 0.0 0.0) (0.0 0.0 0.0) _index)))

(event `SetBox`
  (params (Min :type "Vector Structure") (Max :type "Vector Structure") (Index :type Integer))
  (bind _returnvalue (* Index 2))
  (bind _particlesystem (`self.ParticleSystem`))
  (bind _paramnames (`self.ParamNames`))
  (if (< Index (`self.maxBoxes`))
    (`ParticleSystemComponent.SetVectorParameter` _particlesystem (`|GetArrayItem` _paramnames _returnvalue) Min)
    (`ParticleSystemComponent.SetVectorParameter` _particlesystem (`|GetArrayItem` _paramnames (+ _returnvalue 1)) Max)))