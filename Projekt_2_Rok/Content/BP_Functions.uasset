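; Shared helper functions for fetching the game instance and working with input bindings.
; Key lookup picks an action's gamepad or keyboard/mouse binding based on the game instance's UsingGamepad flag.
; GetKeyName turns that binding into display text with Shift, Ctrl, Alt and Cmd suffixes.
; IsKeyEventEqual matches a key event against named action or axis mappings, using scale sign for axis direction.
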(fn `GetFakeUpGameInstance`
  (returns (GameInstance :type "/Game/BP_GameInstance Object Reference"))
  (bind _asbp_game_instance (cast `/Game/BP_GameInstance` (`GameplayStatics.GetGameInstance` null)))
  (return _asbp_game_instance))

(fn `GetKeyForName`
  (params (ActionName :type Name))
  (returns (Action :type "InputActionKeyMapping Structure"))
  (bind _asfake_up_game_instance_base (cast `FakeUpGameInstanceBase` (`GameplayStatics.GetGameInstance` null)))
  (if (`FakeUpGameInstanceBase.bUsingGamepad` _asfake_up_game_instance_base)
    (for _array_element (`InputSettings.GetActionMappingByName` (`InputSettings.GetInputSettings`) ActionName)
      (if (`KismetInputLibrary.Key_IsGamepadKey` (`.Key` (break `InputActionKeyMapping` _array_element)))
        (return _array_element)))
    (else
      (for _array_element_2 (`InputSettings.GetActionMappingByName` (`InputSettings.GetInputSettings`) ActionName)
        (bind (_actionname _bshift _bctrl _balt _bcmd _key) (break `InputActionKeyMapping` _array_element_2))
        (if (or (`KismetInputLibrary.Key_IsKeyboardKey` _key) (`KismetInputLibrary.Key_IsMouseButton` _key))
          (return _array_element_2))))))

(fn `GetKeyName`
  (params (Key :type Name))
  (returns (Name :type Text))
  (bind _action (`self.GetKeyForName` Key))
  (bind _name (`self.GetSpecialKeysName` _action))
  (return (`|FormatText` "{0}{1}" (`KismetInputLibrary.Key_GetDisplayName` (`.Key` (break `InputActionKeyMapping` _action))) _name)))

(fn `GetSpecialKeysName`
  (params (Keys :type "InputActionKeyMapping Structure"))
  (returns (Name :type Text))
  (return (`KismetTextLibrary.Conv_StringToText` (`KismetStringLibrary.Concat_StrStr` (select `bool` Keys_bShift :`true` " + Shift") (select `bool` Keys_bCtrl :`true` " + Ctrl") (select `bool` Keys_bAlt :`true` " + Alt") (select `bool` Keys_bCmd :`true` " + Cmd")))))

(fn `IsKeyEventEqual`
  (params (KeyEvent :type "KeyEvent Structure") (KeyName :type Name) (AxisPositive :type Boolean :default true))
  (returns (equal :type Boolean))
  (bind _returnvalue (`InputSettings.GetInputSettings`))
  (bind _returnvalue_2 (`KismetInputLibrary.GetKey` KeyEvent))
  (for _array_element (`InputSettings.GetActionMappingByName` _returnvalue KeyName)
    (if (== (`.Key` (break `InputActionKeyMapping` _array_element)) _returnvalue_2)
      (return true)))
  (for _array_element_2 (`InputSettings.GetAxisMappingByName` _returnvalue KeyName)
    (if (and (== (`.Key` (break `InputAxisKeyMapping` _array_element_2)) _returnvalue_2) (select `bool` AxisPositive :`false` (< (`.Scale` (break `InputAxisKeyMapping` _array_element_2)) 0.0) :`true` (> (`.Scale` (break `InputAxisKeyMapping` _array_element_2)) 0.0)))
      (return true)))
  (return false))