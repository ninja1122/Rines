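; BP_Cheats provides debug cheat events for weather, time, player level and god mode, each printing its arguments.
; Weather and time cheats act on every BP_WeatherController, setting weather type, updating day phase or toggling random weather.
; CheatLevel repeatedly grants next-level experience through the player pawn's StatystykiPostaci component, and CheatGod toggles CanTakeDamage on its BP_Unit component.
; CheatWeather prints a "CheatLevel" label instead of its own name.
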(event `CheatWeather`
  (params (type :type "/Game/Weather/BP_WeatherType Enum" :default "NewEnumerator0"))
  (`KismetSystemLibrary.PrintText` (`|FormatText` "CheatLevel {0}" (`KismetTextLibrary.Conv_ByteToText` type)))
  (bind _outactors (`GameplayStatics.GetAllActorsOfClass` "/Game/Weather/BP_WeatherController.BP_WeatherController_C"))
  (for _array_element _outactors
    (`/Game/Weather/BP_WeatherController.SetWeatherType` _array_element type)))

(event `CheatLevel`
  (params (Levels :type Integer))
  (bind _returnvalue (`Actor.GetComponentByClass` (`GameplayStatics.GetPlayerPawn` 0) "/Script/Projekt_2_Rok.StatystykiPostaci"))
  (`KismetSystemLibrary.PrintText` (`|FormatText` "CheatLevel {0}" Levels))
  (for _ (range Levels)
    (`StatystykiPostaci.DodajDoswiadczenie` _returnvalue (`StatystykiPostaci.doswiadczenieNaKoloejnyPoziom` _returnvalue))))

(event `CheatTime`
  (params (seconds :type "Float (double-precision)"))
  (`KismetSystemLibrary.PrintText` (`|FormatText` "CheatTime {0}" seconds))
  (bind _outactors (`GameplayStatics.GetAllActorsOfClass` "/Game/Weather/BP_WeatherController.BP_WeatherController_C"))
  (for _array_element _outactors
    (`/Game/Weather/BP_WeatherController.UpdateDayPhase` _array_element seconds)))

(event `CheatRandomWeather`
  (params (enabled :type Boolean))
  (`KismetSystemLibrary.PrintText` (`|FormatText` "CheatRandomWeather {0}" (`KismetTextLibrary.Conv_BoolToText` enabled)))
  (bind _outactors (`GameplayStatics.GetAllActorsOfClass` "/Game/Weather/BP_WeatherController.BP_WeatherController_C"))
  (for _array_element _outactors
    (set `/Game/Weather/BP_WeatherController.EnableRandomWeather` enabled _array_element)))

(event `CheatGod`
  (params (enabled :type Boolean))
  (`KismetSystemLibrary.PrintText` (`|FormatText` "CheatGod {0}" (`KismetTextLibrary.Conv_BoolToText` enabled)))
  (set `/Game/Combat/Blueprints/BP_Unit.canTakeDamage` (not enabled) (`Actor.GetComponentByClass` (`GameplayStatics.GetPlayerPawn` 0) "/Game/Combat/Blueprints/BP_Unit.BP_Unit_C")))