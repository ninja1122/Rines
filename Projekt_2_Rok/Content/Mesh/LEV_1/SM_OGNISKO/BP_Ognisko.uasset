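; BP_Ognisko is a campfire that the player lights or extinguishes through BP_Interactable, with a Polish prompt matching its state.
; A fireball or flame breath actor overlapping its Box also lights it.
; SetBurningState ignores unchanged states, updates the prompt and toggles the light and fire, firing an ignition burst shortly before the flames start.
; The construction script applies the initial burning state to fire auto-activation and light visibility.
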(event `self.ReceiveBeginPlay`
  (`/Game/Blueprints/Interactable/BP_Interactable.Init` (`self.BP_Interactable`) (`self.Box`) (`self.GetText`)))

(event `self.BP_Interactable.Interacted`
  (`self.SetBurningState` (not (`self.isBuring`))))

(event `self.Box.OnComponentBeginOverlap`
  (params (OverlappedComponent :type "PrimitiveComponent Object Reference") (OtherActor :type "Actor Object Reference") (OtherComp :type "PrimitiveComponent Object Reference") (OtherBodyIndex :type Integer) (bFromSweep :type Boolean) (SweepResult :type "HitResult Structure (by ref)"))
  (if (`self.IsAbleToBeginFire` OtherActor)
    (`self.SetBurningState` true)))

(event `SetBurningState`
  (params (Burning :type Boolean))
  (bind _fire (`self.Fire`))
  (bind _pointlight (`self.PointLight`))
  (if (!= Burning (`self.isBuring`))
    (set `self.isBuring` Burning)
    (set `/Game/Blueprints/Interactable/BP_Interactable.TextToShow` (`self.GetText`) (`self.BP_Interactable`))
    (if (`self.isBuring`)
      (`ActorComponent.Activate` (`self.Explo`) true)
      (`SceneComponent.SetVisibility` _pointlight true false)
      (`KismetSystemLibrary.Delay` 0.3)
      (`ActorComponent.Activate` _fire false)
      (else
        (`SceneComponent.SetVisibility` _pointlight false false)
        (`ActorComponent.Deactivate` _fire)))))

(fn `GetText`
  (returns (Text :type Text))
  (return (select `bool` (`self.isBuring`) :`false` "Naciśnij {0} aby zapalić ognisko" :`true` "Naciśnij {0} aby zgasić ognisko" :!type "Text")))

(fn `IsAbleToBeginFire`
  (params (Actor :type "Actor Object Reference"))
  (returns (Able :type Boolean))
  (bind _returnvalue (`GameplayStatics.GetObjectClass` Actor))
  (return (or (== _returnvalue "/Game/Combat/FireBall/BP_FireBall.BP_FireBall_C") (== _returnvalue "/Game/Combat/FireBall/BP_FlameBreath.BP_FlameBreath_C"))))

(fn `UserConstructionScript`
  (bind _isburing (`self.isBuring`))
  (`ActorComponent.SetAutoActivate` (`self.Fire`) _isburing)
  (`SceneComponent.SetVisibility` (`self.PointLight`) _isburing false))