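; Construction-script Blueprint that lays out a row of gravestone meshes ("nagrobki") along a spline.
; It divides the spline length by the spacing Odstęp and adds a static mesh component at each step, using world-space spline positions with manual attachment and a shared yaw, Obrut.
; The TabZmiennych array selects one of five meshes per step, repeating every twenty entries.
; The event graph has no active logic.
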(fn `UserConstructionScript`
  (bind _spline (`self.Spline`))
  (bind _returned_mesh (`self.returned_mesh`))
  (for _index (range (+ (`.ReturnValue` (`KismetMathLibrary.FMod` (- (`SplineComponent.GetDistanceAlongSplineAtSplinePoint` _spline (- (`SplineComponent.GetNumberOfSplinePoints` _spline) 1)) (`SplineComponent.GetDistanceAlongSplineAtSplinePoint` _spline 0)) (`self.Odstęp`))) 1))
    (bind _returnvalue (`AddComponent|NODE_AddStaticMeshComponent-0` :`bManualAttachment` true :`RelativeTransform` (`KismetMathLibrary.MakeTransform` (`SplineComponent.GetLocationAtDistanceAlongSpline` (`self.Spline`) (* _index (`self.Odstęp`)) "World") (`KismetMathLibrary.MakeRotator` 0.0 0.0 (`self.obrut`)))))
    (set `self.returned_mesh` _returnvalue)
    (switch `int` (`|GetArrayItem` (`self.Tab_Zmiennych`) (mod _index 20))
      (:`1`
        (`StaticMeshComponent.SetStaticMesh` _returned_mesh (`self.Mesh_1`)))
      (:`2`
        (`StaticMeshComponent.SetStaticMesh` _returned_mesh (`self.Mesh_2`)))
      (:`3`
        (`StaticMeshComponent.SetStaticMesh` _returned_mesh (`self.Mesh_3`)))
      (:`4`
        (`StaticMeshComponent.SetStaticMesh` _returned_mesh (`self.Mesh_4`)))
      (:`5`
        (`StaticMeshComponent.SetStaticMesh` _returned_mesh (`self.Mesh_5`))))))