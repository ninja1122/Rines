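; Spline-driven actor, named as a track (Tory), that lays repeated mesh segments along an editable spline.
; The construction script divides the spline length by Selength and adds a collision-free, X-forward spline mesh for each step.
; Segment endpoints are sampled in local space, with tangents clamped to segment length so the meshes follow the curve.
; It has no runtime logic.
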(fn `UserConstructionScript`
  (bind _spline1 (`self.Spline1`))
  (for _index (range (+ (`KismetMathLibrary.FTrunc` (/ (`SplineComponent.GetSplineLength` (`self.Spline1`)) (`self.selength`))) 1))
    (bind _returnvalue (`AddComponent|NODE_AddSplineMeshComponent-0`))
    (`SplineMeshComponent.SetForwardAxis` _returnvalue "X" true)
    (`PrimitiveComponent.SetCollisionEnabled` _returnvalue "NoCollision")
    (bind _returnvalue_2 (* _index (`self.selength`)))
    (bind _returnvalue_3 (* (+ _index 1) (`self.selength`)))
    (`SplineMeshComponent.SetStartAndEnd` _returnvalue (`SplineComponent.GetLocationAtDistanceAlongSpline` _spline1 _returnvalue_2 "Local") (`KismetMathLibrary.ClampVectorSize` (`SplineComponent.GetTangentAtDistanceAlongSpline` _spline1 _returnvalue_2 "Local") 0.0 (`self.selength`)) (`SplineComponent.GetLocationAtDistanceAlongSpline` _spline1 _returnvalue_3 "Local") (`KismetMathLibrary.ClampVectorSize` (`SplineComponent.GetTangentAtDistanceAlongSpline` _spline1 _returnvalue_3 "Local") 0.0 (`self.selength`)) true)))