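; BP_IsWeatherEqual is a behavior tree decorator check that tests whether the map's current weather matches its WeatherType for an NPC.
; It casts the owner to NPC_1_AI_Controller and compares only when that controller's flag for heeding weather and night is set; otherwise it passes.
; The first BP_WeatherController found in the level is cached and supplies the current weather type.
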(fn `PerformConditionCheck`
  (params (OwnerActor :type "Actor Object Reference"))
  (returns (ReturnValue :type Boolean))
  ;[1 1 1] Pobierz i  sprawdz jaka pogoda jest na mapie
  (bind _asnpc_1_ai_controller (cast `/Game/Zaglowiec/NPC/NPC_1_AI_Controller` OwnerActor))
  (set `self.AI_CON_Ref` _asnpc_1_ai_controller)
  (if (`/Game/Zaglowiec/NPC/NPC_1_AI_Controller.CzyZwaracUwageNaPogodeINOCCharacter` (`self.AI_CON_Ref`))
    (if (not (!= (`self.weatherController`) null))
      (bind _outactors (`GameplayStatics.GetAllActorsOfClass` "/Game/Weather/BP_WeatherController.BP_WeatherController_C"))
      (set `self.weatherController` (`|GetArrayItem` _outactors)))
    (return (`|EnumEquality` (`self.weatherType`) (`/Game/Weather/BP_WeatherController.CurrentType` (`self.weatherController`))))
    (else
      (return true))))