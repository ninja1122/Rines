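; BP_FlameBreath is a short-lived flame breath attack actor that stretches out and then destroys itself.
; Init calls a projectile target trace but sets rotation from the camera direction alone, leaving the trace result unused.
; Tick grows Scene1's Z scale with elapsed lifetime until the actor expires after half a second.
; The construction script passes Damage to BPDamageDealer.
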(event `self.ReceiveTick`
  (params (DeltaSeconds :type "Float (single-precision)"))
  (bind _output_get (set `self.lifeTime` (+ DeltaSeconds (`self.lifeTime`))))
  (`SceneComponent.SetWorldScale3D` (`self.Scene1`) (`KismetMathLibrary.MakeVector` 1.0 1.0 (* _output_get 2.0)))
  (if (>= (`self.lifeTime`) 0.5)
    (`self.K2_DestroyActor`)))

(event `Init`
  (params (start :type "Vector Structure") (cameraPosition :type "Vector Structure") (cameraDirection :type "Vector Structure"))
  (`Helpers.findProjectileTargetPosition` start (`self.distance`) (+ cameraPosition cameraDirection) cameraDirection (`self.traceChannel`))
  (`self.K2_SetActorRotation` (`KismetMathLibrary.FindLookAtRotation` start (+ start cameraDirection))))

(fn `UserConstructionScript`
  (set `/Game/Combat/Blueprints/BP_DamageDealer.damage` (`self.damage`) (`self.BP_DamageDealer`)))