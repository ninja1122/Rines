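; BP_FireBall is a fireball projectile that explodes when it is destroyed.
; Init stores the big flag, launches the camera-targeted BPProjectile component and enables sphere collision, which is off from BeginPlay.
; On projectile destruction it spawns a BP_Explosion with that size flag and explosion damage, then destroys itself after a zero-length delay.
; The construction script copies its Damage into the BPDamageDealer component.
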(event `self.ReceiveBeginPlay`
  (add `/Game/Combat/Blueprints/BP_Projectile.OnProjectileDestroyed` (`self.BP_Projectile`) (delegate `OnProjectileDestroyed`))
  (`PrimitiveComponent.SetCollisionEnabled` (`self.Sphere`) "NoCollision"))

(event `OnProjectileDestroyed`
  (params (CollidedWith :type "Actor Soft Object Reference"))
  (`|SpawnActorFromClass` "/Game/Combat/FireBall/BP_Explosion.BP_Explosion_C" (`KismetMathLibrary.Conv_VectorToTransform` (`self.K2_GetActorLocation`)) "Undefined" "OverrideRootScale" null (`self.isBig`) (`self.explosionDamage`) null)
  (`KismetSystemLibrary.Delay` 0.0)
  (`self.K2_DestroyActor`))

(event `Init`
  (params (start :type "Vector Structure") (cameraPosition :type "Vector Structure") (cameraDirection :type "Vector Structure") (isBig :type Boolean))
  (set `self.isBig` isBig)
  (`/Game/Combat/Blueprints/BP_Projectile.InitCameraTargettedProjectile` (`self.BP_Projectile`) start cameraPosition cameraDirection)
  (`PrimitiveComponent.SetCollisionEnabled` (`self.Sphere`) "QueryAndPhysics"))

(fn `UserConstructionScript`
  (set `/Game/Combat/Blueprints/BP_DamageDealer.damage` (`self.damage`) (`self.BP_DamageDealer`)))