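; Player spell caster for a hold-to-charge fire spell with three tiers: flame breath, fireball and big fireball.
; Casting attaches a BP_FireBall to the hand socket, and Tick times the hold until release picks the tier.
; Release locks movement and turns the player to the camera; AnimBP_Player2 fired events then launch the fireball or replace it with BP_FlameBreath.
; Damage scales with spell level, and cancelling destroys the held fireball.
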(event `self.Init`
  (params (actor :type "Actor Object Reference") (manager :type "/Game/Combat/SpellSystem/BP_SpellManager Object Reference"))
  (bind _animbp (`self.GetAnimBP`))
  (`parent.Init` actor manager)
  (add `/Game/Combat/Player/tests/AnimBP_Player2.FireBallFired` _animbp (delegate `FireBallFired`))
  (add `/Game/Combat/Player/tests/AnimBP_Player2.FlameBreathFired` _animbp (delegate `FlameBreathFired`)))

(event `FireBallFired`
  (bind _returnvalue (`GameplayStatics.GetPlayerCameraManager` 0))
  (bind _fireball (`self.fireball`))
  (set `self.castPhase` "NewEnumerator0")
  (`/Engine/EditorBlueprintResources/StandardMacros.IsValid` (`self.fireball`)
    (:`Is Valid`
      (`SceneComponent.K2_DetachFromComponent` (`Actor.RootComponent` _fireball) "KeepWorld" "KeepRelative" "KeepRelative" true)
      (`/Game/Combat/FireBall/BP_FireBall.Init` _fireball (`self.K2_GetActorLocation` (`self.fireball`)) (`PlayerCameraManager.GetCameraLocation` _returnvalue) (`self.GetActorForwardVector` _returnvalue) (`self.isBig`))
      (`/Game/Combat/SpellSystem/BP_SpellManager.SetMovementMode` (`self.ownerManager`) true))))

(event `FlameBreathFired`
  (bind _returnvalue (`GameplayStatics.GetPlayerCameraManager` 0))
  (bind _returnvalue_2 (`self.K2_GetActorLocation` (`self.fireball`)))
  (set `self.castPhase` "NewEnumerator0")
  (`/Engine/EditorBlueprintResources/StandardMacros.IsValid` (`self.fireball`)
    (:`Is Valid`
      (`SceneComponent.K2_DetachFromComponent` (`Actor.RootComponent` (`self.fireball`)) "KeepWorld" "KeepRelative" "KeepRelative" true)
      (bind _returnvalue_3 (`|SpawnActorFromClass` "/Game/Combat/FireBall/BP_FlameBreath.BP_FlameBreath_C" (`KismetMathLibrary.Conv_VectorToTransform` _returnvalue_2) "Undefined" "OverrideRootScale" null (`/Game/Combat/Blueprints/BP_Helpers.Evaluate` (`self.flameBreathDamage`) (`self.level`)) null))
      (`/Game/Combat/FireBall/BP_FlameBreath.Init` _returnvalue_3 _returnvalue_2 (`PlayerCameraManager.GetCameraLocation` _returnvalue) (`self.GetActorForwardVector` _returnvalue))
      (`self.K2_DestroyActor` (`self.fireball`))
      (set `self.fireball` null)
      (`self.SetMaxCooldown`)
      (`/Game/Combat/SpellSystem/BP_SpellManager.SetMovementMode` (`self.ownerManager`) true))))

(event `self.ReceiveTick`
  (params (DeltaSeconds :type "Float (single-precision)"))
  (`parent.ReceiveTick` DeltaSeconds)
  (if (`|EnumEquality` (`self.castPhase`) "NewEnumerator1")
    (set `self.castingLength` (+ (`self.castingLength`) DeltaSeconds))))

(event `self.CastSpell`
  (if (and (`self.isReady`) (not (`/Game/Combat/SpellSystem/BP_SpellManager.IsPlayerFalling` (`self.ownerManager`))))
    (if (`|EnumEquality` (`self.castPhase`) "NewEnumerator0")
      (set `self.castingLength` 0.0)
      (set `self.castPhase` "NewEnumerator1")
      (`self.BeginCast`))))

(event `self.ReleaseSpell`
  (if (`|EnumEquality` (`self.castPhase`) "NewEnumerator1")
    (set `self.castPhase` "NewEnumerator2")
    (if (>= (`self.castingLength`) 0.75)
      (`self.CastFireball` (>= (`self.castingLength`) 1.5))
      (else
        (`self.CastFlameBreath`)))))

(event `SetPlayerAnimState`
  (params (State :type "/Game/Combat/Player/BP_PlayerState Enum" :default "NewEnumerator0"))
  (`/Game/Combat/Player/tests/AnimBP_Player2.SetState` (`self.GetAnimBP`) State))

(event `BeginCast`
  (`self.SetPlayerAnimState` "NewEnumerator1")
  (bind _returnvalue (`|SpawnActorFromClass` "/Game/Combat/FireBall/BP_FireBall.BP_FireBall_C" (`KismetMathLibrary.Conv_VectorToTransform` (0.0 0.0 0.0)) "Undefined" "OverrideRootScale" null (`/Game/Combat/Blueprints/BP_Helpers.Evaluate` (`self.fireBallDamage`) (`self.level`)) (`/Game/Combat/Blueprints/BP_Helpers.Evaluate` (`self.explosionDamage`) (`self.level`)) null))
  (set `self.fireball` _returnvalue)
  (bind _ascharacter (cast `Character` (`self.ownerPlayer`)))
  (`SceneComponent.K2_AttachToComponent` (`Actor.RootComponent` _returnvalue) (`self.GetComponentByClass` _ascharacter "/Script/Engine.SkeletalMeshComponent") "SOCKET_FIREBALL" "KeepRelative" "KeepWorld" "KeepWorld" true))

(event `CastFlameBreath`
  (`self.SetPlayerAnimState` "NewEnumerator2")
  (`/Game/Combat/SpellSystem/BP_SpellManager.SetMovementMode` (`self.ownerManager`) false)
  (`/Game/Combat/SpellSystem/BP_SpellManager.RotatePlayer` (`self.ownerManager`) (`self.GetActorForwardVector` (`GameplayStatics.GetPlayerCameraManager` 0))))

(event `CastFireball`
  (params (big :type Boolean))
  (set `self.isBig` big)
  (`self.SetPlayerAnimState` "NewEnumerator3")
  (`/Game/Combat/SpellSystem/BP_SpellManager.SetMovementMode` (`self.ownerManager`) false)
  (`/Game/Combat/SpellSystem/BP_SpellManager.RotatePlayer` (`self.ownerManager`) (`self.GetActorForwardVector` (`GameplayStatics.GetPlayerCameraManager` 0))))

(event `self.CancelSpell`
  (bind _fireball (`self.fireball`))
  (`|ExecutionSequence`
    (:`then_0`
      (if (`|EnumInequality` (`self.castPhase`) "NewEnumerator0")
        (set `self.castPhase` "NewEnumerator0")
        (`self.SetPlayerAnimState` "NewEnumerator0")))
    (:`then_1`
      (`/Engine/EditorBlueprintResources/StandardMacros.IsValid` _fireball
        (:`Is Valid`
          (`self.K2_DestroyActor` _fireball)
          (set `self.fireball` null))))))

(fn `GetAnimBP`
  (returns (AnimBP :type "/Game/Combat/Player/tests/AnimBP_Player2 Object Reference"))
  (bind _ascharacter (cast `Character` (`self.ownerPlayer`)))
  (bind _asanim_bp_player_2 (cast `/Game/Combat/Player/tests/AnimBP_Player2` (`SkeletalMeshComponent.GetAnimInstance` (`Character.Mesh` _ascharacter))))
  (return _asanim_bp_player_2))

(fn `GetSpellInfo`
  (params (ForNextLevel :type Boolean))
  (returns (Text :type Text))
  (locals (ForNextLevel_ :type Boolean))
  (set `local.ForNextLevel_` ForNextLevel)
  (bind _name (`/Game/BP_Functions.GetKeyName` "Fireball"))
  (return (`|FormatText` "Przytrzymaj {key}, aby naładować kulę ognia.  \n- I stopień {FireBreathDamage} obrażeń bliskiego zasięgu \n- II stopień {FireBallDamage} obrażeń dalekiego zasięgu \n- III stopień zadaje dodatkowo {FireBallExplosionDamage} obrażeń obszarowych" _name (`/Game/Combat/Blueprints/BP_Helpers.EvaluateString` (`self.flameBreathDamage`) (`self.level`) (`local.ForNextLevel_`)) (`/Game/Combat/Blueprints/BP_Helpers.EvaluateString` (`self.fireBallDamage`) (`self.level`) (`local.ForNextLevel_`)) (`/Game/Combat/Blueprints/BP_Helpers.EvaluateString` (`self.explosionDamage`) (`self.level`) (`local.ForNextLevel_`)))))

(fn `UserConstructionScript`
  (`parent.UserConstructionScript`))