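; BP_Cougar is an enemy cougar character that gains aggro when damaged and drops a Skora actor plus a random potion on death.
; It stores its spawn location in the AI blackboard and relies on a BP_Unit component for damage and death events.
; Hits damage other units only during a specific AnimBP_Cougar state, gated by a jump-attack cooldown counted down on Tick.
; Tick also smoothly rotates it toward its velocity.
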(event `self.ReceiveBeginPlay`
  (bind _bp_unit (`self.BP_Unit`))
  (add `/Game/Combat/Blueprints/BP_Unit.UnitTookDamage` _bp_unit (delegate `CougarTookDamage`))
  (add `/Game/Combat/Blueprints/BP_Unit.UnitDied` _bp_unit (delegate `UnitDied_`))
  (`BlackboardComponent.SetValueAsVector` (`AIBlueprintHelperLibrary.GetBlackboard` (`AIBlueprintHelperLibrary.GetAIController` self)) "SpawnPoint" (`self.K2_GetActorLocation`)))

(event `CougarTookDamage`
  (params (damage :type "Float (double-precision)") (type :type "/Game/Combat/Blueprints/BP_DamageType Enum" :default "NewEnumerator0"))
  (set `/Game/Combat/Blueprints/BP_Unit.hasAggro` true (`self.BP_Unit`)))

(event `UnitDied_`
  (params (Actor :type "Actor Object Reference") (Unit :type "/Game/Combat/Blueprints/BP_Unit Object Reference"))
  (`|SpawnActorFromClass` "/Game/Blueprints/Inventory/skora.skora_C" (`KismetMathLibrary.Conv_VectorToTransform` (`self.K2_GetActorLocation`)) "AlwaysSpawn" "OverrideRootScale" null null)
  (`/Game/BP_GameInstance.SpawnRandomPotion` (`/Game/BP_Functions.GetFakeUpGameInstance`) (`self.K2_GetActorLocation`)))

(event `DealDamage`)

(event `self.ReceiveTick`
  (params (DeltaSeconds :type "Float (single-precision)"))
  (set `self.jumpAttackCooldown` (- (`self.jumpAttackCooldown`) (`GameplayStatics.GetWorldDeltaSeconds`)))
  (`self.RotateToDirectiion`))

(event `self.ReceiveHit`
  (params (MyComp :type "PrimitiveComponent Object Reference") (Other :type "Actor Object Reference") (OtherComp :type "PrimitiveComponent Object Reference") (bSelfMoved :type Boolean) (HitLocation :type "Vector Structure") (HitNormal :type "Vector Structure") (NormalImpulse :type "Vector Structure") (Hit :type "HitResult Structure (by ref)"))
  (bind _returnvalue (`self.GetComponentByClass` Other "/Game/Combat/Blueprints/BP_Unit.BP_Unit_C"))
  (if (<= (`self.jumpAttackCooldown`) 0.0)
    (bind _asanim_bp_cougar (cast `/Game/Combat/Cougar/AnimBP_Cougar` (`SkeletalMeshComponent.GetAnimInstance` (`self.Mesh`))))
    (if (`/Game/Combat/Cougar/AnimBP_Cougar.IsStateInProgress` _asanim_bp_cougar "NewEnumerator2")
      (`/Engine/EditorBlueprintResources/StandardMacros.IsValid` _returnvalue
        (:`Is Valid`
          (`/Game/Combat/Blueprints/BP_Unit.Take Damage` _returnvalue 45.0 "NewEnumerator0")
          (set `self.jumpAttackCooldown` 4.0))))))

(event `RotateToDirectiion`
  (bind _velocity (`MovementComponent.Velocity` (`self.CharacterMovement`)))
  (if (!= (`KismetMathLibrary.VSizeSquared` _velocity) 0.0)
    (`self.K2_SetActorRotation` (`KismetMathLibrary.RLerp` (`self.K2_GetActorRotation`) (`KismetMathLibrary.FindLookAtRotation` (`KismetMathLibrary.MakeVector` 0.0) _velocity) 0.4 true))))

(fn `UserConstructionScript`)