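; BP_RatSpit is a rat spit projectile actor that bursts into a green explosion when its flight ends.
; Init launches it forward from its location in a given direction through the BPProjectile component.
; That component's destroyed event spawns BP_GreenExplosion, plus BP_GreenFire if LeaveFire is set and the collided-with reference is valid.
; The actor then destroys itself after a zero-length delay.
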(event `self.ReceiveBeginPlay`
  (add `/Game/Combat/Blueprints/BP_Projectile.OnProjectileDestroyed` (`self.BP_Projectile`) (delegate `OnProjectileDestroyed`)))

(event `OnProjectileDestroyed`
  (params (CollidedWith :type "Actor Soft Object Reference"))
  (`|SpawnActorFromClass` "/Game/Combat/RatSpit/BP_GreenExplosion.BP_GreenExplosion_C" (`KismetMathLibrary.Conv_VectorToTransform` (`self.K2_GetActorLocation`)) "Undefined" "OverrideRootScale" null false null)
  (if (and (`KismetSystemLibrary.IsValidSoftObjectReference` CollidedWith) (`self.LeaveFire`))
    (`|SpawnActorFromClass` "/Game/Combat/GreenFire/BP_GreenFire.BP_GreenFire_C" (`KismetMathLibrary.Conv_VectorToTransform` (`self.K2_GetActorLocation`)) "Undefined" "OverrideRootScale" null null))
  (`KismetSystemLibrary.Delay` 0.0)
  (`self.K2_DestroyActor`))

(event `Init`
  (params (direction :type "Vector Structure"))
  (`/Game/Combat/Blueprints/BP_Projectile.InitForwardProjectile` (`self.BP_Projectile`) (`self.K2_GetActorLocation`) direction))

(fn `UserConstructionScript`)