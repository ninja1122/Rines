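; BP_Kostek is an AI-controlled melee combat character built on a BP_Unit component for health, aggro and damage.
; It records its spawn point in the blackboard on BeginPlay and gains aggro when damaged.
; AttackInFront damages the blackboard TargetActor through its BP_Unit if it passes range and forward-cone checks, and SetLowHealth overrides health.
; Tick smoothly turns it toward horizontal velocity and plays random sounds at random intervals while alive.
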(event `self.ReceiveBeginPlay`
  (add `/Game/Combat/Blueprints/BP_Unit.UnitTookDamage` (`self.BP_Unit`) (delegate `CougarTookDamage`))
  (`BlackboardComponent.SetValueAsVector` (`AIBlueprintHelperLibrary.GetBlackboard` (`AIBlueprintHelperLibrary.GetAIController` self)) "SpawnPoint" (`self.K2_GetActorLocation`)))

(event `CougarTookDamage`
  (params (damage :type "Float (double-precision)") (type :type "/Game/Combat/Blueprints/BP_DamageType Enum" :default "NewEnumerator0"))
  (set `/Game/Combat/Blueprints/BP_Unit.hasAggro` true (`self.BP_Unit`)))

(event `AttackInFront`
  (bind _asactor (cast `Actor` (`BlackboardComponent.GetValueAsObject` (`AIBlueprintHelperLibrary.GetBlackboard` (`AIBlueprintHelperLibrary.GetAIController` self)) "TargetActor")))
  (bind _returnvalue (- (`self.K2_GetActorLocation` _asactor) (`self.K2_GetActorLocation`)))
  (if (and (<= (`KismetMathLibrary.VSize` _returnvalue) 250.0) (>= (`KismetMathLibrary.Dot_VectorVector` (`KismetMathLibrary.Normal` _returnvalue) (`self.GetActorForwardVector`)) (`KismetMathLibrary.DegCos` 45.0)))
    (bind _returnvalue_2 (`self.GetComponentByClass` _asactor "/Game/Combat/Blueprints/BP_Unit.BP_Unit_C"))
    (`/Engine/EditorBlueprintResources/StandardMacros.IsValid` _returnvalue_2
      (:`Is Valid`
        (`/Game/Combat/Blueprints/BP_Unit.Take Damage` _returnvalue_2 7.0 "NewEnumerator0")))))

(event `SetLowHealth`
  (set `/Game/Combat/Blueprints/BP_Unit.health` (make `/Game/Combat/Blueprints/BP_UnitHealth` 250.0 250.0) (`self.BP_Unit`)))

(event `self.ReceiveTick`
  (params (DeltaSeconds :type "Float (single-precision)"))
  (bind _audio (`self.Audio`))
  (bind _returnvalue (* (`MovementComponent.Velocity` (`self.CharacterMovement`)) (1.0 1.0 0.0)))
  (`|ExecutionSequence`
    (:`then_0`
      (if (!= (`KismetMathLibrary.VSizeSquared` _returnvalue) 0.0)
        (`self.K2_SetActorRotation` (`KismetMathLibrary.RLerp` (`self.K2_GetActorRotation`) (`KismetMathLibrary.FindLookAtRotation` (`KismetMathLibrary.MakeVector` 0.0) _returnvalue) 0.4 true))))
    (:`then_1`
      (if (`/Game/Combat/Blueprints/BP_Unit.IsAlive` (`self.BP_Unit`))
        (set `self.randomSoundTime` (- (`self.randomSoundTime`) (`GameplayStatics.GetWorldDeltaSeconds`)))
        (if (<= (`self.randomSoundTime`) 0.0)
          (set `self.randomSoundTime` (`KismetMathLibrary.RandomFloatInRange` 1.0 2.5))
          (`AudioComponent.SetSound` _audio (`|GetArrayItem` (`self.randomSounds`) (`KismetMathLibrary.RandomInteger` 2)))
          (`AudioComponent.Play` _audio 0.0))))))

(fn `UserConstructionScript`)