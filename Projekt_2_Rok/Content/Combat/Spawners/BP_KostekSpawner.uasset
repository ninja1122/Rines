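; BP_KostekSpawner is a spawner that adds a smoke-burst entrance to spawned actors and can start a Kostek enemy at low health.
; Its Trigger Spawn override spawns BP_SmokeBurst at its own transform, calls the parent spawn and hides the new actor's skeletal mesh.
; A custom event restores mesh visibility after a short delay if the actor is still valid.
; When LowHealth is set, it calls SetLowHealth on a spawned BP_Kostek.
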(event `self.ReceiveBeginPlay`)

(event `Set Visible After Delay`
  (params (Actor :type "Actor Object Reference"))
  (bind _actor (`self.Actor`))
  (set `self.Actor` Actor)
  (`KismetSystemLibrary.Delay` 1.0)
  (`/Engine/EditorBlueprintResources/StandardMacros.IsValid` _actor
    (:`Is Valid`
      (`SceneComponent.SetVisibility` (`self.GetComponentByClass` _actor "/Script/Engine.SkeletalMeshComponent") true false))))

(fn `Trigger Spawn`
  (returns (Actor :type "Actor Object Reference"))
  (`|SpawnActorFromClass` "/Game/Combat/SmokeBurst/BP_SmokeBurst.BP_SmokeBurst_C" (`self.GetTransform`) "Undefined" "OverrideRootScale" null null)
  (bind _actor (`parent.Trigger Spawn`))
  (`SceneComponent.SetVisibility` (`self.GetComponentByClass` _actor "/Script/Engine.SkeletalMeshComponent") false false)
  (`self.Set Visible After Delay` _actor)
  (if (`self.lowHealth`)
    (bind _asbp_kostek (cast `/Game/Combat/Kostek/BP_Kostek` _actor)
      (:`then`
        (`/Game/Combat/Kostek/BP_Kostek.SetLowHealth` _asbp_kostek))
      (:`CastFailed`
        _)))
  (return _actor))

(fn `UserConstructionScript`
  (`parent.UserConstructionScript`))