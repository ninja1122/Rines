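; BP_KostekSpawnController coordinates Kostek enemy spawners and fire pillars in combat.
; TriggerSpawn fires every spawner, or only flagged ones during a pillar phase, and switches the pillars to match.
; Pillar-phase spawns are tracked through their BP_Unit death events.
; When the last tracked enemy dies, the pillars deactivate and, after a short delay, all spawners trigger in normal phase.
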(event `TriggerSpawn`
  (params (PillarPhase :type Boolean :default true))
  (for (_array_element _array_index) (`self.Spawners`)
    (if (or (not PillarPhase) (`|GetArrayItem` (`self.SpawnFirePillarsPhase`) _array_index))
      (bind _actor (`/Game/Combat/Spawners/BP_Spawner.Trigger Spawn` _array_element))
      (if PillarPhase
        (`KismetArrayLibrary.Array_Add` (`self.Enemies`) _actor)
        (add `/Game/Combat/Blueprints/BP_Unit.UnitDied` (`self.GetComponentByClass` _actor "/Game/Combat/Blueprints/BP_Unit.BP_Unit_C") (delegate `Kostek Died`)))))
  (`self.Set Active Pillars` PillarPhase))

(event `Kostek Died`
  (params (Actor :type "Actor Object Reference") (Unit :type "/Game/Combat/Blueprints/BP_Unit Object Reference"))
  (`KismetArrayLibrary.Array_RemoveItem` (`self.Enemies`) Actor)
  (if (== (`KismetArrayLibrary.Array_Length` (`self.Enemies`)) 0)
    (`self.Set Active Pillars` false)
    (`KismetSystemLibrary.Delay` 1.0)
    (`self.TriggerSpawn` false)))

(event `Set Active Pillars`
  (params (Activate :type Boolean))
  (for _array_element (`self.FirePillars`)
    (`/Game/Combat/FilePillar/BP_FirePillar.SetActivate` _array_element Activate)))

(fn `UserConstructionScript`)