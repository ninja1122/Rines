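; BP_Rat is an enemy rat unit that spits projectiles at its blackboard target, gains aggro when damaged and drops a random potion on death.
; Each Tick smoothly turns it toward its movement, or toward the target's velocity-predicted position during one animation state.
; The animation's spit event spawns BP_RatSpit along that direction and cycles a shot counter that sets a stop-shooting flag.
; Random idle sounds play while it lives.
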(event `self.ReceiveBeginPlay`
  (bind _bp_unit (`self.BP_Unit`))
  (add `/Game/Combat/Blueprints/BP_Unit.UnitTookDamage` _bp_unit (delegate `UnitTookDamage`))
  (add `/Game/Combat/Blueprints/BP_Unit.UnitDied` _bp_unit (delegate `UnitDied_`))
  (bind _asanim_bp_rat (cast `/Game/Combat/Rat/AnimBP_Rat` (`SkeletalMeshComponent.GetAnimInstance` (`self.Mesh`))))
  (add `/Game/Combat/Rat/AnimBP_Rat.FireSpitFired` _asanim_bp_rat (delegate `FireSpitFired`))
  (`BlackboardComponent.SetValueAsVector` (`AIBlueprintHelperLibrary.GetBlackboard` (`AIBlueprintHelperLibrary.GetAIController` self)) "SpawnPoint" (`self.K2_GetActorLocation`)))

(event `UnitTookDamage`
  (params (damage :type "Float (double-precision)") (type :type "/Game/Combat/Blueprints/BP_DamageType Enum" :default "NewEnumerator0"))
  (set `/Game/Combat/Blueprints/BP_Unit.hasAggro` true (`self.BP_Unit`)))

(event `UnitDied_`
  (params (Actor :type "Actor Object Reference") (Unit :type "/Game/Combat/Blueprints/BP_Unit Object Reference"))
  (`/Game/BP_GameInstance.SpawnRandomPotion` (`/Game/BP_Functions.GetFakeUpGameInstance`) (`self.K2_GetActorLocation`)))

(event `FireSpitFired`
  (bind _returnvalue (mod (+ (`self.shotCounter`) 1) 6))
  (set `self.shotCounter` _returnvalue)
  (set `self.shouldStopShooting` (< _returnvalue 3))
  (bind _asactor (cast `Actor` (`BlackboardComponent.GetValueAsObject` (`AIBlueprintHelperLibrary.GetBlackboard` (`AIBlueprintHelperLibrary.GetAIController` self)) "TargetActor")))
  (bind _returnvalue_2 (`|SpawnActorFromClass` "/Game/Combat/RatSpit/BP_RatSpit.BP_RatSpit_C" (`KismetMathLibrary.Conv_VectorToTransform` (`SceneComponent.GetSocketLocation` (`self.Mesh`) "SOCKET_Spit")) "Undefined" "OverrideRootScale" null null))
  (`/Game/Combat/RatSpit/BP_RatSpit.Init` _returnvalue_2 (`self.Direction`)))

(event `self.ReceiveTick`
  (params (DeltaSeconds :type "Float (single-precision)"))
  (bind _audio (`self.Audio`))
  (bind _returnvalue (* (`self.Direction`) (1.0 1.0 0.0)))
  (bind _returnvalue_2 (`AIBlueprintHelperLibrary.GetBlackboard` (`AIBlueprintHelperLibrary.GetAIController` self)))
  (`|ExecutionSequence`
    (:`then_0`
      (bind _inprogress (message `/Game/Combat/Blueprints/BP_Stateful.RawIsStateInProgress` (`SkeletalMeshComponent.GetAnimInstance` (`self.Mesh`)) (enumliteral `/Game/Combat/Rat/BP_RatState` "NewEnumerator2")))
      (if (and _inprogress (`BlackboardComponent.GetValueAsBool` _returnvalue_2 "FoundActor"))
        (bind _asactor (cast `Actor` (`BlackboardComponent.GetValueAsObject` _returnvalue_2 "TargetActor"))
          (:`then`
            (bind _returnvalue_3 (- (* (`self.K2_GetActorLocation` _asactor) (1.0 1.0 1.0)) (* (`self.K2_GetActorLocation`) (1.0 1.0 1.0))))
            (set `self.Direction` (`KismetMathLibrary.Normal` (+ _returnvalue_3 (* (`MovementComponent.Velocity` (`self.GetComponentByClass` _asactor "/Script/Engine.CharacterMovementComponent")) (/ (`KismetMathLibrary.VSize` _returnvalue_3) 2500.0))))))
          (:`CastFailed`
            (set `self.Direction` (`KismetMathLibrary.Normal` (`MovementComponent.Velocity` (`self.CharacterMovement`))) :!label _label)))
        (else
          (goto _label))))
    (:`then_1`
      (if (!= (`KismetMathLibrary.VSizeSquared` _returnvalue) 0.0)
        (`self.K2_SetActorRotation` (`KismetMathLibrary.RLerp` (`self.K2_GetActorRotation`) (`KismetMathLibrary.FindLookAtRotation` (`KismetMathLibrary.MakeVector` 0.0) _returnvalue) 0.4 true))))
    (:`then_2`
      (if (`/Game/Combat/Blueprints/BP_Unit.IsAlive` (`self.BP_Unit`))
        (set `self.randomSoundTime` (- (`self.randomSoundTime`) (`GameplayStatics.GetWorldDeltaSeconds`)))
        (if (<= (`self.randomSoundTime`) 0.0)
          (set `self.randomSoundTime` (`KismetMathLibrary.RandomFloatInRange` 1.0 8.0))
          (`AudioComponent.SetSound` _audio (`|GetArrayItem` (`self.randomSounds`) (`KismetMathLibrary.RandomInteger` 2)))
          (`AudioComponent.Play` _audio 0.0))))))

(fn `UserConstructionScript`)