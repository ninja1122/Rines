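; Spell manager component that owns its character's spell set and routes cast, release and channel-cancel requests to it.
; Keeps a map of spell class to spawned caster actor, reusing existing casters when the set changes, destroying removed ones and passing the list to the HUD for cooldowns.
; Blocks new casts while any spell is casting, offers movement, rotation and falling helpers for the owning Character, and serializes each caster.
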(event `self.ReceiveBeginPlay`
  (`self.UpdateSpells`))

(event `SetSpells`
  (params (Spells :type "Array of /Game/Combat/SpellSystem/BP_SpellCaster Class Reference"))
  (`BlueprintMapLibrary.Map_Clear` (`self.newSpells`))
  (set `self.toRemoveSpells` (`self.currentSpells`))
  (for _array_element Spells
    (`BlueprintMapLibrary.Map_Add` (`self.newSpells`) _array_element (`BlueprintMapLibrary.Map_Find` (`self.currentSpells`) _array_element))
    (`BlueprintMapLibrary.Map_Remove` (`self.toRemoveSpells`) _array_element))
  (set `self.currentSpells` (`self.newSpells`))
  (bind _values (`BlueprintMapLibrary.Map_Values` (`self.toRemoveSpells`)))
  (for _array_element_2 _values
    (`Actor.K2_DestroyActor` _array_element_2))
  (`BlueprintMapLibrary.Map_Clear` (`self.toRemoveSpells`))
  (`self.UpdateSpells`))

(event `UpdateSpells`
  (bind _currentspells (`self.currentSpells`))
  (bind _keys (`BlueprintMapLibrary.Map_Keys` _currentspells))
  (bind _values (`BlueprintMapLibrary.Map_Values` _currentspells))
  (for (_ _array_index) _keys
    (`/Engine/EditorBlueprintResources/StandardMacros.IsValid` (`|GetArrayItem` _values _array_index)
      (:`Is Not Valid`
        (bind _output (`|GetArrayItem` _keys _array_index))
        (bind _returnvalue (`|SpawnActorFromClass` _output (`KismetMathLibrary.MakeTransform` (0.0 0.0 0.0)) "Undefined" "OverrideRootScale" null null))
        (`/Game/Combat/SpellSystem/BP_SpellCaster.Init` _returnvalue (`self.GetOwner`) self)
        (`BlueprintMapLibrary.Map_Add` (`self.currentSpells`) _output _returnvalue))))
  (bind _asbp_hud (cast `/Game/Combat/Ui/BP_Hud` (`PlayerController.GetHUD` (`GameplayStatics.GetPlayerController` 0))))
  (bind _values_2 (`BlueprintMapLibrary.Map_Values` (`self.currentSpells`)))
  (`/Game/Combat/Ui/BP_Hud.SetSpellCooldowns` _asbp_hud _values_2))

(event `CastSpell`
  (params (type :type "/Game/Combat/SpellSystem/BP_SpellCaster Class Reference"))
  (bind (_value _returnvalue) (`BlueprintMapLibrary.Map_Find` (`self.currentSpells`) type))
  (if _returnvalue
    (if (not (`self.IsAnySpellCasting`))
      (`/Game/Combat/SpellSystem/BP_SpellCaster.CastSpell` _value))))

(event `ReleaseSpell`
  (params (Type :type "/Game/Combat/SpellSystem/BP_SpellCaster Class Reference"))
  (bind (_value _returnvalue) (`BlueprintMapLibrary.Map_Find` (`self.currentSpells`) Type))
  (if _returnvalue
    (`/Game/Combat/SpellSystem/BP_SpellCaster.ReleaseSpell` _value)))

(event `SetMovementMode`
  (params (Enabled :type Boolean))
  (bind _ascharacter (cast `Character` (`self.GetOwner`)))
  (`CharacterMovementComponent.SetMovementMode` (`Character.CharacterMovement` _ascharacter) (select `bool` Enabled :`false` "MOVE_None" :`true` "MOVE_Walking" :!type "EMovementMode Enum") 0))

(event `RotatePlayer`
  (params (Direction :type "Vector Structure"))
  (bind _ascharacter (cast `Character` (`self.GetOwner`)))
  (`Actor.K2_SetActorRotation` _ascharacter (`KismetMathLibrary.MakeRotator` 0.0 0.0 (.yaw (`KismetMathLibrary.FindLookAtRotation` (`KismetMathLibrary.MakeVector` 0.0 0.0 1.0) Direction))) false))

(event `CancelChannels`
  (bind _values (`BlueprintMapLibrary.Map_Values` (`self.currentSpells`)))
  (for _array_element _values
    (`/Engine/EditorBlueprintResources/StandardMacros.IsValid` _array_element
      (:`Is Valid`
        (if (`|EnumEquality` (`/Game/Combat/SpellSystem/BP_SpellCaster.castPhase` _array_element) "NewEnumerator1")
          (`/Game/Combat/SpellSystem/BP_SpellCaster.CancelSpell` _array_element))))))

(event `self.serialize`
  (params (archive :type "SaveGameArchive Object Reference"))
  (`self.UpdateSpells`)
  (bind _values (`BlueprintMapLibrary.Map_Values` (`self.currentSpells`)))
  (for _array_element _values
    (`SaveGameArchive.serialize` archive _array_element)))

(fn `GetSpellCaster`
  (params (type :type "/Game/Combat/SpellSystem/BP_SpellCaster Class Reference"))
  (returns (spellCaster :type "/Game/Combat/SpellSystem/BP_SpellCaster Object Reference") (found :type Boolean))
  (bind (_value _returnvalue) (`BlueprintMapLibrary.Map_Find` (`self.currentSpells`) type))
  (return _value _returnvalue))

(fn `GetSpells`
  (returns (NewParam :type "Array of /Game/Combat/SpellSystem/BP_SpellCaster Class Reference"))
  (bind _keys (`BlueprintMapLibrary.Map_Keys` (`self.currentSpells`)))
  (return _keys))

(fn `IsAnySpellCasting`
  (returns (IsCasting :type Boolean))
  (bind _values (`BlueprintMapLibrary.Map_Values` (`self.currentSpells`)))
  (for _array_element _values
    (`/Engine/EditorBlueprintResources/StandardMacros.IsValid` _array_element
      (:`Is Valid`
        (if (`|EnumEquality` (`/Game/Combat/SpellSystem/BP_SpellCaster.castPhase` _array_element) "NewEnumerator2")
          (return true)))))
  (return false))

(fn `IsPlayerFalling`
  (returns (IsFalling :type Boolean))
  (bind _ascharacter (cast `Character` (`self.GetOwner`)))
  (return (`NavMovementComponent.IsFalling` (`Character.CharacterMovement` _ascharacter))))