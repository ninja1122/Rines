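; BP_SpellCaster is a base spell actor that provides cooldown, leveling and display text, with empty cast, release, cancel and info functions as apparent override points.
; Init stores the owning player and manager, while Tick counts down the cooldown in the Stats struct that gates IsReady.
; LevelUp spends a development point (PunktyRozwoju) from the player pawn's StatystykiPostaci component.
; Serialize passes the stats, but not Level, through an archive.
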(event `self.ReceiveTick`
  (params (DeltaSeconds :type "Float (single-precision)"))
  (bind (_available _cooldown _maxcooldown _casttime) (break `/Game/Combat/SpellSystem/BP_BasicSpellStats` (`self.stats`)))
  (set `self.stats` (make `/Game/Combat/SpellSystem/BP_BasicSpellStats` _available (`KismetMathLibrary.FClamp` (- _cooldown DeltaSeconds) 0.0 _maxcooldown) _maxcooldown _casttime)))

(event `Init`
  (params (actor :type "Actor Object Reference") (manager :type "/Game/Combat/SpellSystem/BP_SpellManager Object Reference"))
  (set `self.ownerPlayer` actor)
  (set `self.ownerManager` manager))

(event `self.serialize`
  (params (archive :type "SaveGameArchive Object Reference"))
  (bind (_stats_available _stats_cooldown _stats_maxcooldown _stats_casttime) (break `/Game/Combat/SpellSystem/BP_BasicSpellStats` (`self.stats`)))
  (`SaveGameArchive.serializeBool` archive _stats_available)
  (`SaveGameArchive.serializeFloat` archive _stats_cooldown)
  (`SaveGameArchive.serializeFloat` archive _stats_maxcooldown)
  (`SaveGameArchive.serializeFloat` archive _stats_casttime))

(fn `CancelSpell`)

(fn `CastSpell`)

(fn `GetSpellCooldownInfo`
  (params (ForNextLevel :type Boolean))
  (returns (CooldownText :type Text))
  (bind (_stats_available _stats_cooldown _stats_maxcooldown) (break `/Game/Combat/SpellSystem/BP_BasicSpellStats` (`self.stats`)))
  (return (`|FormatText` "{Cooldown}s" _stats_maxcooldown)))

(fn `GetSpellInfo`
  (params (ForNextLevel :type Boolean))
  (returns (Text :type Text))
  (return ""))

(fn `GetSpellNameWithLevel`
  (params (ForNextLevel :type Boolean))
  (returns (Name :type Text))
  (bind _level (`self.level`))
  (bind _returnvalue (`Helpers.convertToRomanNumeral` (select `bool` ForNextLevel :`false` _level :`true` (+ _level 1))))
  (return (`|FormatText` "{Name} {Level}" (`self.name`) _returnvalue)))

(fn `isReady`
  (returns (ready :type Boolean))
  (return (<= (`.cooldown_6_9218338C49683BA5F0C657BCAB803BA3` (break `/Game/Combat/SpellSystem/BP_BasicSpellStats` (`self.stats`))) 0.0)))

(fn `LevelUp`
  (bind _punktyrozwoju (`StatystykiPostaci.punktyRozwoju` (`self.GetComponentByClass` (`GameplayStatics.GetPlayerPawn` 0) "/Script/Projekt_2_Rok.StatystykiPostaci")))
  (if (> _punktyrozwoju 0)
    (`/Engine/EditorBlueprintResources/StandardMacros.DecrementInt` _punktyrozwoju
      (:`  `
        (`/Engine/EditorBlueprintResources/StandardMacros.IncrementInt` (`self.level`))))))

(fn `ReleaseSpell`)

(fn `SetMaxCooldown`
  (bind (_available _cooldown _maxcooldown _casttime) (break `/Game/Combat/SpellSystem/BP_BasicSpellStats` (`self.stats`)))
  (set `self.stats` (make `/Game/Combat/SpellSystem/BP_BasicSpellStats` _available _maxcooldown _maxcooldown _casttime)))

(fn `UserConstructionScript`)