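; BP_Batman is a flying, AI-controlled enemy that spits BP_RatSpit projectiles at its blackboard target, and its death advances a mission part.
; Animation-driven shots spawn projectiles, while Tick smooths rotation toward target or velocity and briefly lifts it depending on animation state.
; Echo triggers every Kostek spawner in low-health mode and restarts a curve-driven intensity fade on a dynamic material blended into the tagged post-process volume.
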(event `self.ReceiveBeginPlay`
  (bind _bp_unit (`self.BP_Unit`))
  (bind _asanim_bp_batman (cast `/Game/Combat/Batman/AnimBP_Batman` (`SkeletalMeshComponent.GetAnimInstance` (`self.Mesh`))))
  (add `/Game/Combat/Batman/AnimBP_Batman.Shot` _asanim_bp_batman (delegate `Shot`))
  (add `/Game/Combat/Blueprints/BP_Unit.UnitTookDamage` _bp_unit (delegate `TookDamage`))
  (add `/Game/Combat/Blueprints/BP_Unit.UnitDied` _bp_unit (delegate `Died`))
  (bind _outactors (`GameplayStatics.GetAllActorsOfClass` "/Game/Combat/Batman/BP_BatPoint.BP_BatPoint_C"))
  (set `self.points` _outactors)
  (bind _outactors_2 (`GameplayStatics.GetAllActorsOfClass` "/Game/Combat/Spawners/BP_KostekSpawner.BP_KostekSpawner_C"))
  (set `self.kostekSpawners` _outactors_2)
  (bind _outactors_3 (`GameplayStatics.GetAllActorsWithTag` "BatPostProcess"))
  (bind _aspost_process_volume (cast `PostProcessVolume` (`|GetArrayItem` _outactors_3))
    (:`then`
      (set `self.postProcessVolume` _aspost_process_volume))
    (:`CastFailed`
      _))
  (`CharacterMovementComponent.SetMovementMode` (`self.CharacterMovement`) "MOVE_Flying" 0)
  (bind _returnvalue (`KismetMaterialLibrary.CreateDynamicMaterialInstance` "/Game/Combat/Batman/MAT_BatManPostProcess.MAT_BatManPostProcess"))
  (bind _output_get (set `self.postProcessMaterial` _returnvalue))
  (`PostProcessVolume.AddOrUpdateBlendable` (`self.postProcessVolume`) _output_get 1.0)
  (`BlackboardComponent.SetValueAsVector` (`AIBlueprintHelperLibrary.GetBlackboard` (`AIBlueprintHelperLibrary.GetAIController` self)) "SpawnPosition" (`self.K2_GetActorLocation`)))

(event `Shot`
  (bind _returnvalue (`SceneComponent.GetSocketLocation` (`self.Mesh`) "SOCKET_Spit"))
  (bind _output_get (set `self.shotCounter` (mod (+ (`self.shotCounter`) 1) 2)))
  (set `self.shouldStopShooting` (== _output_get 0))
  (bind _asactor (cast `Actor` (`BlackboardComponent.GetValueAsObject` (`AIBlueprintHelperLibrary.GetBlackboard` (`AIBlueprintHelperLibrary.GetAIController` self)) "TargetActor")))
  (bind _returnvalue_2 (`|SpawnActorFromClass` "/Game/Combat/RatSpit/BP_RatSpit.BP_RatSpit_C" (`KismetMathLibrary.Conv_VectorToTransform` _returnvalue) "Undefined" "OverrideRootScale" null null))
  (set `/Game/Combat/RatSpit/BP_RatSpit.LeaveFire` true _returnvalue_2)
  (`/Game/Combat/RatSpit/BP_RatSpit.Init` _returnvalue_2 (`KismetMathLibrary.Normal` (- (`self.K2_GetActorLocation` _asactor) _returnvalue))))

(event `TookDamage`
  (params (damage :type "Float (double-precision)") (type :type "/Game/Combat/Blueprints/BP_DamageType Enum" :default "NewEnumerator0"))
  (set `/Game/Combat/Blueprints/BP_Unit.hasAggro` true (`self.BP_Unit`)))

(event `Died`
  (params (Actor :type "Actor Object Reference") (Unit :type "/Game/Combat/Blueprints/BP_Unit Object Reference"))
  (`/Game/BP_GameInstance.SetMissionPart` (`/Game/BP_Functions.GetFakeUpGameInstance`) 3 4))

(event `Echo`
  (set `self.echoTime` 0.0)
  (for _array_element (`self.kostekSpawners`)
    (set `/Game/Combat/Spawners/BP_KostekSpawner.lowHealth` true _array_element)
    (`/Game/Combat/Spawners/BP_Spawner.Trigger Spawn` _array_element)))

(event `self.ReceiveTick`
  (params (DeltaSeconds :type "Float (single-precision)"))
  (`self.GetDirection`)
  (`self.RotateToDirectiion`)
  (`self.UpdatePostProcess`)
  (bind _asanim_bp_batman (cast `/Game/Combat/Batman/AnimBP_Batman` (`SkeletalMeshComponent.GetAnimInstance` (`self.Mesh`))))
  (if (`|EnumInequality` (`/Game/Combat/Batman/AnimBP_Batman.state` _asanim_bp_batman) "NewEnumerator3")
    (bind _output_get (set `self.moveStart` (+ (`self.moveStart`) (`GameplayStatics.GetWorldDeltaSeconds`))))
    (if (< _output_get 1.0)
      (`self.K2_SetActorLocation` (+ (`self.K2_GetActorLocation`) (* (0.0 0.0 100.0) (`GameplayStatics.GetWorldDeltaSeconds`)))))))

(event `GetDirection`
  (bind _inprogress (message `/Game/Combat/Blueprints/BP_Stateful.RawIsStateInProgress` (`SkeletalMeshComponent.GetAnimInstance` (`self.Mesh`)) (enumliteral `/Game/Combat/Batman/BP_BatManState` "NewEnumerator1")))
  (if _inprogress
    (bind _asactor (cast `Actor` (`BlackboardComponent.GetValueAsObject` (`AIBlueprintHelperLibrary.GetBlackboard` (`AIBlueprintHelperLibrary.GetAIController` self)) "TargetActor"))
      (:`then`
        (set `self.direction` (`KismetMathLibrary.Normal` (- (`self.K2_GetActorLocation` _asactor) (`SceneComponent.GetSocketLocation` (`self.Mesh`) "SOCKET_Spit")))))
      (:`CastFailed`
        (set `self.direction` (`MovementComponent.Velocity` (`self.CharacterMovement`)) :!label _label)))
    (else
      (goto _label))))

(event `RotateToDirectiion`
  (bind _direction (`self.direction`))
  (if (!= (`KismetMathLibrary.VSizeSquared` _direction) 0.0)
    (`self.K2_SetActorRotation` (`KismetMathLibrary.RLerp` (`self.K2_GetActorRotation`) (`KismetMathLibrary.FindLookAtRotation` (`KismetMathLibrary.MakeVector` 0.0) _direction) 0.4 true))))

(event `UpdatePostProcess`
  (set `self.echoTime` (+ (`self.echoTime`) (/ (`GameplayStatics.GetWorldDeltaSeconds`) 10.0)))
  (`MaterialInstanceDynamic.SetScalarParameterValue` (`self.postProcessMaterial`) "intensity" (`CurveFloat.GetFloatValue` (`self.curve`) (`KismetMathLibrary.FClamp` (`self.echoTime`)))))

(fn `UserConstructionScript`)