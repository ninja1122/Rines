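; BP_Unit is a combat component giving its owning actor health, damage, healing with optional resurrection, and death/resurrection events.
; Deaths of one unit class award Exp to the player's StatystykiPostaci component.
; Tick counts down a crowd-control stack that toggles Character movement or, once dead, feeds DeathTime into dynamic materials created at BeginPlay for all but one class.
; A Serialize event archives health and alive state.
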(event `Take Damage`
  (params (damage :type "Float (double-precision)") (type :type "/Game/Combat/Blueprints/BP_DamageType Enum" :default "NewEnumerator0"))
  (bind _isalive (`self.IsAlive`))
  (bind (_current _maximum) (break `/Game/Combat/Blueprints/BP_UnitHealth` (`self.health`)))
  (if (`self.canTakeDamage`)
    (set `self.health` (make `/Game/Combat/Blueprints/BP_UnitHealth` (`KismetMathLibrary.FMax` (- _current damage)) _maximum))
    (`self.UnitTookDamage` damage type)
    (if (not (== _isalive (`self.wasAlive`)))
      (`self.UnitDied` (`self.GetOwner`) self)
      (set `self.wasAlive` _isalive)
      (if (`|EnumEquality` (`self.unitClass`) "NewEnumerator1")
        (`StatystykiPostaci.DodajDoswiadczenie` (`Actor.GetComponentByClass` (`GameplayStatics.GetPlayerCharacter` 0) "/Script/Projekt_2_Rok.StatystykiPostaci") (`self.exp`))))))

(event `Heal`
  (params (HealAmount :type "Float (double-precision)") (RessurectIfNeeded :type Boolean :default false))
  (bind _isalive (`self.IsAlive`))
  (bind (_current _maximum) (break `/Game/Combat/Blueprints/BP_UnitHealth` (`self.health`)))
  (if (`self.IsAlive`)
    (set `self.health` (make `/Game/Combat/Blueprints/BP_UnitHealth` (`KismetMathLibrary.FMin` (+ _current HealAmount) _maximum) _maximum) :!label _label)
    (if (not (== _isalive (`self.wasAlive`)))
      (`self.UnitRessurected`)
      (set `self.wasAlive` _isalive))
    (elif RessurectIfNeeded
      (goto _label))))

(event `self.ReceiveBeginPlay`
  (bind _returnvalue (`Actor.GetComponentByClass` (`self.GetOwner`) "/Script/Engine.PrimitiveComponent"))
  (if (`|EnumInequality` (`self.unitClass`) "NewEnumerator0")
    (`/Engine/EditorBlueprintResources/StandardMacros.IsValid` _returnvalue
      (:`Is Valid`
        (for _index (range (`PrimitiveComponent.GetNumMaterials` _returnvalue))
          (bind _returnvalue_2 (`PrimitiveComponent.CreateDynamicMaterialInstance` _returnvalue _index (`PrimitiveComponent.GetMaterial` _returnvalue _index) "None"))
          (`KismetArrayLibrary.Array_Add` (`self.material`) _returnvalue_2))))))

(event `self.ReceiveTick`
  (params (DeltaSeconds :type "Float (single-precision)"))
  (if (`self.IsAlive`)
    (`self.UpdateCrowdControls`)
    (else
      (set `self.deathTime` (+ (`self.deathTime`) DeltaSeconds))
      (`self.UpdateMaterials`))))

(event `ApplyCrowdControl`
  (params (Type :type "/Game/Combat/Blueprints/BP_CrowdControlType Enum" :default "NewEnumerator0") (Duration :type "Float (double-precision)"))
  (`KismetArrayLibrary.Array_Add` (`self.crowdControlStack`) (make `/Game/Combat/Blueprints/BP_CrowdControlEntry` Type Duration))
  (switch `/Game/Combat/Blueprints/BP_CrowdControlType` Type
    (:`NewEnumerator0`
      (bind _ascharacter (cast `Character` (`self.GetOwner`)))
      (`CharacterMovementComponent.SetMovementMode` (`Character.CharacterMovement` _ascharacter) "MOVE_None" 0))))

(event `DisableCrowdControl`
  (params (Type :type "/Game/Combat/Blueprints/BP_CrowdControlType Enum" :default "NewEnumerator0"))
  (switch `/Game/Combat/Blueprints/BP_CrowdControlType` Type
    (:`NewEnumerator0`
      (bind _ascharacter (cast `Character` (`self.GetOwner`)))
      (`CharacterMovementComponent.SetMovementMode` (`Character.CharacterMovement` _ascharacter) "MOVE_Walking" 0))))

(event `UpdateMaterials`
  (for _array_element (`self.material`)
    (`MaterialInstanceDynamic.SetScalarParameterValue` _array_element "DeathTime" (`KismetMathLibrary.FClamp` (`self.deathTime`) 0.0 5.0))))

(event `UpdateCrowdControls`
  (bind _crowdcontrolstack (`self.crowdControlStack`))
  (bind _returnvalue (`KismetArrayLibrary.Array_Length` _crowdcontrolstack))
  (for (_array_element _array_index) _crowdcontrolstack
    (bind (_type _duration) (break `/Game/Combat/Blueprints/BP_CrowdControlEntry` _array_element))
    (`KismetArrayLibrary.Array_Set` (`self.crowdControlStack`) _array_index (make `/Game/Combat/Blueprints/BP_CrowdControlEntry` _type (- _duration (`GameplayStatics.GetWorldDeltaSeconds`)))))
  (if (> _returnvalue 0)
    (for _index (range (- _returnvalue 1) 1)
      (bind (_type_2 _duration_2) (break `/Game/Combat/Blueprints/BP_CrowdControlEntry` (`|GetArrayItem` (`self.crowdControlStack`) _index)))
      (if (<= _duration_2 0.0)
        (`self.DisableCrowdControl` _type_2)
        (`KismetArrayLibrary.Array_Remove` (`self.crowdControlStack`) _index)))))

(event `self.Serialize`
  (params (archive :type "SaveGameArchive Object Reference"))
  (bind (_health_current _health_maximum) (break `/Game/Combat/Blueprints/BP_UnitHealth` (`self.health`)))
  (`SaveGameArchive.serializeFloat` archive _health_current)
  (`SaveGameArchive.serializeFloat` archive _health_maximum)
  (`SaveGameArchive.serializeBool` archive (`self.wasAlive`)))

(fn `CanMove`
  (returns (CanMove :type Boolean))
  (bind _ascharacter (cast `Character` (`self.GetOwner`)))
  (return (`|EnumInequality` (`CharacterMovementComponent.MovementMode` (`Character.CharacterMovement` _ascharacter)) "MOVE_None")))

(fn `IsAlive`
  (returns (IsAlive :type Boolean))
  (return (> (`.current_4_1115F832448A02AAC2FE9296550DBD47` (break `/Game/Combat/Blueprints/BP_UnitHealth` (`self.health`))) 0.0)))