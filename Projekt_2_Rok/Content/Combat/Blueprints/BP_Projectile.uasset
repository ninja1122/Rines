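; Actor component that drives its owner as a combat projectile, using the owner's ProjectileMovementComponent.
; Init events aim the owner along a direction or at a camera-traced target, then launch it at Speed.
; Overlaps and hits, unless Passthrough, trigger the destroy event, which optionally spawns an actor and fires OnProjectileDestroyed without destroying the owner itself.
; Tick estimates travel from Speed, stopping or triggering that event at the range limit.
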(event `self.ReceiveBeginPlay`
  (bind _returnvalue (`self.GetOwner`))
  (set `self.particleMovement` (`|ConvertAsset` (`Actor.GetComponentByClass` _returnvalue "/Script/Engine.ProjectileMovementComponent")))
  (if (not (`self.passthrough`))
    (add `Actor.OnActorBeginOverlap` _returnvalue (delegate `CustomEvent_0`))
    (add `Actor.OnActorHit` _returnvalue (delegate `EventHit`))))

(event `CustomEvent_0`
  (params (OverlappedActor :type "Actor Object Reference") (OtherActor :type "Actor Object Reference"))
  (`self.DestoyProjectile` (`|ConvertAsset` OtherActor)))

(event `EventHit`
  (params (SelfActor :type "Actor Object Reference") (OtherActor :type "Actor Object Reference") (NormalImpulse :type "Vector Structure") (Hit :type "HitResult Structure (by ref)"))
  (`self.DestoyProjectile` (`|ConvertAsset` OtherActor)))

(event `InitCameraTargettedProjectile`
  (params (start :type "Vector Structure") (cameraPosition :type "Vector Structure") (cameraDirection :type "Vector Structure"))
  (bind _output (`|ConvertAsset` (`self.particleMovement`)))
  (bind _returnvalue (`Helpers.findProjectileTargetPosition` start (`self.distance`) (+ cameraPosition cameraDirection) cameraDirection (`self.traceChannel`)))
  (`Actor.K2_SetActorRotation` (`self.GetOwner`) (`KismetMathLibrary.FindLookAtRotation` start _returnvalue) false)
  (`/Engine/EditorBlueprintResources/StandardMacros.IsValid` _output
    (:`Is Valid`
      (`ProjectileMovementComponent.SetVelocityInLocalSpace` _output (`KismetMathLibrary.MakeVector` (`self.speed`)))
      (set `self.enabled` true))))

(event `InitForwardProjectile`
  (params (start :type "Vector Structure") (direction :type "Vector Structure"))
  (bind _output (`|ConvertAsset` (`self.particleMovement`)))
  (`Actor.K2_SetActorRotation` (`self.GetOwner`) (`KismetMathLibrary.FindLookAtRotation` start (+ start (* direction 100.0))) false)
  (`/Engine/EditorBlueprintResources/StandardMacros.IsValid` _output
    (:`Is Valid`
      (`ProjectileMovementComponent.SetVelocityInLocalSpace` _output (`KismetMathLibrary.MakeVector` (`self.speed`)))
      (set `self.enabled` true))))

(event `self.ReceiveTick`
  (params (DeltaSeconds :type "Float (single-precision)"))
  (if (`self.enabled`)
    (bind _output_get (set `self.travelledDistance` (+ (`self.travelledDistance`) (* (`self.speed`) DeltaSeconds))))
    (if (>= _output_get (`self.distance`))
      (if (`self.disableOnRangeLimit`)
        (set `self.enabled` false)
        (`ProjectileMovementComponent.SetVelocityInLocalSpace` (`|ConvertAsset` (`self.particleMovement`)) (0.0 0.0 0.0))
        (else
          (`self.DestoyProjectile` null))))))

(event `DestoyProjectile`
  (params (ColidedWith :type "Actor Soft Object Reference"))
  (bind _spawn (`self.spawn`))
  (if (!= _spawn null)
    (`|SpawnActorFromClass` _spawn (`KismetMathLibrary.Conv_VectorToTransform` (`Actor.K2_GetActorLocation` (`self.GetOwner`))) "Undefined" "OverrideRootScale" null null))
  (`self.OnProjectileDestroyed` ColidedWith))