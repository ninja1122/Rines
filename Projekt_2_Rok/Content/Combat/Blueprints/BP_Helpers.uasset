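; BP_Helpers is a collection of shared combat helper functions for health, damage, level scaling and ragdolls.
; DealDamageInSphere overlaps one object type and calls TakeDamage on actors whose BP_Unit component matches the given UnitClass.
; Evaluate scales a base value linearly per level, and EvaluateString formats it as rich text, optionally previewing the next level.
; SetRagdollEnabled toggles mesh physics, collision and character movement mode together.
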(fn `DealDamageInSphere`
  (params (position :type "Vector Structure") (radius :type "Float (double-precision)") (damage :type "Float (double-precision)") (type :type "/Game/Combat/Blueprints/BP_DamageType Enum" :default "NewEnumerator0") (class :type "/Game/Combat/Blueprints/BP_UnitClass Enum" :default "NewEnumerator0"))
  (bind _outactors (`KismetSystemLibrary.SphereOverlapActors` null position radius (`|MakeArray` "ObjectTypeQuery8" :!type "EObjectTypeQuery Enum")))
  (for _array_element _outactors
    (bind _returnvalue (`Actor.GetComponentByClass` _array_element "/Game/Combat/Blueprints/BP_Unit.BP_Unit_C"))
    (`/Engine/EditorBlueprintResources/StandardMacros.IsValid` _returnvalue
      (:`Is Valid`
        (if (`|EnumEquality` (`/Game/Combat/Blueprints/BP_Unit.unitClass` _returnvalue) class)
          (`/Game/Combat/Blueprints/BP_Unit.Take Damage` _returnvalue damage type))))))

(fn `Evaluate`
  (params (In :type "/Game/Combat/Blueprints/BP_LevelableFloat Structure") (Level :type Integer))
  (returns (Out :type "Float (double-precision)"))
  (return (+ In_Base_4_3EE1AC5A4E35BE8D0549C9A91F482264 (* (- Level 1) In_PerLevel_5_68E3078D42768AC62A3C7B9AA3FAD9BB))))

(fn `EvaluateString`
  (params (In :type "/Game/Combat/Blueprints/BP_LevelableFloat Structure") (Level :type Integer) (ForNextLevel :type Boolean))
  (returns (Text :type Text))
  (if (and ForNextLevel (!= (`.PerLevel_5_68E3078D42768AC62A3C7B9AA3FAD9BB` (break `/Game/Combat/Blueprints/BP_LevelableFloat` In)) 0.0))
    (return (`|FormatText` "<damage>{Damage} </>(<perLevel>{PerLevel}</>)" (`self.Evaluate` In (+ Level 1)) (`KismetTextLibrary.Conv_DoubleToText` (`.PerLevel_5_68E3078D42768AC62A3C7B9AA3FAD9BB` (break `/Game/Combat/Blueprints/BP_LevelableFloat` In)) "HalfToEven" true true 1 324 0 2)))
    (else
      (return (`|FormatText` "<damage>{Damage}</>" (`self.Evaluate` In Level))))))

(fn `GetPercentageHealth`
  (params (health :type "/Game/Combat/Blueprints/BP_UnitHealth Structure"))
  (returns (percentage :type "Float (double-precision)"))
  (bind (_current _maximum) (break `/Game/Combat/Blueprints/BP_UnitHealth` health))
  (if (!= _maximum 0.0)
    (return (/ _current _maximum))
    (else
      (return 0.0))))

(fn `SetRagdollEnabled`
  (params (Mesh :type "SkeletalMeshComponent Object Reference") (CharacterMovement :type "CharacterMovementComponent Object Reference") (Enable :type Boolean :default true))
  (`SkeletalMeshComponent.SetAllBodiesSimulatePhysics` Mesh Enable)
  (`PrimitiveComponent.SetSimulatePhysics` Mesh Enable)
  (`SkeletalMeshComponent.SetEnablePhysicsBlending` Mesh Enable)
  (`PrimitiveComponent.WakeAllRigidBodies` Mesh)
  (set `SkeletalMeshComponent.PhysicsTransformUpdateMode` (select `bool` Enable :`false` "ComponentTransformIsKinematic" :`true` "SimulationUpatesComponentTransform" :!type "EPhysicsTransformUpdateMode Enum") Mesh)
  (`PrimitiveComponent.SetCollisionEnabled` Mesh (select `bool` Enable :`false` "NoCollision" :`true` "QueryAndPhysics" :!type "ECollisionEnabled Enum"))
  (`CharacterMovementComponent.SetMovementMode` CharacterMovement (select `bool` Enable :`false` "MOVE_Walking" :`true` "MOVE_None" :!type "EMovementMode Enum") 0))