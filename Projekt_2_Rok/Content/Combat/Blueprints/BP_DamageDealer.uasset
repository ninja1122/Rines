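; Component that damages units of a target class that overlap its owning actor, either once or periodically.
; With zero TickRate, each actor is hit once on overlap, optionally via a Parent dealer that keeps the hit record.
; With positive TickRate, Tick accumulates time and damages all tracked overlapping units each interval.
; Periodic hits use a fixed damage type rather than the Type variable; both modes require the component to be active.
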(event `self.ReceiveBeginPlay`
  (bind _returnvalue (`self.GetOwner`))
  (add `Actor.OnActorBeginOverlap` _returnvalue (delegate `EventOverlap2`))
  (add `Actor.OnActorEndOverlap` _returnvalue (delegate `EventEndOverlap2`)))

(event `EventOverlap2`
  (params (OverlappedActor :type "Actor Object Reference") (OtherActor :type "Actor Object Reference"))
  (bind _parent (`self.parent`))
  (`BlueprintSetLibrary.Set_Add` (`self.overlappedUnits`) (`Actor.GetComponentByClass` OtherActor "/Game/Combat/Blueprints/BP_Unit.BP_Unit_C"))
  (`/Engine/EditorBlueprintResources/StandardMacros.IsValid` _parent
    (:`Is Valid`
      (`self.DamageActor` _parent OtherActor))
    (:`Is Not Valid`
      (if (not (`self.useParent`))
        (`self.DamageActor` OtherActor)))))

(event `EventEndOverlap2`
  (params (OverlappedActor :type "Actor Object Reference") (OtherActor :type "Actor Object Reference"))
  (`BlueprintSetLibrary.Set_Remove` (`self.overlappedUnits`) (`Actor.GetComponentByClass` OtherActor "/Game/Combat/Blueprints/BP_Unit.BP_Unit_C")))

(event `DamageActor`
  (params (Actor :type "Actor Object Reference"))
  (bind _returnvalue (`Actor.GetComponentByClass` Actor "/Game/Combat/Blueprints/BP_Unit.BP_Unit_C"))
  (bind _output (`|ConvertAsset` Actor))
  (if (and (`self.IsActive`) (== (`self.tickRate`) 0.0))
    (if (not (`BlueprintSetLibrary.Set_Contains` (`self.damageDealtTo`) _output))
      (`/Engine/EditorBlueprintResources/StandardMacros.IsValid` _returnvalue
        (:`Is Valid`
          (if (`|EnumEquality` (`/Game/Combat/Blueprints/BP_Unit.unitClass` _returnvalue) (`self.damagedUnitClass`))
            (`/Game/Combat/Blueprints/BP_Unit.Take Damage` _returnvalue (`self.damage`) (`self.type`))
            (`BlueprintSetLibrary.Set_Add` (`self.damageDealtTo`) _output)))))))

(event `self.ReceiveTick`
  (params (DeltaSeconds :type "Float (single-precision)"))
  (if (`self.IsActive`)
    (if (> (`self.tickRate`) 0.0)
      (bind _output_get (set `self.currentTickTime` (+ (`self.currentTickTime`) (`GameplayStatics.GetWorldDeltaSeconds`))))
      (if (>= _output_get (`self.tickRate`))
        (set `self.currentTickTime` (- (`self.currentTickTime`) (`self.tickRate`)))
        (bind _result (`BlueprintSetLibrary.Set_ToArray` (`self.overlappedUnits`)))
        (for _array_element _result
          (`/Engine/EditorBlueprintResources/StandardMacros.IsValid` _array_element
            (:`Is Valid`
              (if (`|EnumEquality` (`/Game/Combat/Blueprints/BP_Unit.unitClass` _array_element) (`self.damagedUnitClass`))
                (`/Game/Combat/Blueprints/BP_Unit.Take Damage` _array_element (`self.damage`) "NewEnumerator0")))))))))