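; Teleport spell that moves the owning character a level-scaled distance along its movement input, or camera forward when idle, flattened to horizontal.
; On cast it sets the level-based cooldown, triggers camera follow and spawns a world-fixed particle effect.
; A forward capsule trace stops at obstacles, then a downward trace must find ground before the character relocates, so cooldown applies even without movement.
; Also supplies Polish tooltip and cooldown text.
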(event `self.CastSpell`
  (bind (_stats_available _stats_cooldown _stats_maxcooldown _stats_casttime) (break `/Game/Combat/SpellSystem/BP_BasicSpellStats` (`self.stats`)))
  (bind _returnvalue (`self.GetComponentByClass` (`self.character`) "/Script/Engine.CapsuleComponent"))
  (bind _returnvalue_2 (+ (`self.K2_GetActorLocation` (`self.character`)) (`KismetMathLibrary.MakeVector` 0.0)))
  (bind _returnvalue_3 (/ (`CapsuleComponent.CapsuleRadius` (`self.GetComponentByClass` (`self.character`) "/Script/Engine.CapsuleComponent")) 2.0))
  (bind _returnvalue_4 (/ (`CapsuleComponent.CapsuleRadius` _returnvalue) 2.0))
  (if (`self.isReady`)
    (set `self.stats` (make `/Game/Combat/SpellSystem/BP_BasicSpellStats` _stats_available _stats_cooldown (`/Game/Combat/Blueprints/BP_Helpers.Evaluate` (`self.cooldown_0`) (`self.level`)) _stats_casttime))
    (`self.SetMaxCooldown`)
    (bind _asthird_person_character (cast `/Game/ThirdPersonCPP/Blueprints/ThirdPersonCharacter` (`self.ownerPlayer`)))
    (`/Game/ThirdPersonCPP/Blueprints/ThirdPersonCharacter.MakeCameraFollow` _asthird_person_character)
    (set `self.evaluatedDistance` (* (`/Game/Combat/Blueprints/BP_Helpers.Evaluate` (`self.distance`) (`self.level`)) 100.0))
    (bind _ascharacter (cast `Character` (`self.ownerPlayer`)))
    (bind _mesh (`Character.Mesh` _ascharacter))
    (bind (_returnvalue_location _returnvalue_rotation) (`KismetMathLibrary.BreakTransform` (`SceneComponent.K2_GetComponentToWorld` _mesh)))
    (bind _returnvalue_5 (`NiagaraFunctionLibrary.SpawnSystemAttached` "/Game/Combat/Teleport/PS_TeleportSystem.PS_TeleportSystem" _mesh "None" _returnvalue_location _returnvalue_rotation "KeepRelativeOffset"))
    (`SceneComponent.SetAbsolute` _returnvalue_5 true true false)
    (bind _ascharacter_2 (cast `Character` (`self.ownerPlayer`)))
    (set `self.character` _ascharacter_2)
    (`self.GetTeleportDirection`)
    (bind (_outhit _returnvalue_6) (`KismetSystemLibrary.CapsuleTraceSingle` _returnvalue_2 (+ _returnvalue_2 (* (`self.teleportDirection`) (`self.evaluatedDistance`))) _returnvalue_3 _returnvalue_3 "TraceTypeQuery3"))
    (bind (_bblockinghit _binitialoverlap _time _distance _location _impactpoint _normal) (`GameplayStatics.BreakHitResult` _outhit))
    (bind _returnvalue_7 (select `bool` _returnvalue_6 :`false` (+ (`self.K2_GetActorLocation` (`self.character`)) (* (`self.teleportDirection`) (`self.evaluatedDistance`))) :`true` (+ _location (* _normal _returnvalue_4))))
    (bind (_outhit_2 _returnvalue_8) (`KismetSystemLibrary.CapsuleTraceSingle` _returnvalue_7 (+ _returnvalue_7 (0.0 0.0 -300.0)) _returnvalue_4 _returnvalue_4 "TraceTypeQuery3"))
    (if _returnvalue_8
      (`self.K2_SetActorLocation` (`self.character`) (+ (`.Location` (`GameplayStatics.BreakHitResult` _outhit_2)) (`KismetMathLibrary.MakeVector` 0.0 0.0 (+ _returnvalue_4 (`CapsuleComponent.CapsuleHalfHeight` _returnvalue)))) false true))))

(event `GetTeleportDirection`
  (bind _returnvalue (`PawnMovementComponent.GetLastInputVector` (`Character.CharacterMovement` (`self.character`))))
  (set `self.teleportDirection` (`KismetMathLibrary.Normal` (`KismetMathLibrary.MakeVector` (.x (select `bool` (>= (`KismetMathLibrary.VSizeSquared` _returnvalue) 0.1) :`false` (`self.GetActorForwardVector` (`GameplayStatics.GetPlayerCameraManager` 0)) :`true` (`KismetMathLibrary.Normal` _returnvalue))) (.y (select `bool` (>= (`KismetMathLibrary.VSizeSquared` _returnvalue) 0.1) :`false` (`self.GetActorForwardVector` (`GameplayStatics.GetPlayerCameraManager` 0)) :`true` (`KismetMathLibrary.Normal` _returnvalue)))))))

(fn `GetSpellCooldownInfo`
  (params (ForNextLevel :type Boolean))
  (returns (CooldownText :type Text))
  (return (`|FormatText` "{Cooldown}s" (`/Game/Combat/Blueprints/BP_Helpers.EvaluateString` (`self.cooldown_0`) (`self.level`) ForNextLevel))))

(fn `GetSpellInfo`
  (params (ForNextLevel :type Boolean))
  (returns (Text :type Text))
  (bind _name (`/Game/BP_Functions.GetKeyName` "Teleport"))
  (return (`|FormatText` "Wciśnij {key} aby skorzystać z teleportu. Przenosi postać o {Distance} metrów w kierunku poruszania się." _name (`/Game/Combat/Blueprints/BP_Helpers.EvaluateString` (`self.distance`) (`self.level`) ForNextLevel))))

(fn `UserConstructionScript`
  (`parent.UserConstructionScript`))