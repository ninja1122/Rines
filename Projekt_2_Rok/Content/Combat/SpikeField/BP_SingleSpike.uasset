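; A single spike of a spike field combat hazard that rises, lingers for a lifetime, then sinks and destroys itself.
; Tick interpolates the skeletal mesh's height at constant speed and switches to hiding when the timer expires, opening the spikes through AnimBP_Spikes.
; The Collided event closes the spikes in the anim blueprint, restarts the timer and extends the lifetime.
; Construction offsets the meshes vertically and links the damage dealer to a parent dealer.
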(event `self.ReceiveBeginPlay`
  (bind _asanim_bp_spikes (cast `/Game/Combat/SpikeField/xd/AnimBP_Spikes` (`SkeletalMeshComponent.GetAnimInstance` (`self.SM_Kolce_zapadanie`))))
  (set `self.animBp` _asanim_bp_spikes))

(event `self.ReceiveTick`
  (params (DeltaSeconds :type "Float (single-precision)"))
  (bind _hiding (`self.hiding`))
  (set `self.time` (+ (`self.time`) (`GameplayStatics.GetWorldDeltaSeconds`)))
  (`SceneComponent.K2_SetRelativeLocation` (`self.SM_Kolce_zapadanie`) (`KismetMathLibrary.MakeVector` 0.0 0.0 (`KismetMathLibrary.FInterpTo_Constant` (.z (.location (`SceneComponent.GetRelativeTransform` (`self.SM_Kolce_zapadanie`)))) (+ (`self.yPosition`) (select `bool` _hiding :`false` (select `bool` (`self.wasCollided`) :`false` 100.0 :`true` 100.0 :!type "Float (single-precision)") :`true` -120.0)) (`GameplayStatics.GetWorldDeltaSeconds`) (select `bool` _hiding :`false` 1000.0 :`true` 720.0 :!type "Float (single-precision)"))) false false)
  (if (`self.hiding`)
    (if (>= (`self.time`) (+ (`self.lifeTime`) 1.0))
      (`self.K2_DestroyActor`))
    (elif (>= (`self.time`) (`self.lifeTime`))
      (set `self.hiding` true)
      (set `/Game/Combat/SpikeField/xd/AnimBP_Spikes.closedSpikes` false (`self.animBp`)))))

(event `Collided`
  (set `self.wasCollided` true)
  (set `/Game/Combat/SpikeField/xd/AnimBP_Spikes.closedSpikes` true (`self.animBp`))
  (set `self.lifeTime` (+ (`self.lifeTime`) 1.75))
  (set `self.time` 0.0))

(fn `UserConstructionScript`
  (bind _bp_damagedealer (`self.BP_DamageDealer`))
  (`SceneComponent.K2_AddLocalOffset` (`self.StaticMesh`) (`KismetMathLibrary.MakeVector` 0.0 0.0 (`self.yPosition`)) false false)
  (`SceneComponent.K2_AddLocalOffset` (`self.SM_Kolce_zapadanie`) (`KismetMathLibrary.MakeVector` 0.0 0.0 (`self.yPosition`)) false false)
  (set `/Game/Combat/Blueprints/BP_DamageDealer.parent` (`self.parentDamageDealer`) _bp_damagedealer)
  (set `/Game/Combat/Blueprints/BP_DamageDealer.useParent` true _bp_damagedealer)
  (set `/Game/Combat/Blueprints/BP_DamageDealer.damage` (`self.damage`) (`self.BP_DamageDealer`)))