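; Spike field attack: a forward-moving projectile that lays a trail of damaging BP_SingleSpike actors along the ground.
; Each tick a box trace snaps it to the surface height, and spikes spawn on a cooldown while the projectile is enabled.
; A steep slope or upward step stops spawning, notifies every spike and applies timed crowd control to units overlapping them.
; Once collided or disabled, it destroys itself when no valid spikes remain.
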(event `self.ReceiveBeginPlay`
  (add `/Game/Combat/Blueprints/BP_Projectile.OnProjectileDestroyed` (`self.BP_Projectile`) (delegate `OnProjectileDestroyed`)))

(event `OnProjectileDestroyed`
  (params (CollidedWith :type "Actor Soft Object Reference"))
  (`KismetSystemLibrary.Delay` 0.0)
  (`self.K2_DestroyActor`))

(event `Init`
  (params (position :type "Vector Structure") (direction :type "Vector Structure"))
  (`/Game/Combat/Blueprints/BP_Projectile.InitForwardProjectile` (`self.BP_Projectile`) position direction))

(event `self.ReceiveTick`
  (params (DeltaSeconds :type "Float (single-precision)"))
  (bind _returnvalue (`self.K2_GetActorLocation`))
  (bind (_returnvalue_x _returnvalue_y) (`KismetMathLibrary.BreakVector` (`self.K2_GetActorLocation`)))
  (bind _spawncd (`self.spawnCd`))
  (`self.DestroyIfNeeded`)
  (`/Engine/EditorBlueprintResources/StandardMacros.IsValid` self
    (:`Is Valid`
      (bind (_outhit _returnvalue_2) (`KismetSystemLibrary.BoxTraceSingle` (+ (* (`self.GetActorForwardVector`) 100.0) _returnvalue (0.0 0.0 100.0)) (+ _returnvalue (0.0 0.0 -500.0)) (100.0 100.0 10.0) (`self.K2_GetActorRotation`) "TraceTypeQuery3"))
      (if _returnvalue_2
        (bind (_bblockinghit _binitialoverlap _time _distance _location _impactpoint _normal) (`GameplayStatics.BreakHitResult` _outhit))
        (bind (_returnvalue_x_2 _returnvalue_y_2 _returnvalue_z) (`KismetMathLibrary.BreakVector` (+ _location (0.0 0.0 0.0))))
        (bind _returnvalue_3 (`KismetMathLibrary.MakeVector` _returnvalue_x _returnvalue_y _returnvalue_z))
        (bind (_returnvalue_x_3 _returnvalue_y_3 _returnvalue_z_2) (`KismetMathLibrary.BreakVector` (- _returnvalue_3 (`self.K2_GetActorLocation`))))
        (if (or (>= _returnvalue_z_2 60.0) (<= (`KismetMathLibrary.Dot_VectorVector` _normal (0.0 0.0 1.0)) 0.8))
          (`self.Collided`))
        (`self.K2_SetActorLocation` _returnvalue_3)
        (set `self.spawnCd` (- _spawncd (`GameplayStatics.GetWorldDeltaSeconds`)))
        (if (and (<= _spawncd 0.0) (`/Game/Combat/Blueprints/BP_Projectile.enabled` (`self.BP_Projectile`)))
          (set `self.spawnCd` (`self.spawnMaxCd`))
          (if (not (`self.wasCollided`))
            (bind _returnvalue_4 (`|SpawnActorFromClass` "/Game/Combat/SpikeField/BP_SingleSpike.BP_SingleSpike_C" (`KismetMathLibrary.MakeTransform` (`self.K2_GetActorLocation`) (`KismetMathLibrary.MakeRotator` (.roll (`KismetMathLibrary.RotatorFromAxisAndAngle` _normal (`KismetMathLibrary.RandomFloatInRange` 0.0 360.0))) (.pitch (`KismetMathLibrary.RotatorFromAxisAndAngle` _normal (`KismetMathLibrary.RandomFloatInRange` 0.0 360.0))) (.yaw (`KismetMathLibrary.RotatorFromAxisAndAngle` _normal (`KismetMathLibrary.RandomFloatInRange` 0.0 360.0))))) "AlwaysSpawn" "OverrideRootScale" null (`self.BP_DamageDealer`) (`self.damage`) null))
            (`KismetArrayLibrary.Array_Add` (`self.spikes`) _returnvalue_4)))))))

(event `Collided`
  (if (not (`self.wasCollided`))
    (set `self.wasCollided` true)
    (for _array_element (`self.spikes`)
      (`/Game/Combat/SpikeField/BP_SingleSpike.Collided` _array_element)
      (for _array_element_2 (`self.GetOverlappingActors` _array_element null)
        (`KismetArrayLibrary.Array_AddUnique` (`self.overlappingActors`) _array_element_2)))
    (`self.StunOverlapped`)))

(event `StunOverlapped`
  (for _array_element (`self.overlappingActors`)
    (bind _returnvalue (`self.GetComponentByClass` _array_element "/Game/Combat/Blueprints/BP_Unit.BP_Unit_C"))
    (`/Engine/EditorBlueprintResources/StandardMacros.IsValid` _returnvalue
      (:`Is Valid`
        (`/Game/Combat/Blueprints/BP_Unit.ApplyCrowdControl` _returnvalue "NewEnumerator0" (`self.snareDuration`))))))

(event `DestroyIfNeeded`
  (if (or (`self.wasCollided`) (not (`/Game/Combat/Blueprints/BP_Projectile.enabled` (`self.BP_Projectile`))))
    (set `self.destroyNow` true)
    (for _array_element (`self.spikes`)
      (`/Engine/EditorBlueprintResources/StandardMacros.IsValid` _array_element
        (:`Is Valid`
          (set `self.destroyNow` false)
          (break))))
    (if (`self.destroyNow`)
      (`self.K2_DestroyActor`))))

(fn `UserConstructionScript`
  (set `/Game/Combat/Blueprints/BP_DamageDealer.damage` (`self.damage`) (`self.BP_DamageDealer`)))