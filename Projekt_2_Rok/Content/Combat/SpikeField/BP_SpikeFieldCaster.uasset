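; Player spell caster for Spike Field, which releases spikes that damage enemies and, per its tooltip, snare units in their path upon hitting an obstacle.
; Casting requires readiness and not falling, then starts cooldown, cancels channels, turns the player along flattened camera forward and locks movement.
; AnimBP_Player2 events time the rest: fired spawns BP_SpikeField ahead of the player with level-scaled damage and snare duration, end restores movement.
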(event `self.Init`
  (params (actor :type "Actor Object Reference") (manager :type "/Game/Combat/SpellSystem/BP_SpellManager Object Reference"))
  (`parent.Init` actor manager)
  (bind _ascharacter (cast `Character` (`self.ownerPlayer`)))
  (bind _asanim_bp_player_2 (cast `/Game/Combat/Player/tests/AnimBP_Player2` (`SkeletalMeshComponent.GetAnimInstance` (`Character.Mesh` _ascharacter))))
  (add `/Game/Combat/Player/tests/AnimBP_Player2.SpikeFieldFired` _asanim_bp_player_2 (delegate `SpikeFieldFired`))
  (add `/Game/Combat/Player/tests/AnimBP_Player2.SpikeFieldEnd` _asanim_bp_player_2 (delegate `SpikeFieldEnd`)))

(event `SpikeFieldFired`
  (bind _returnvalue (`|SpawnActorFromClass` "/Game/Combat/SpikeField/BP_SpikeField.BP_SpikeField_C" (`KismetMathLibrary.Conv_VectorToTransform` (`self.position`)) "Undefined" "OverrideRootScale" null (`/Game/Combat/Blueprints/BP_Helpers.Evaluate` (`self.damage`) (`self.level`)) (`/Game/Combat/Blueprints/BP_Helpers.Evaluate` (`self.snareDuration`) (`self.level`)) null))
  (`/Game/Combat/SpikeField/BP_SpikeField.Init` _returnvalue (`self.position`) (`self.direction`)))

(event `SpikeFieldEnd`
  (`/Game/Combat/SpellSystem/BP_SpellManager.SetMovementMode` (`self.ownerManager`) true)
  (set `self.castPhase` "NewEnumerator0"))

(event `self.CastSpell`
  (bind _returnvalue (`KismetMathLibrary.MakeVector` (.x (`self.GetActorForwardVector` (`GameplayStatics.GetPlayerCameraManager` 0))) (.y (`self.GetActorForwardVector` (`GameplayStatics.GetPlayerCameraManager` 0)))))
  (if (and (`self.isReady`) (not (`/Game/Combat/SpellSystem/BP_SpellManager.IsPlayerFalling` (`self.ownerManager`))))
    (`self.SetMaxCooldown`)
    (`/Game/Combat/SpellSystem/BP_SpellManager.CancelChannels` (`self.ownerManager`))
    (set `self.direction` _returnvalue)
    (set `self.position` (+ (`self.K2_GetActorLocation` (`self.ownerPlayer`)) (* _returnvalue 150.0)))
    (`/Game/Combat/SpellSystem/BP_SpellManager.RotatePlayer` (`self.ownerManager`) (`self.direction`))
    (bind _ascharacter (cast `Character` (`self.ownerPlayer`)))
    (bind _asanim_bp_player_2 (cast `/Game/Combat/Player/tests/AnimBP_Player2` (`SkeletalMeshComponent.GetAnimInstance` (`Character.Mesh` _ascharacter))))
    (`/Game/Combat/Player/tests/AnimBP_Player2.SetState` _asanim_bp_player_2 "NewEnumerator4")
    (`/Game/Combat/SpellSystem/BP_SpellManager.SetMovementMode` (`self.ownerManager`) false)
    (set `self.castPhase` "NewEnumerator2")))

(fn `GetSpellInfo`
  (params (ForNextLevel :type Boolean))
  (returns (Text :type Text))
  (locals (ForNextLevel_ :type Boolean))
  (set `local.ForNextLevel_` ForNextLevel)
  (bind _name (`/Game/BP_Functions.GetKeyName` "SpikeField"))
  (return (`|FormatText` "Uwolnij kolce przeszywające wrogów, przyciskiem {Key}, zadając {Damage} obrażeń. Po napotkaniu przeszkody unieruchamiają przez {SnareDuration} sekund wszystkie jednostki na swojej drodze." _name (`/Game/Combat/Blueprints/BP_Helpers.EvaluateString` (`self.damage`) (`self.level`) (`local.ForNextLevel_`)) (`/Game/Combat/Blueprints/BP_Helpers.EvaluateString` (`self.snareDuration`) (`self.level`) (`local.ForNextLevel_`)))))

(fn `UserConstructionScript`
  (`parent.UserConstructionScript`))