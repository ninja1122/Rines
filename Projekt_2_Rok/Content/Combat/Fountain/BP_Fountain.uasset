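; Timed fountain area effect that pushes overlapping enemies outward and, if Heal is set, heals players, with a bonus on first contact.
; Each tick processes overlapped units; the horizontal push weakens with distance and age until the actor destroys itself.
; The construction script converts DamagePerSecond into per-tick damage for BPDamageDealer.
; Init aligns it to a surface normal, and a dynamic material shows heal mode and a sine-based fade.
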(event `self.ReceiveBeginPlay`
  (bind _returnvalue (`PrimitiveComponent.CreateDynamicMaterialInstance` (`self.StaticMesh`) 0 null "None"))
  (bind _output_get (set `self.material` _returnvalue))
  (`MaterialInstanceDynamic.SetScalarParameterValue` _output_get "heal" (select `bool` (`self.heal`) :`true` 1.0 :!type "Float (single-precision)")))

(event `self.ReceiveTick`
  (params (DeltaSeconds :type "Float (single-precision)"))
  (bind _material (`self.material`))
  (bind _output_get (set `self.lifeTimeElapsed` (+ (`self.lifeTimeElapsed`) DeltaSeconds)))
  (if (>= _output_get (`self.lifeTime`))
    (`self.K2_DestroyActor`)
    (else
      (`self.MoveUnits` (`GameplayStatics.GetWorldDeltaSeconds`))
      (`MaterialInstanceDynamic.SetScalarParameterValue` _material "Fade" (`KismetMathLibrary.FClamp` (* (`KismetMathLibrary.Sin` (`KismetMathLibrary.MultiplyByPi` (/ (`self.lifeTimeElapsed`) (`self.lifeTime`)))) 4.0)))
      (`MaterialInstanceDynamic.SetScalarParameterValue` _material "FTime" (`self.lifeTimeElapsed`)))))

(event `self.ReceiveActorEndOverlap`
  (params (OtherActor :type "Actor Object Reference"))
  (`KismetArrayLibrary.Array_RemoveItem` (`self.overlappedActors`) (`|ConvertAsset` OtherActor)))

(event `self.ReceiveActorBeginOverlap`
  (params (OtherActor :type "Actor Object Reference"))
  (`KismetArrayLibrary.Array_AddUnique` (`self.overlappedActors`) (`|ConvertAsset` OtherActor)))

(event `MoveUnits`
  (params (delta :type "Float (double-precision)"))
  (for _array_element (`self.overlappedActors`)
    (bind _output (`|ConvertAsset` _array_element))
    (`/Engine/EditorBlueprintResources/StandardMacros.IsValid` _output
      (:`Is Valid`
        (bind _returnvalue (`self.GetComponentByClass` _output "/Game/Combat/Blueprints/BP_Unit.BP_Unit_C"))
        (`/Engine/EditorBlueprintResources/StandardMacros.IsValid` _returnvalue
          (:`Is Valid`
            (switch `/Game/Combat/Blueprints/BP_UnitClass` (`/Game/Combat/Blueprints/BP_Unit.unitClass` _returnvalue)
              (:`NewEnumerator0`
                (if (`self.heal`)
                  (`self.TryToHealSingleUnit` _output)))
              (:`NewEnumerator1`
                (`self.MoveSingleUnit` _output)))))))))

(event `Init`
  (params (Normal :type "Vector Structure"))
  (`self.K2_SetActorRotation` (`KismetMathLibrary.MakeRotFromZ` Normal)))

(fn `MoveSingleUnit`
  (params (actor :type "Actor Object Reference"))
  (bind _returnvalue (`self.K2_GetActorLocation` actor))
  (bind _returnvalue_2 (- _returnvalue (`self.K2_GetActorLocation`)))
  (`self.K2_SetActorLocation` actor (+ _returnvalue (* (`KismetMathLibrary.Normal` (* _returnvalue_2 (1.0 1.0 0.0))) (* (* (`GameplayStatics.GetWorldDeltaSeconds`) (`KismetMathLibrary.FClamp` (- 500.0 (`KismetMathLibrary.VSize` _returnvalue_2)) 100.0 500.0)) (* (- 1.0 (/ (`self.lifeTimeElapsed`) (`self.lifeTime`))) 4.0)))) false false))

(fn `TryToHealSingleUnit`
  (params (Actor :type "Actor Object Reference"))
  (bind _returnvalue (`self.GetComponentByClass` Actor "/Game/Combat/Blueprints/BP_Unit.BP_Unit_C"))
  (bind _output (`|ConvertAsset` Actor))
  (bind _healedactors (`self.healedActors`))
  (bind _returnvalue_2 (* (`self.healPerSecond`) (`GameplayStatics.GetWorldDeltaSeconds`)))
  (if (`BlueprintSetLibrary.Set_Contains` _healedactors _output)
    (`/Game/Combat/Blueprints/BP_Unit.Heal` _returnvalue _returnvalue_2 false)
    (else
      (`BlueprintSetLibrary.Set_Add` _healedactors _output)
      (`/Game/Combat/Blueprints/BP_Unit.Heal` _returnvalue (+ _returnvalue_2 (`self.firstHealValue`)) false))))

(fn `UserConstructionScript`
  (bind _bp_damagedealer (`self.BP_DamageDealer`))
  (set `/Game/Combat/Blueprints/BP_DamageDealer.damage` (* (`/Game/Combat/Blueprints/BP_DamageDealer.tickRate` _bp_damagedealer) (`self.damagePerSecond`)) _bp_damagedealer))