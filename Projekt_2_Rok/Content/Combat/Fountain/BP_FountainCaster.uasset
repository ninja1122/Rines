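; Fountain spell caster that spawns a BP_Fountain beneath the player, configured for level-scaled damage per second and optional healing.
; Casting requires readiness and not falling, then starts the cooldown, cancels channels and traces downward for the spawn location and surface normal.
; Healing is enabled, consuming one Potion, only when one is in inventory and health is at or below half.
; GetSpellInfo builds the Polish tooltip from level-evaluated values.
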(event `self.CastSpell`
  (bind _ownerplayer (`self.ownerPlayer`))
  (bind _returnvalue (`self.K2_GetActorLocation` _ownerplayer))
  (if (and (`self.isReady`) (not (`/Game/Combat/SpellSystem/BP_SpellManager.IsPlayerFalling` (`self.ownerManager`))))
    (`self.SetMaxCooldown`)
    (`/Game/Combat/SpellSystem/BP_SpellManager.CancelChannels` (`self.ownerManager`))
    (bind _outhit (`KismetSystemLibrary.LineTraceSingle` _returnvalue (+ _returnvalue (0.0 0.0 -200.0)) "TraceTypeQuery3" false (`|MakeArray` _ownerplayer)))
    (if true
      (set `self.CanCurrentlyHeal` (`self.CanHeal`))
      (if (`self.CanCurrentlyHeal`)
        (`PlayerInventory.RemoveFromInventoryString` (`self.GetComponentByClass` (`GameplayStatics.GetPlayerPawn` 0) "/Script/Projekt_2_Rok.PlayerInventory") "Potion" 1))
      (bind (_bblockinghit _binitialoverlap _time _distance _location _impactpoint _normal) (`GameplayStatics.BreakHitResult` _outhit))
      (bind _returnvalue_2 (`|SpawnActorFromClass` "/Game/Combat/Fountain/BP_Fountain.BP_Fountain_C" (`KismetMathLibrary.Conv_VectorToTransform` _location) "Undefined" "OverrideRootScale" null (`/Game/Combat/Blueprints/BP_Helpers.Evaluate` (`self.healPerSecond`) (`self.level`)) (`/Game/Combat/Blueprints/BP_Helpers.Evaluate` (`self.firstHeal`) (`self.level`)) (`self.CanCurrentlyHeal`) (`/Game/Combat/Blueprints/BP_Helpers.Evaluate` (`self.damagePerSecond`) (`self.level`)) null))
      (`/Game/Combat/Fountain/BP_Fountain.Init` _returnvalue_2 _normal))))

(fn `CanHeal`
  (returns (CanHeal :type Boolean))
  (bind _returnvalue (`GameplayStatics.GetPlayerPawn` 0))
  (bind _returnvalue_2 (`PlayerInventory.CheckIsInInventory` (`self.GetComponentByClass` _returnvalue "/Script/Projekt_2_Rok.PlayerInventory") "Potion" 1))
  (return (and _returnvalue_2 (<= (`/Game/Combat/Blueprints/BP_Helpers.GetPercentageHealth` (`/Game/Combat/Blueprints/BP_Unit.health` (`self.GetComponentByClass` _returnvalue "/Game/Combat/Blueprints/BP_Unit.BP_Unit_C"))) 0.5))))

(fn `GetSpellInfo`
  (params (ForNextLevel :type Boolean))
  (returns (Text :type Text))
  (locals (ForNextLevel_ :type Boolean))
  (set `local.ForNextLevel_` ForNextLevel)
  (bind _name (`/Game/BP_Functions.GetKeyName` "Fountain"))
  (return (`|FormatText` "Kliknij {key}, aby aktywować źródło życia.  \nZużywa eliksiry życia regenerując jednorazowo {FirstHeal} punktów zdrowia, a następnie dodatkowo {HealPerSecond} punktów na sekundę. \nLeczy gdy gracz ma poniżej 50% zdrowia. Dodatkowo zadaje {Damage} obrażeń obszarowych na sekundę.  \nAktywuje chwilową przestrzeń ochronną." _name (`/Game/Combat/Blueprints/BP_Helpers.EvaluateString` (`self.firstHeal`) (`self.level`) (`local.ForNextLevel_`)) (`/Game/Combat/Blueprints/BP_Helpers.EvaluateString` (`self.healPerSecond`) (`self.level`) (`local.ForNextLevel_`)) (`/Game/Combat/Blueprints/BP_Helpers.EvaluateString` (`self.damagePerSecond`) (`self.level`) (`local.ForNextLevel_`)))))

(fn `UserConstructionScript`
  (`parent.UserConstructionScript`))