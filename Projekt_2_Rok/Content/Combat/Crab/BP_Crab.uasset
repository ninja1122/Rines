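; Crab enemy character, driven by an AI blackboard and a BP_Unit component, with an optional jump ability.
; Claw attacks damage the blackboard target within short range and a frontal cone; jump hits deal heavier damage, gated by animation state and cooldown.
; Taking damage triggers aggro; death drops meat, plus a random potion for jump-capable crabs.
; Tick smoothly turns it toward its velocity and plays random sounds while alive.
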(event `self.ReceiveBeginPlay`
  (bind _returnvalue (`AIBlueprintHelperLibrary.GetBlackboard` (`AIBlueprintHelperLibrary.GetAIController` self)))
  (`BlackboardComponent.SetValueAsVector` _returnvalue "SpawnPoint" (`self.K2_GetActorLocation`))
  (`BlackboardComponent.SetValueAsBool` _returnvalue "CanJump" (`self.hasAbilityToJump`))
  (add `/Game/Combat/Blueprints/BP_Unit.UnitTookDamage` (`self.BP_Unit`) (delegate `CrabTookDamage`))
  (add `/Game/Combat/Blueprints/BP_Unit.UnitDied` (`self.BP_Unit`) (delegate `UnitDied`)))

(event `CrabTookDamage`
  (params (damage :type "Float (double-precision)") (type :type "/Game/Combat/Blueprints/BP_DamageType Enum" :default "NewEnumerator0"))
  (set `/Game/Combat/Blueprints/BP_Unit.hasAggro` true (`self.BP_Unit`)))

(event `UnitDied`
  (params (Actor :type "Actor Object Reference") (Unit :type "/Game/Combat/Blueprints/BP_Unit Object Reference"))
  (`|SpawnActorFromClass` "/Game/Blueprints/Inventory/Krab_Mieso.Krab_Mieso_C" (`KismetMathLibrary.Conv_VectorToTransform` (`self.K2_GetActorLocation`)) "AlwaysSpawn" "OverrideRootScale" null null)
  (if (`self.hasAbilityToJump`)
    (`/Game/BP_GameInstance.SpawnRandomPotion` (`/Game/BP_Functions.GetFakeUpGameInstance`) (`self.K2_GetActorLocation`))))

(event `ClawDamage`
  (bind _asactor (cast `Actor` (`BlackboardComponent.GetValueAsObject` (`AIBlueprintHelperLibrary.GetBlackboard` (`AIBlueprintHelperLibrary.GetAIController` self)) "Target")))
  (bind _returnvalue (- (`self.K2_GetActorLocation` _asactor) (`self.K2_GetActorLocation`)))
  (if (and (<= (`KismetMathLibrary.VSize` _returnvalue) 250.0) (>= (`KismetMathLibrary.Dot_VectorVector` (`KismetMathLibrary.Normal` _returnvalue) (`self.GetActorForwardVector`)) (`KismetMathLibrary.DegCos` 45.0)))
    (bind _returnvalue_2 (`self.GetComponentByClass` _asactor "/Game/Combat/Blueprints/BP_Unit.BP_Unit_C"))
    (`/Engine/EditorBlueprintResources/StandardMacros.IsValid` _returnvalue_2
      (:`Is Valid`
        (`/Game/Combat/Blueprints/BP_Unit.Take Damage` _returnvalue_2 10.0 "NewEnumerator0")))))

(event `self.ReceiveHit`
  (params (MyComp :type "PrimitiveComponent Object Reference") (Other :type "Actor Object Reference") (OtherComp :type "PrimitiveComponent Object Reference") (bSelfMoved :type Boolean) (HitLocation :type "Vector Structure") (HitNormal :type "Vector Structure") (NormalImpulse :type "Vector Structure") (Hit :type "HitResult Structure (by ref)"))
  (bind _returnvalue (`self.GetComponentByClass` Other "/Game/Combat/Blueprints/BP_Unit.BP_Unit_C"))
  (if (<= (`self.jumpAttackCooldown`) 0.0)
    (bind _asanim_bp_crab (cast `/Game/Combat/Crab/AnimBP_Crab` (`SkeletalMeshComponent.GetAnimInstance` (`self.Mesh`))))
    (if (`/Game/Combat/Crab/AnimBP_Crab.isStateInProgress` _asanim_bp_crab "NewEnumerator2")
      (`/Engine/EditorBlueprintResources/StandardMacros.IsValid` _returnvalue
        (:`Is Valid`
          (`/Game/Combat/Blueprints/BP_Unit.Take Damage` _returnvalue 30.0 "NewEnumerator0")
          (set `self.jumpAttackCooldown` 5.0))))))

(event `self.ReceiveTick`
  (params (DeltaSeconds :type "Float (single-precision)"))
  (bind _audio (`self.Audio`))
  (bind _velocity (`MovementComponent.Velocity` (`self.CharacterMovement`)))
  (`|ExecutionSequence`
    (:`then_0`
      (set `self.jumpAttackCooldown` (`KismetMathLibrary.FMax` (- (`self.jumpAttackCooldown`) DeltaSeconds)))
      (if (!= (`KismetMathLibrary.VSizeSquared` _velocity) 0.0)
        (`self.K2_SetActorRotation` (`KismetMathLibrary.RLerp` (`self.K2_GetActorRotation`) (`KismetMathLibrary.FindLookAtRotation` (`KismetMathLibrary.MakeVector` 0.0) _velocity) 0.4 true))))
    (:`then_1`
      (if (`/Game/Combat/Blueprints/BP_Unit.IsAlive` (`self.BP_Unit`))
        (set `self.randomSoundTime` (- (`self.randomSoundTime`) (`GameplayStatics.GetWorldDeltaSeconds`)))
        (if (<= (`self.randomSoundTime`) 0.0)
          (set `self.randomSoundTime` (`KismetMathLibrary.RandomFloatInRange` 1.0 3.0))
          (`AudioComponent.SetSound` _audio (`|GetArrayItem` (`self.randomSounds`) (`KismetMathLibrary.RandomInteger` 2)))
          (`AudioComponent.Play` _audio 0.0))))))

(fn `UserConstructionScript`)