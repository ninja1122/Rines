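; GameNameSequence is a trigger Blueprint that plays a short game-name cinematic when the player character overlaps its box.
; It enters cinematic mode, hides the BP_Hud, blends the view to its camera and shows the RinesCinematic widget.
; After timed delays it blends back to the player, restores HUD and control, and removes the widget.
; The Lvl1GameName flag on the game instance, set at the end, prevents replays.
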(event `self.Box.OnComponentBeginOverlap`
  (params (OverlappedComponent :type "PrimitiveComponent Object Reference") (OtherActor :type "Actor Object Reference") (OtherComp :type "PrimitiveComponent Object Reference") (OtherBodyIndex :type Integer) (bFromSweep :type Boolean) (SweepResult :type "HitResult Structure (by ref)"))
  (bind _returnvalue (`GameplayStatics.GetPlayerController` 0))
  (if (== OtherActor (`GameplayStatics.GetPlayerCharacter` 0))
    (bind _asfake_up_game_instance_base (cast `FakeUpGameInstanceBase` (`GameplayStatics.GetGameInstance`)))
    (if (not (`FakeUpGameInstanceBase.Lvl1GameName` _asfake_up_game_instance_base))
      (`PlayerController.SetCinematicMode` _returnvalue true false true true true)
      (bind _asbp_hud (cast `/Game/Combat/Ui/BP_Hud` (`PlayerController.GetHUD` _returnvalue)))
      (`/Game/Combat/Ui/BP_Hud.SetHudVisible` _asbp_hud false)
      (`PlayerController.SetViewTargetWithBlend` (`GameplayStatics.GetPlayerController` 0) (`self.Camera`) 3.0 "VTBlend_EaseInOut" 3.0 false)
      (`KismetSystemLibrary.Delay` 2.0)
      (`/Engine/EditorBlueprintResources/StandardMacros.IsValid` (stale _returnvalue_2)
        (:`Is Valid`
          _)
        (:`Is Not Valid`
          (bind _returnvalue_2 (`|CreateWidget` "/Game/Widgets/RinesCinematic/RinesCinematic.RinesCinematic_C" (`GameplayStatics.GetPlayerController` 0)))))
      (`UserWidget.AddToViewport` _returnvalue_2 0)
      (`KismetSystemLibrary.Delay` 7.0)
      (`PlayerController.SetViewTargetWithBlend` (`GameplayStatics.GetPlayerController` 0) (`GameplayStatics.GetPlayerCharacter` 0) 3.0 "VTBlend_EaseInOut" 3.0 false)
      (`KismetSystemLibrary.Delay` 3.0)
      (`PlayerController.SetCinematicMode` (`GameplayStatics.GetPlayerController` 0) false false true true true)
      (`/Game/Combat/Ui/BP_Hud.SetHudVisible` _asbp_hud true)
      (bind _asfake_up_game_instance_base_2 (cast `FakeUpGameInstanceBase` (`GameplayStatics.GetGameInstance`)))
      (set `FakeUpGameInstanceBase.Lvl1GameName` true _asfake_up_game_instance_base_2)
      (`Widget.RemoveFromParent` _returnvalue_2))))

(fn `UserConstructionScript`)