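; SequenceLight is a trigger that lights a series of fire lights one after another when the player enters its box.
; On overlap by player 0's character, it calls LightFire on each entry in Lights, using a for-each loop unrolled with a Delay between iterations.
; Once that list is done, it calls LightFire on every LightsEnd entry at once as a finale.
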(event `self.Box.OnComponentBeginOverlap`
  (params (OverlappedComponent :type "PrimitiveComponent Object Reference") (OtherActor :type "Actor Object Reference") (OtherComp :type "PrimitiveComponent Object Reference") (OtherBodyIndex :type Integer) (bFromSweep :type Boolean) (SweepResult :type "HitResult Structure (by ref)"))
  (bind _variable (`|TemporaryVariable`))
  (bind _variable_2 (`|TemporaryVariable`))
  (bind _lights (`self.Lights`))
  (if (== OtherActor (`GameplayStatics.GetPlayerCharacter` 0))
    (`|AssignmentStatement` _variable_2)
    (`|AssignmentStatement` _variable)
    (if (< _variable_2 (`KismetArrayLibrary.Array_Length` _lights)) :!label _label
      (`|AssignmentStatement` _variable _variable_2)
      (`|ExecutionSequence`
        (:`then_0`
          (`/Game/Blueprints/SequenceLight/BP_Ognisko_SequenceLight.LightFire` (`|GetArrayItem` _lights _variable)))
        (:`then_1`
          (`KismetSystemLibrary.Delay` (`self.Delay`))
          (`|AssignmentStatement` _variable_2 (+ _variable_2 1))
          (goto _label)))
      (else
        (for _array_element (`self.LightsEnd`)
          (`/Game/Blueprints/SequenceLight/BP_Ognisko_SequenceLight.LightFire` _array_element))))))

(fn `UserConstructionScript`)