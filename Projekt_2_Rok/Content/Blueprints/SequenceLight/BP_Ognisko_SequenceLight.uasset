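; Campfire (Ognisko) actor that can be lit or extinguished, toggling its fire effect and point light.
; LightFire sets the burning state, which on a change either plays a burst and starts fire and light after a short delay, or shuts both off.
; The construction script applies the initial burning state and light radius.
; IsAbleToBeginFire accepts only BP_FireBall or BP_FlameBreath actors as igniters.
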(event `LightFire`
  (`self.SetBurningState` true))

(event `SetBurningState`
  (params (Burning :type Boolean))
  (bind _fire (`self.Fire`))
  (bind _pointlight (`self.PointLight`))
  (if (!= Burning (`self.isBuring`))
    (set `self.isBuring` Burning)
    (if (`self.isBuring`)
      (`ActorComponent.Activate` (`self.Explo`) true)
      (`KismetSystemLibrary.Delay` 0.3)
      (`ActorComponent.Activate` _fire false)
      (`SceneComponent.SetVisibility` _pointlight true false)
      (else
        (`ActorComponent.Deactivate` _fire)
        (`SceneComponent.SetVisibility` _pointlight false false)))))

(fn `IsAbleToBeginFire`
  (params (Actor :type "Actor Object Reference"))
  (returns (Able :type Boolean))
  (bind _returnvalue (`GameplayStatics.GetObjectClass` Actor))
  (return (or (== _returnvalue "/Game/Combat/FireBall/BP_FireBall.BP_FireBall_C") (== _returnvalue "/Game/Combat/FireBall/BP_FlameBreath.BP_FlameBreath_C"))))

(fn `UserConstructionScript`
  (bind _pointlight (`self.PointLight`))
  (bind _isburing (`self.isBuring`))
  (`ActorComponent.SetAutoActivate` (`self.Fire`) _isburing)
  (`SceneComponent.SetVisibility` _pointlight _isburing false)
  (`LocalLightComponent.SetAttenuationRadius` _pointlight (`self.Radius`)))