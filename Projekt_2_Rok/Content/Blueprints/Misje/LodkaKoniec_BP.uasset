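; Mission-ending boat that lets the player sail away to LEV_1 through an interactable box trigger.
; Interaction is enabled only while mission index 1 in the game instance is at part 7.
; Interacting shows a load screen, saves the player, sets the load save name and plays a StoryIntro video, opening the level shortly after it ends.
; An older overlap-driven key prompt and direct level load remain disconnected.
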(event `self.ReceiveBeginPlay`
  (`/Game/Blueprints/Interactable/BP_Interactable.Init` (`self.BP_Interactable`) (`self.Box`) "Naciśnij {0} aby odpłynąć"))

(event `self.BP_Interactable.ShouldShowInteract`
  (set `/Game/Blueprints/Interactable/BP_Interactable.Interactable` (== (`.KtoraCzescMisji` (break `Misje` (`|GetArrayItem` (`FakeUpGameInstanceBase.testMisje` (cast `/Game/BP_GameInstance` (`GameplayStatics.GetGameInstance`) :!pure true)) 1))) 7) (`self.BP_Interactable`)))

(event `self.BP_Interactable.Interacted`
  (`/Engine/EditorBlueprintResources/StandardMacros.IsValid` (stale _returnvalue)
    (:`Is Valid`
      _)
    (:`Is Not Valid`
      (bind _returnvalue (`|CreateWidget` "/Game/Widgets/LoadScreen.LoadScreen_C" (`GameplayStatics.GetPlayerController` 0)))))
  (`UserWidget.AddToViewport` _returnvalue 0)
  (`SaveGamePlayerComponent.SavePlayer` (`self.GetComponentByClass` (`GameplayStatics.GetPlayerCharacter` 0) "/Script/Projekt_2_Rok.SaveGamePlayerComponent") "player")
  (set `FakeUpGameInstanceBase.LoadSaveName` "S" (cast `FakeUpGameInstanceBase` (`GameplayStatics.GetGameInstance`) :!pure true))
  (bind _returnvalue_2 (`|CreateWidget` "/Game/Widgets/StoryIntro/StoryIntro.StoryIntro_C" (`GameplayStatics.GetPlayerController` 0)))
  (`UserWidget.AddToViewport` _returnvalue_2 0)
  (add `MediaPlayer.OnEndReached` (`/Game/Widgets/StoryIntro/StoryIntro.MediaPlayer` _returnvalue_2) (delegate `OnFInish`)))

(event `OnFInish`
  (`KismetSystemLibrary.Delay` 0.1)
  (`GameplayStatics.OpenLevel` "LEV_1"))

(event `self.Box.OnComponentBeginOverlap`
  (params (OverlappedComponent :type "PrimitiveComponent Object Reference") (OtherActor :type "Actor Object Reference") (OtherComp :type "PrimitiveComponent Object Reference") (OtherBodyIndex :type Integer) (bFromSweep :type Boolean) (SweepResult :type "HitResult Structure (by ref)")))

(event `self.Box.OnComponentEndOverlap`
  (params (OverlappedComponent :type "PrimitiveComponent Object Reference") (OtherActor :type "Actor Object Reference") (OtherComp :type "PrimitiveComponent Object Reference") (OtherBodyIndex :type Integer)))

(event `InputAction|Interact`
  (params (Key :type "Key Structure")))

(fn `UserConstructionScript`)