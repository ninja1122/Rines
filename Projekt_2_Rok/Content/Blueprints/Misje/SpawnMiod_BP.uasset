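; Mission trigger actor that spawns honey (Miod) pickups for a quest.
; When the player character overlaps its Box, it checks whether the mission at index 1 in the GameInstance's TestMisje array is at part 3.
; If so, a DoOnce spawns seven Miod actors at hard-coded world locations, ignoring collisions.
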(event `self.Box.OnComponentBeginOverlap`
  (params (OverlappedComponent :type "PrimitiveComponent Object Reference") (OtherActor :type "Actor Object Reference") (OtherComp :type "PrimitiveComponent Object Reference") (OtherBodyIndex :type Integer) (bFromSweep :type Boolean) (SweepResult :type "HitResult Structure (by ref)"))
  (if (== OtherActor (`GameplayStatics.GetPlayerCharacter` 0))
    (if (== (`.KtoraCzescMisji` (break `Misje` (`|GetArrayItem` (`FakeUpGameInstanceBase.testMisje` (cast `/Game/BP_GameInstance` (`GameplayStatics.GetGameInstance`) :!pure true)) 1))) 3)
      (`/Engine/EditorBlueprintResources/StandardMacros.DoOnce` false
        (:`Completed`
          (`|SpawnActorFromClass` "/Game/Blueprints/Inventory/Miod.Miod_C" (`KismetMathLibrary.MakeTransform` (-11820.0 -190.0 410.0)) "AlwaysSpawn" "OverrideRootScale" null null)
          (`|SpawnActorFromClass` "/Game/Blueprints/Inventory/Miod.Miod_C" (`KismetMathLibrary.MakeTransform` (-12470.0 -20.0 500.0)) "AlwaysSpawn" "OverrideRootScale" null null)
          (`|SpawnActorFromClass` "/Game/Blueprints/Inventory/Miod.Miod_C" (`KismetMathLibrary.MakeTransform` (-12210.0 -520.0 530.0)) "AlwaysSpawn" "OverrideRootScale" null null)
          (`|SpawnActorFromClass` "/Game/Blueprints/Inventory/Miod.Miod_C" (`KismetMathLibrary.MakeTransform` (-12550.0 -770.0 640.0)) "AlwaysSpawn" "OverrideRootScale" null null)
          (`|SpawnActorFromClass` "/Game/Blueprints/Inventory/Miod.Miod_C" (`KismetMathLibrary.MakeTransform` (-11620.0 -700.0 500.0)) "AlwaysSpawn" "OverrideRootScale" null null)
          (`|SpawnActorFromClass` "/Game/Blueprints/Inventory/Miod.Miod_C" (`KismetMathLibrary.MakeTransform` (-11610.0 -1150.0 550.0)) "AlwaysSpawn" "OverrideRootScale" null null)
          (`|SpawnActorFromClass` "/Game/Blueprints/Inventory/Miod.Miod_C" (`KismetMathLibrary.MakeTransform` (-11070.0 -550.0 500.0)) "AlwaysSpawn" "OverrideRootScale" null null))))))

(fn `UserConstructionScript`)