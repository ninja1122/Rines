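; Mission trigger that spawns a Drewno (wood) actor at a fixed world location during a quest.
; When the player begins or ends overlap with the Box, it checks the game instance's TestMisje entry at index 1 for mission part 5.
; Both overlap events share one DoOnce, so the wood spawns only once, regardless of collisions at that spot.
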(event `self.Box.OnComponentBeginOverlap`
  (params (OverlappedComponent :type "PrimitiveComponent Object Reference") (OtherActor :type "Actor Object Reference") (OtherComp :type "PrimitiveComponent Object Reference") (OtherBodyIndex :type Integer) (bFromSweep :type Boolean) (SweepResult :type "HitResult Structure (by ref)"))
  (if (== OtherActor (`GameplayStatics.GetPlayerCharacter` 0))
    (if (== (`.KtoraCzescMisji` (break `Misje` (`|GetArrayItem` (`FakeUpGameInstanceBase.testMisje` (cast `/Game/BP_GameInstance` (`GameplayStatics.GetGameInstance`) :!pure true)) 1))) 5) :!label _label
      (`/Engine/EditorBlueprintResources/StandardMacros.DoOnce` false
        (:`Completed`
          (`|SpawnActorFromClass` "/Game/Blueprints/Inventory/drewno.Drewno_C" (`KismetMathLibrary.MakeTransform` (-3936.0 -5840.0 160.0)) "AlwaysSpawn" "OverrideRootScale" null null))))))

(event `self.Box.OnComponentEndOverlap`
  (params (OverlappedComponent :type "PrimitiveComponent Object Reference") (OtherActor :type "Actor Object Reference") (OtherComp :type "PrimitiveComponent Object Reference") (OtherBodyIndex :type Integer))
  (if (== OtherActor (`GameplayStatics.GetPlayerCharacter` 0))
    (goto _label)))

(fn `UserConstructionScript`)