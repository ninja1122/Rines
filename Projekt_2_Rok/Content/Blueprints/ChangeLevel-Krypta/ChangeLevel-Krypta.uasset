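; ChangeLevel-Krypta is an interactable level transition that sends the player into the crypt level LEV_1_krypta.
; It sets up a BPInteractable prompt on its Box trigger, shown as interactable only while the mission for IDmisji is at part 1.
; On interaction it shows a loading screen, saves the player's location and data via SaveGamePlayerComponent, then opens the level.
; Older overlap and key-press prompt logic remains but is disconnected.
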(event `self.ReceiveBeginPlay`
  (`/Game/Blueprints/Interactable/BP_Interactable.Init` (`self.BP_Interactable`) (`self.Box`) "Naciśnij {0} aby przejść"))

(event `self.BP_Interactable.ShouldShowInteract`
  (set `/Game/Blueprints/Interactable/BP_Interactable.Interactable` (== (`.KtoraCzescMisji` (break `Misje` (`.Mission` (`/Game/BP_GameInstance.GetMissionForNpc` (cast `/Game/BP_GameInstance` (`GameplayStatics.GetGameInstance`) :!pure true) (`self.IDmisji`))))) 1) (`self.BP_Interactable`)))

(event `self.BP_Interactable.Interacted`
  (bind _returnvalue (`self.GetComponentByClass` (`GameplayStatics.GetPlayerCharacter` 0) "/Script/Projekt_2_Rok.SaveGamePlayerComponent"))
  (`/Engine/EditorBlueprintResources/StandardMacros.IsValid` (stale _returnvalue_2)
    (:`Is Valid`
      _)
    (:`Is Not Valid`
      (bind _returnvalue_2 (`|CreateWidget` "/Game/Widgets/LoadScreen.LoadScreen_C"))))
  (`UserWidget.AddToViewport` _returnvalue_2 0)
  (bind _returnvalue_3 (`GameplayStatics.GetCurrentLevelName` true))
  (`SaveGamePlayerComponent.SaveLocation` _returnvalue (`KismetStringLibrary.Concat_StrStr` _returnvalue_3 "-save"))
  (`SaveGamePlayerComponent.SavePlayer` _returnvalue "player")
  (`GameplayStatics.OpenLevel` "LEV_1_krypta"))

(event `self.Box.OnComponentBeginOverlap`
  (params (OverlappedComponent :type "PrimitiveComponent Object Reference") (OtherActor :type "Actor Object Reference") (OtherComp :type "PrimitiveComponent Object Reference") (OtherBodyIndex :type Integer) (bFromSweep :type Boolean) (SweepResult :type "HitResult Structure (by ref)")))

(event `self.Box.OnComponentEndOverlap`
  (params (OverlappedComponent :type "PrimitiveComponent Object Reference") (OtherActor :type "Actor Object Reference") (OtherComp :type "PrimitiveComponent Object Reference") (OtherBodyIndex :type Integer)))

(event `InputAction|Interact`
  (params (Key :type "Key Structure")))

(fn `UserConstructionScript`)