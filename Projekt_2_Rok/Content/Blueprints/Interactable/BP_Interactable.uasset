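; BP_Interactable is an actor component serving as both an interactable marker and the player's interaction manager.
; Initialized interactables register with the player's instance while their trigger is overlapped.
; Only the player's instance ticks, showing the closest candidate's text on BP_Hud; Interact fires that candidate's Interacted dispatcher.
; Selection compares squared horizontal distance, calling ShouldShowInteract so listeners can veto candidates through the Interactable flag.
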(event `self.ReceiveBeginPlay`
  (bind _returnvalue (== (`self.GetOwner`) (`GameplayStatics.GetPlayerPawn` 0)))
  (`self.SetComponentTickEnabled` _returnvalue)
  (if (not _returnvalue)
    (set `self.PlayerInteractable` (`Actor.GetComponentByClass` (`GameplayStatics.GetPlayerPawn` 0) "BP_Interactable_C"))))

(event `Init`
  (params (Trigger :type "PrimitiveComponent Object Reference") (TextToShow :type Text))
  (add `PrimitiveComponent.OnComponentBeginOverlap` Trigger (delegate `BeginOverlap`))
  (add `PrimitiveComponent.OnComponentEndOverlap` Trigger (delegate `EndOverlap`))
  (set `self.Trigger` Trigger)
  (set `self.TextToShow` TextToShow))

(event `BeginOverlap`
  (params (OverlappedComponent :type "PrimitiveComponent Object Reference") (OtherActor :type "Actor Object Reference") (OtherComp :type "PrimitiveComponent Object Reference") (OtherBodyIndex :type Integer) (bFromSweep :type Boolean) (SweepResult :type "HitResult Structure (by ref)"))
  (`KismetArrayLibrary.Array_AddUnique` (`/Game/Blueprints/Interactable/BP_Interactable.CurrentInteractables` (`self.PlayerInteractable`)) self))

(event `EndOverlap`
  (params (OverlappedComponent :type "PrimitiveComponent Object Reference") (OtherActor :type "Actor Object Reference") (OtherComp :type "PrimitiveComponent Object Reference") (OtherBodyIndex :type Integer))
  (`KismetArrayLibrary.Array_RemoveItem` (`/Game/Blueprints/Interactable/BP_Interactable.CurrentInteractables` (`self.PlayerInteractable`)) self))

(event `self.ReceiveTick`
  (params (DeltaSeconds :type "Float (single-precision)"))
  (bind _interactable (`self.GetClosestInteractable`))
  (bind _asbp_hud (cast `/Game/Combat/Ui/BP_Hud` (`PlayerController.GetHUD` (`GameplayStatics.GetPlayerController` 0))))
  (`/Engine/EditorBlueprintResources/StandardMacros.IsValid` _interactable
    (:`Is Valid`
      (`/Game/Combat/Ui/BP_Hud.SetInteractable` _asbp_hud (`/Game/Blueprints/Interactable/BP_Interactable.TextToShow` _interactable)))
    (:`Is Not Valid`
      (`/Game/Combat/Ui/BP_Hud.SetInteractable` _asbp_hud ""))))

(event `Interact`
  (bind _interactable (`self.GetClosestInteractable`))
  (`/Engine/EditorBlueprintResources/StandardMacros.IsValid` _interactable
    (:`Is Valid`
      (`self.Interacted` _interactable))))

(fn `GetClosestInteractable`
  (returns (Interactable :type "/Game/Blueprints/Interactable/BP_Interactable Object Reference"))
  (locals (ClosestDistance :type "Float (double-precision)" :default 10000000000.0) (ClosestInteractable :type "/Game/Blueprints/Interactable/BP_Interactable Object Reference"))
  (for _array_element (`self.CurrentInteractables`)
    (`/Engine/EditorBlueprintResources/StandardMacros.IsValid` _array_element
      (:`Is Valid`
        (set `/Game/Blueprints/Interactable/BP_Interactable.Interactable` true _array_element)
        (bind _returnvalue (`KismetMathLibrary.VSizeSquared` (- (* (`SceneComponent.K2_GetComponentLocation` (`/Game/Blueprints/Interactable/BP_Interactable.Trigger` _array_element)) (1.0 1.0 0.0)) (* (`Actor.K2_GetActorLocation` (`self.GetOwner`)) (1.0 1.0 0.0)))))
        (if (< _returnvalue (`local.ClosestDistance`))
          (`self.ShouldShowInteract` _array_element)
          (if (`/Game/Blueprints/Interactable/BP_Interactable.Interactable` _array_element)
            (set `local.ClosestDistance` _returnvalue)
            (set `local.ClosestInteractable` _array_element))))))
  (return (`local.ClosestInteractable`)))