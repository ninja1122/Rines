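; TempTrader is a trader actor the player can trade with by pressing Interact while inside its collider.
; Overlap shows or removes a "Press E to trade" prompt and toggles the actor's input.
; Interact opens a TraderMain widget fed the player's inventory and the trader's stock and gold, then pauses the game.
; Back or PauseMenu copies stock and gold back from the widget, closes it, restores the prompt and unpauses.
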(event `self.Collider.OnComponentBeginOverlap`
  (params (OverlappedComponent :type "PrimitiveComponent Object Reference") (OtherActor :type "Actor Object Reference") (OtherComp :type "PrimitiveComponent Object Reference") (OtherBodyIndex :type Integer) (bFromSweep :type Boolean) (SweepResult :type "HitResult Structure (by ref)"))
  (if (== OtherActor (`GameplayStatics.GetPlayerCharacter` 0))
    (`/Engine/EditorBlueprintResources/StandardMacros.IsValid` (stale _returnvalue)
      (:`Is Valid`
        _)
      (:`Is Not Valid`
        (bind _returnvalue (`|CreateWidget` "/Game/Widgets/Trader/Press_E_to_trade.Press_E_to_trade_C" (`GameplayStatics.GetPlayerController` 0)))))
    (`UserWidget.AddToViewport` _returnvalue 0)
    (`self.EnableInput` (`GameplayStatics.GetPlayerController` 0))))

(event `self.Collider.OnComponentEndOverlap`
  (params (OverlappedComponent :type "PrimitiveComponent Object Reference") (OtherActor :type "Actor Object Reference") (OtherComp :type "PrimitiveComponent Object Reference") (OtherBodyIndex :type Integer))
  (if (== OtherActor (`GameplayStatics.GetPlayerCharacter` 0))
    (bind _foundwidgets (`WidgetBlueprintLibrary.GetAllWidgetsOfClass` "/Game/Widgets/Trader/Press_E_to_trade.Press_E_to_trade_C"))
    (if (!= (`KismetArrayLibrary.Array_Length` _foundwidgets) 0)
      (`Widget.RemoveFromParent` (`|GetArrayItem` _foundwidgets)))
    (`self.DisableInput` (`GameplayStatics.GetPlayerController` 0))))

(event `InputAction|Interact`
  (params (Key :type "Key Structure"))
  (:`Pressed`
    (bind _foundwidgets (`WidgetBlueprintLibrary.GetAllWidgetsOfClass` "/Game/Widgets/Trader/Press_E_to_trade.Press_E_to_trade_C"))
    (if (!= (`KismetArrayLibrary.Array_Length` _foundwidgets) 0)
      (`Widget.RemoveFromParent` (`|GetArrayItem` _foundwidgets)))
    (`/Engine/EditorBlueprintResources/StandardMacros.IsValid` (stale _returnvalue)
      (:`Is Valid`
        _)
      (:`Is Not Valid`
        (bind _returnvalue (`|CreateWidget` "/Game/Widgets/Trader/TraderMain.TraderMain_C"))))
    (set `/Game/Widgets/Trader/TraderMain.PlayerInventory` (`PlayerInventory.inventory` (`self.GetComponentByClass` (`GameplayStatics.GetPlayerCharacter` 0) "/Script/Projekt_2_Rok.PlayerInventory")) _returnvalue)
    (set `/Game/Widgets/Trader/TraderMain.TraderGold` (`self.GoldQuantity`) _returnvalue)
    (set `/Game/Widgets/Trader/TraderMain.TraderInventory` (`self.content`) _returnvalue)
    (`UserWidget.AddToViewport` _returnvalue 0)
    (set `PlayerController.bShowMouseCursor` true (`GameplayStatics.GetPlayerController` 0))
    (`GameplayStatics.SetGamePaused` true)
    (set `/Game/Widgets/Trader/TraderMain.TraderActor` self _returnvalue)))

(event `Back`
  (`/Engine/EditorBlueprintResources/StandardMacros.IsValid` (stale _returnvalue) :!label _label
    (:`Is Valid`
      _)
    (:`Is Not Valid`
      (bind _returnvalue (`|CreateWidget` "/Game/Widgets/Trader/Press_E_to_trade.Press_E_to_trade_C" (`GameplayStatics.GetPlayerController` 0)))))
  (`UserWidget.AddToViewport` _returnvalue 0)
  (bind _foundwidgets (`WidgetBlueprintLibrary.GetAllWidgetsOfClass` "/Game/Widgets/Trader/TraderMain.TraderMain_C"))
  (if (!= (`KismetArrayLibrary.Array_Length` _foundwidgets) 0)
    (bind _output (`|GetArrayItem` _foundwidgets))
    (set `self.content` (`/Game/Widgets/Trader/TraderMain.TraderInventory` _output))
    (set `self.GoldQuantity` (`/Game/Widgets/Trader/TraderMain.TraderGold` _output))
    (`Widget.RemoveFromParent` _output))
  (set `PlayerController.bShowMouseCursor` false (`GameplayStatics.GetPlayerController` 0))
  (`GameplayStatics.SetGamePaused` false))

(event `InputAction|PauseMenu` :paused true
  (params (Key :type "Key Structure"))
  (:`Pressed`
    (goto _label)))

(fn `UserConstructionScript`)