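; Level-change trigger for the crypt exit ("WyjsciezKrypty") that sends the player to LEV_1.
; BeginPlay registers the Box with the BPInteractable component, along with a Polish key prompt.
; On interaction it shows a LoadScreen widget, saves the player, sets the game instance's LoadSaveName to "K" and opens the level.
; Older overlap-prompt and key-input logic remains unconnected.
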(event `self.ReceiveBeginPlay`
  (`/Game/Blueprints/Interactable/BP_Interactable.Init` (`self.BP_Interactable`) (`self.Box`) "Naciśnij {0} aby przejść"))

(event `self.BP_Interactable.Interacted`
  (`/Engine/EditorBlueprintResources/StandardMacros.IsValid` (stale _returnvalue)
    (:`Is Valid`
      _)
    (:`Is Not Valid`
      (bind _returnvalue (`|CreateWidget` "/Game/Widgets/LoadScreen.LoadScreen_C"))))
  (`UserWidget.AddToViewport` _returnvalue 0)
  (`SaveGamePlayerComponent.SavePlayer` (`self.GetComponentByClass` (`GameplayStatics.GetPlayerCharacter` 0) "/Script/Projekt_2_Rok.SaveGamePlayerComponent") "player")
  (set `FakeUpGameInstanceBase.LoadSaveName` "K" (cast `FakeUpGameInstanceBase` (`GameplayStatics.GetGameInstance`) :!pure true))
  (`GameplayStatics.OpenLevel` "LEV_1"))

(event `self.Box.OnComponentBeginOverlap`
  (params (OverlappedComponent :type "PrimitiveComponent Object Reference") (OtherActor :type "Actor Object Reference") (OtherComp :type "PrimitiveComponent Object Reference") (OtherBodyIndex :type Integer) (bFromSweep :type Boolean) (SweepResult :type "HitResult Structure (by ref)")))

(event `self.Box.OnComponentEndOverlap`
  (params (OverlappedComponent :type "PrimitiveComponent Object Reference") (OtherActor :type "Actor Object Reference") (OtherComp :type "PrimitiveComponent Object Reference") (OtherBodyIndex :type Integer)))

(event `InputAction|Interact`
  (params (Key :type "Key Structure")))

(fn `UserConstructionScript`)