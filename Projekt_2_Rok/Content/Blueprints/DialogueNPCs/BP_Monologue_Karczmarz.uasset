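; Innkeeper (Karczmarz) quest NPC running a staged fetch mission for crab meat, honey and wood via a spawned BP_DialogueController.
; Box overlap advances odd stages when the player holds the items and syncs the conversation ID; odd stages play random filler lines.
; Conversation end removes items, grants experience and advances even stages.
; Voice audio auto-advances lines, while a Timeline-bobbed marker signals a new quest or ready hand-in.
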(event `self.ReceiveBeginPlay`
  (bind _returnvalue (`|SpawnActorFromClass` "/Game/Blueprints/DialogueNPCs/BP_DialogueController.BP_DialogueController_C" (`KismetMathLibrary.MakeTransform` (0.0 0.0 0.0)) "Undefined" "OverrideRootScale" null null))
  (bind _output_get (set `self.DialogueController` _returnvalue))
  (`/Game/Blueprints/DialogueNPCs/BP_DialogueController.Init` _output_get (`self.NPC_ID`) self self "/Game/Blueprints/DialogueNPCs/Dialogi/002__Karczmarz_-_Pieczen_Z_Kraba.002__Karczmarz_-_Pieczen_Z_Kraba")
  (`/Game/Blueprints/Interactable/BP_Interactable.Init` (`self.BP_Interactable`) (`self.Box`) (`/Game/BP_GameInstance.String_NpcInteract` (`/Game/BP_Functions.GetFakeUpGameInstance`)))
  (add `AudioComponent.OnAudioFinished` (`self.Audio1`) (delegate `AudioFinished`))
  (`self.WyswietlZnacznik`)
  (`self.PoruszanieZnacznikiem`)
  (add `FakeUpGameInstanceBase.addedToInventoryDelegate` (`/Game/BP_Functions.GetFakeUpGameInstance`) (delegate `Added To Inv`)))

(event `Added To Inv`
  (params (InventoryItems :type "Array of PickupableActor Object Reference (by ref)"))
  (`self.SprawdzCzyMasz`))

(event `AudioFinished`
  (if (`/Game/Blueprints/DialogueNPCs/BP_DialogueController.IsOpen` (`self.DialogueController`))
    (`/Game/Blueprints/DialogueNPCs/BP_DialogueController.NextLine` (`self.DialogueController`))))

(event `/Game/Blueprints/DialogueNPCs/BP_DialogueControllerDelegate.ConversationDidEnd`
  (bind _returnvalue (`self.GetComponentByClass` (`GameplayStatics.GetPlayerCharacter` 0) "/Script/Projekt_2_Rok.PlayerInventory"))
  (bind (_valid _mission) (`/Game/BP_GameInstance.GetMissionForNpc` (cast `/Game/BP_GameInstance` (`GameplayStatics.GetGameInstance`) :!pure true) (`self.NPC_ID`)))
  (`SkeletalMeshComponent.Stop` (`self.SkeletalMesh`))
  (`SkeletalMeshComponent.SetAnimationMode` (`self.SkeletalMesh`) "AnimationBlueprint")
  (`AudioComponent.Stop` (`self.Audio1`))
  (if _valid
    (switch `int` (`.KtoraCzescMisji` (break `Misje` _mission))
      (:`0`
        _)
      (:`1`
        _)
      (:`2`
        (`PlayerInventory.RemoveFromInventoryString` _returnvalue "Krab_Mieso" 0)
        (`StatystykiPostaci.DodajDoswiadczenie` (`self.GetComponentByClass` (`GameplayStatics.GetPlayerCharacter` 0) "/Script/Projekt_2_Rok.StatystykiPostaci") (`|GetArrayItem` (`self.Dos`))))
      (:`3`
        _)
      (:`4`
        (`PlayerInventory.RemoveFromInventoryString` _returnvalue "Miod" 0)
        (`StatystykiPostaci.DodajDoswiadczenie` (`self.GetComponentByClass` (`GameplayStatics.GetPlayerCharacter` 0) "/Script/Projekt_2_Rok.StatystykiPostaci") (`|GetArrayItem` (`self.Dos`))))
      (:`5`
        _)
      (:`6`
        (`PlayerInventory.RemoveFromInventoryString` _returnvalue "Drewno" 0)
        (`StatystykiPostaci.DodajDoswiadczenie` (`self.GetComponentByClass` (`GameplayStatics.GetPlayerCharacter` 0) "/Script/Projekt_2_Rok.StatystykiPostaci") (`|GetArrayItem` (`self.Dos`))))
      (:`7`
        _))
    (bind (_valid_2 _mission_2) (`/Game/BP_GameInstance.AdvanceEvenMission` (cast `/Game/BP_GameInstance` (`GameplayStatics.GetGameInstance`) :!pure true) (`self.NPC_ID`)))
    (if _valid_2
      (set `self.Conversation_ID` (`.KtoraCzescMisji` (break `Misje` _mission_2)))
      (`self.WyswietlZnacznik`))))

(event `SprawdzCzyMasz`
  (if (or (`self.CzyMaszMieso`) (`self.CzyMaszMiod`) (`self.CzyMaszDrewno`))
    (`self.WyswietlZnacznik`)))

(event `self.BP_Interactable.Interacted`
  (bind _dialoguecontroller (`self.DialogueController`))
  (`self.SchowajZnacznik`)
  (if (not (`/Game/Blueprints/DialogueNPCs/BP_DialogueController.IsOpen` _dialoguecontroller))
    (`/Game/Blueprints/DialogueNPCs/BP_DialogueController.BeginConversation` _dialoguecontroller (`self.Conversation_ID`) 1)
    (`SceneComponent.K2_SetRelativeRotation` (`self.SkeletalMesh`) (`KismetMathLibrary.MakeRotator` 0.0 0.0 (.yaw (`KismetMathLibrary.FindLookAtRotation` (`self.K2_GetActorLocation`) (`self.K2_GetActorLocation` (`GameplayStatics.GetPlayerCharacter` 0))))) false false)
    (`SkeletalMeshComponent.PlayAnimation` (`self.SkeletalMesh`) "/Game/Mesh/Postacie/SM_karczmarz/SM_Karczmarz_gadanie.SM_Karczmarz_gadanie" true)))

(event `self.Box.OnComponentBeginOverlap`
  (params (OverlappedComponent :type "PrimitiveComponent Object Reference") (OtherActor :type "Actor Object Reference") (OtherComp :type "PrimitiveComponent Object Reference") (OtherBodyIndex :type Integer) (bFromSweep :type Boolean) (SweepResult :type "HitResult Structure (by ref)"))
  (bind _returnvalue (`self.GetComponentByClass` (`GameplayStatics.GetPlayerCharacter` 0) "/Script/Projekt_2_Rok.PlayerInventory"))
  (bind (_valid _mission) (`/Game/BP_GameInstance.GetMissionForNpc` (cast `/Game/BP_GameInstance` (`GameplayStatics.GetGameInstance`) :!pure true) (`self.NPC_ID`)))
  (bind (_valid_2 _mission_2) (`/Game/BP_GameInstance.GetMissionForNpc` (cast `/Game/BP_GameInstance` (`GameplayStatics.GetGameInstance`) :!pure true) (`self.NPC_ID`)))
  (if _valid_2
    (switch `int` (`.KtoraCzescMisji` (break `Misje` _mission_2))
      (:`0`
        _)
      (:`1`
        (bind _returnvalue_2 (`PlayerInventory.CheckIsInInventory` _returnvalue "Krab_Mieso" (`self.Ile_miesa`)))
        (if _returnvalue_2
          (`/Game/BP_GameInstance.AdvanceMission` (cast `/Game/BP_GameInstance` (`GameplayStatics.GetGameInstance`) :!pure true) (`self.NPC_ID`) 1 :!label _label)))
      (:`2`
        _)
      (:`3`
        (bind _returnvalue_3 (`PlayerInventory.CheckIsInInventory` _returnvalue "Miod" (`self.Ile_miodu`)))
        (if _returnvalue_3
          (goto _label)
          (else
            _)))
      (:`4`
        _)
      (:`5`
        (bind _returnvalue_4 (`PlayerInventory.CheckIsInInventory` _returnvalue "Drewno" (`self.Ile_drewna`)))
        (if _returnvalue_4
          (goto _label)
          (else
            _)))
      (:`6`
        _)
      (:`7`
        _))
    (if (== OtherActor (`GameplayStatics.GetPlayerCharacter` 0))
      (if _valid
        (set `self.Conversation_ID` (`.KtoraCzescMisji` (break `Misje` _mission)))))))

(event `/Game/Blueprints/DialogueNPCs/BP_DialogueControllerDelegate.PlayAudio`
  (params (Id :type Integer))
  (bind _audio1 (`self.Audio1`))
  (bind _asfake_up_game_instance_base (cast `FakeUpGameInstanceBase` (`GameplayStatics.GetGameInstance`))
    (:`then`
      (bind _returnvalue (/ (`KismetMathLibrary.Conv_IntToDouble` (`FakeUpGameInstanceBase.AudioDialogueLevel` _asfake_up_game_instance_base)) 10.0))
      (if (> _returnvalue 0.0)
        (`AudioComponent.SetVolumeMultiplier` (`self.Audio1`) _returnvalue)
        (else
          (`AudioComponent.SetVolumeMultiplier` (`self.Audio1`) 0.01 :!label _label_2))))
    (:`CastFailed`
      (goto _label_2)))
  ;[1 1 1] Otworzenie Dzwieku
  (if (`AudioComponent.IsPlaying` _audio1)
    (`AudioComponent.Stop` _audio1))
  (`AudioComponent.SetSound` _audio1 (`|GetArrayItem` (`self.TablicaWypowiedzi`) Id))
  (`AudioComponent.Play` _audio1 0.0))

(event `WyswietlZnacznik`
  ;[1 1 1] Wyswietl Znacznik
  (if (not (`/Game/Blueprints/DialogueNPCs/BP_DialogueController.IsOpen` (`self.DialogueController`)))
    (if (or (`self.CzyMaszMieso`) (`self.CzyMaszMiod`) (`self.CzyMaszDrewno`) (== (`.KtoraCzescMisji` (break `Misje` (`.Mission` (`/Game/BP_GameInstance.GetMissionForNpc` (cast `/Game/BP_GameInstance` (`GameplayStatics.GetGameInstance`) :!pure true) (`self.NPC_ID`))))) 0))
      (set `self.CzyJestPytajnik` true)
      (else
        (set `self.CzyJestPytajnik` false)))
    ;[1 1 1] Pytajnik
    (if (`self.CzyJestPytajnik`)
      (`SceneComponent.SetVisibility` (`self.Znacznik2`) true true)
      (else
        (`SceneComponent.SetVisibility` (`self.Znacznik2`) false true)))))

(event `SchowajZnacznik`
  ;[1 1 1] Schowaj Znacznik
  (`SceneComponent.SetVisibility` (`self.Znacznik2`) false true))

(event `PoruszanieZnacznikiem`
  (set `self.lokacjaDolna` (0.0 0.0 -40.0))
  (set `self.lokacjaGorna` (0.0 0.0 40.0))
  (bind _output_get (set `self.Startowa_lokacja` (`SceneComponent.RelativeLocation` (`self.Znacznik2`))))
  (`SceneComponent.K2_SetRelativeLocation` (`self.Znacznik2`) _output_get true false)
  (bind (_direction _newtrack_0) (`Timeline|Timeline_0` :!via `PlayFromStart` :!label _label_3)
    (:`Update`
      (`SceneComponent.K2_SetRelativeLocation` (`self.Znacznik2`) (+ (* (`self.lokacjaGorna`) _newtrack_0) (`self.Startowa_lokacja`)) false false))
    (:`Finished`
      (set `self.Startowa_lokacja` (`SceneComponent.RelativeLocation` (`self.Znacznik2`)))
      ;[1 1 1] Odpal Event Wyswietl Znacznik
      (`self.WyswietlZnacznik`)
      (bind (_direction_2 _newtrack_0_2) (`Timeline|Timeline_1` :!via `PlayFromStart`)
        (:`Update`
          (`SceneComponent.K2_SetRelativeLocation` (`self.Znacznik2`) (+ (* (`self.lokacjaDolna`) _newtrack_0_2) (`self.Startowa_lokacja`)) false false))
        (:`Finished`
          (set `self.Startowa_lokacja` (`SceneComponent.RelativeLocation` (`self.Znacznik2`)))
          (goto _label_3 :!via `PlayFromStart`))))))

(fn `CzyMaszDrewno`
  (returns (Mam :type Boolean))
  (bind _returnvalue (`PlayerInventory.CheckIsInInventory` (`self.GetComponentByClass` (`GameplayStatics.GetPlayerCharacter` 0) "/Script/Projekt_2_Rok.PlayerInventory") "Drewno" (`self.Ile_drewna`)))
  (if (and _returnvalue (or (== (`.KtoraCzescMisji` (break `Misje` (`.Mission` (`/Game/BP_GameInstance.GetMissionForNpc` (cast `/Game/BP_GameInstance` (`GameplayStatics.GetGameInstance`) :!pure true) (`self.NPC_ID`))))) 5) (== (`.KtoraCzescMisji` (break `Misje` (`.Mission` (`/Game/BP_GameInstance.GetMissionForNpc` (cast `/Game/BP_GameInstance` (`GameplayStatics.GetGameInstance`) :!pure true) (`self.NPC_ID`))))) 6)))
    (return true)
    (else
      (return false))))

(fn `CzyMaszMieso`
  (returns (Mam :type Boolean))
  (bind _returnvalue (`PlayerInventory.CheckIsInInventory` (`self.GetComponentByClass` (`GameplayStatics.GetPlayerCharacter` 0) "/Script/Projekt_2_Rok.PlayerInventory") "Krab_Mieso" (`self.Ile_miesa`)))
  (if (and _returnvalue (or (== (`.KtoraCzescMisji` (break `Misje` (`.Mission` (`/Game/BP_GameInstance.GetMissionForNpc` (cast `/Game/BP_GameInstance` (`GameplayStatics.GetGameInstance`) :!pure true) (`self.NPC_ID`))))) 1) (== (`.KtoraCzescMisji` (break `Misje` (`.Mission` (`/Game/BP_GameInstance.GetMissionForNpc` (cast `/Game/BP_GameInstance` (`GameplayStatics.GetGameInstance`) :!pure true) (`self.NPC_ID`))))) 2)))
    (return true)
    (else
      (return false))))

(fn `CzyMaszMiod`
  (returns (Mam :type Boolean))
  (bind _returnvalue (`PlayerInventory.CheckIsInInventory` (`self.GetComponentByClass` (`GameplayStatics.GetPlayerCharacter` 0) "/Script/Projekt_2_Rok.PlayerInventory") "Miod" (`self.Ile_miodu`)))
  (if (and _returnvalue (or (== (`.KtoraCzescMisji` (break `Misje` (`.Mission` (`/Game/BP_GameInstance.GetMissionForNpc` (cast `/Game/BP_GameInstance` (`GameplayStatics.GetGameInstance`) :!pure true) (`self.NPC_ID`))))) 3) (== (`.KtoraCzescMisji` (break `Misje` (`.Mission` (`/Game/BP_GameInstance.GetMissionForNpc` (cast `/Game/BP_GameInstance` (`GameplayStatics.GetGameInstance`) :!pure true) (`self.NPC_ID`))))) 4)))
    (return true)
    (else
      (return false))))

(fn `UserConstructionScript`)

(fn `WillGetLine`
  (params (CurrentConversation :type Integer) (CurrentLine :type Integer))
  (returns (NewConversation :type Integer) (NewLine :type Integer))
  (switch `int` CurrentConversation
    (:`0`
      _)
    (:`1`
      (return 1 (`KismetMathLibrary.RandomIntegerInRange` 1 4)))
    (:`2`
      _)
    (:`3`
      (return 1 (`KismetMathLibrary.RandomIntegerInRange` 1 4)))
    (:`4`
      _)
    (:`5`
      (return 1 (`KismetMathLibrary.RandomIntegerInRange` 1 4)))
    (:`6`
      _)
    (:`7`
      (return 1 (`KismetMathLibrary.RandomIntegerInRange` 1 4))))
  (return CurrentConversation CurrentLine))