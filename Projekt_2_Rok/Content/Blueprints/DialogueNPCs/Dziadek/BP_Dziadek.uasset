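; Floating dialogue NPC for Antoni's grandfather (Dziadek), offering a one-time voiced conversation that branches Antoni's mission.
; It spawns a BP_DialogueController with itself as delegate, playing per-line audio at the saved volume and auto-advancing when each clip finishes.
; Specific lines set mission parts in the GameInstance, and the first line disables further interaction.
; Ending dialogue triggers KostekSpawnController, stops the overlap-spawned Niagara particles and removes mission items from inventory.
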(event `self.ReceiveBeginPlay`
  (add `AudioComponent.OnAudioFinished` (`self.Audio`) (delegate `AudioFinished`))
  (bind _returnvalue (`|SpawnActorFromClass` "/Game/Blueprints/DialogueNPCs/BP_DialogueController.BP_DialogueController_C" (`KismetMathLibrary.MakeTransform` (0.0 0.0 0.0)) "Undefined" "OverrideRootScale" null null))
  (bind _output_get (set `self.DialogueController` _returnvalue))
  (`/Game/Blueprints/DialogueNPCs/BP_DialogueController.Init` _output_get (`self.NPC_ID`) self self "/Game/Blueprints/DialogueNPCs/Dialogi/10__Dziadek_Antoniego.10__Dziadek_Antoniego")
  (`/Game/Blueprints/Interactable/BP_Interactable.Init` (`self.BP_Interactable`) (`self.Box`) (`/Game/BP_GameInstance.String_NpcInteract` (`/Game/BP_Functions.GetFakeUpGameInstance`))))

(event `AudioFinished`
  (if (`/Game/Blueprints/DialogueNPCs/BP_DialogueController.IsOpen` (`self.DialogueController`))
    (`/Game/Blueprints/DialogueNPCs/BP_DialogueController.NextLine` (`self.DialogueController`))))

(event `/Game/Blueprints/DialogueNPCs/BP_DialogueControllerDelegate.ConversationDidEnd`
  (bind _returnvalue (`self.GetComponentByClass` (`GameplayStatics.GetPlayerCharacter` 0) "/Script/Projekt_2_Rok.PlayerInventory"))
  (bind (_valid _mission) (`/Game/BP_GameInstance.GetMissionForNpc` (cast `/Game/BP_GameInstance` (`GameplayStatics.GetGameInstance`) :!pure true) (`self.NPC_ID`)))
  (`AudioComponent.Stop` (`self.Audio`))
  (`/Game/Combat/Spawners/BP_KostekSpawnController.TriggerSpawn` (`self.kostekSpawnController`) true)
  (`NiagaraComponent.SetNiagaraVariableFloat` (`self.MeshParticles`) "User.SpawnRate" 0.0)
  (if _valid
    (switch `int` (`.KtoraCzescMisji` (break `Misje` _mission))
      (:`0`)
      (:`1`)
      (:`2`
        (`PlayerInventory.RemoveFromInventoryString` _returnvalue "Krab_Mieso" 0))
      (:`3`)
      (:`4`
        (`PlayerInventory.RemoveFromInventoryString` _returnvalue "Miod" 0))
      (:`5`)
      (:`6`
        (`PlayerInventory.RemoveFromInventoryString` _returnvalue "Drewno" 0))
      (:`7`))))

(event `self.BP_Interactable.Interacted`
  (bind _dialoguecontroller (`self.DialogueController`))
  (if (`/Game/Blueprints/DialogueNPCs/BP_DialogueController.IsOpen` _dialoguecontroller)
    _
    (elif (== (`self.Conversation_ID`) 0)
      (`/Game/Blueprints/DialogueNPCs/BP_DialogueController.BeginConversation` _dialoguecontroller (`self.Conversation_ID`) 1)
      (`SceneComponent.K2_SetRelativeRotation` (`self.SkeletalMesh`) (`KismetMathLibrary.MakeRotator` 0.0 0.0 (.yaw (`KismetMathLibrary.FindLookAtRotation` (`self.K2_GetActorLocation`) (`self.K2_GetActorLocation` (`GameplayStatics.GetPlayerCharacter` 0))))) false false))))

(event `self.BP_Interactable.ShouldShowInteract`
  (set `/Game/Blueprints/Interactable/BP_Interactable.Interactable` (== (`self.Conversation_ID`) 0) (`self.BP_Interactable`)))

(event `self.ReceiveTick`
  (params (DeltaSeconds :type "Float (single-precision)"))
  (`SceneComponent.K2_SetRelativeLocation` (`self.OffsetScene`) (`KismetMathLibrary.MakeVector` 0.0 0.0 (* (`KismetMathLibrary.Sin` (* (`KismetSystemLibrary.GetGameTimeInSeconds`) (`self.floatingSpeed`))) (`self.floatingHeigth`))) false false))

(event `self.Sphere.OnComponentBeginOverlap`
  (params (OverlappedComponent :type "PrimitiveComponent Object Reference") (OtherActor :type "Actor Object Reference") (OtherComp :type "PrimitiveComponent Object Reference") (OtherBodyIndex :type Integer) (bFromSweep :type Boolean) (SweepResult :type "HitResult Structure (by ref)"))
  (`/Engine/EditorBlueprintResources/StandardMacros.DoOnce` false
    (:`Completed`
      (bind _returnvalue (`NiagaraFunctionLibrary.SpawnSystemAttached` "/Game/Blueprints/DialogueNPCs/Dziadek/PS_Dziadek.PS_Dziadek" (`self.SkeletalMesh`) "None" (0.0 0.0 0.0) (struct) "KeepRelativeOffset"))
      (set `self.MeshParticles` _returnvalue))))

(event `/Game/Blueprints/DialogueNPCs/BP_DialogueControllerDelegate.DidMoveToNextLine`
  (params (ConversationId :type Integer) (LineId :type Integer))
  (`|ExecutionSequence`
    (:`then_0`
      ;[1 1 1] Droga do mozliwosc 1 u Antoniego
      (if (or (and (== ConversationId 0) (== LineId 12)) (and (== ConversationId 0) (== LineId 33)))
        ;[1 1 1] Aktywowanie event z GameInstance, ktory
        (`/Game/BP_GameInstance.SetMissionPart` (cast `/Game/BP_GameInstance` (`GameplayStatics.GetGameInstance`) :!pure true) (`self.ID_Zadania`) 2)))
    (:`then_1`
      ;[1 1 1] Droga do mozliwosc 2 u Antoniego
      (if (or (and (== ConversationId 0) (== LineId 14)) (and (== ConversationId 0) (== LineId 35)))
        ;[1 1 1] Aktywowanie event z GameInstance, ktory
        (`/Game/BP_GameInstance.SetMissionPart` (cast `/Game/BP_GameInstance` (`GameplayStatics.GetGameInstance`) :!pure true) (`self.ID_Zadania`) 3)))
    (:`then_2`
      ;[1 1 1] Droga do mozliwosc 3 u Antoniego
      (if (and (== ConversationId 1) (== LineId 16))
        ;[1 1 1] Aktywowanie event z GameInstance, ktory
        (`/Game/BP_GameInstance.SetMissionPart` (cast `/Game/BP_GameInstance` (`GameplayStatics.GetGameInstance`) :!pure true) (`self.ID_Zadania`) 4)))
    (:`then_3`
      ;[1 1 1] Droga do mozliwosc 4 u Antoniego
      (if (or (and (== ConversationId 0) (== LineId 18)) (and (== ConversationId 0) (== LineId 28)) (and (== ConversationId 0) (== LineId 37)) (and (== ConversationId 0) (== LineId 39)) (and (== ConversationId 0) (== LineId 41)))
        ;[1 1 1] Aktywowanie event z GameInstance, ktory
        (`/Game/BP_GameInstance.SetMissionPart` (cast `/Game/BP_GameInstance` (`GameplayStatics.GetGameInstance`) :!pure true) (`self.ID_Zadania`) 5)))
    (:`then_4`
      ;[1 1 1] Droga do mozliwosc 5 u Antoniego
      (if (and (== ConversationId 0) (== LineId 23))
        ;[1 1 1] Aktywowanie event z GameInstance, ktory
        (`/Game/BP_GameInstance.SetMissionPart` (cast `/Game/BP_GameInstance` (`GameplayStatics.GetGameInstance`) :!pure true) (`self.ID_Zadania`) 6)))
    (:`then_5`
      (if (and (== ConversationId 0) (== LineId 1))
        (set `self.Conversation_ID` 1)))))

(event `/Game/Blueprints/DialogueNPCs/BP_DialogueControllerDelegate.PlayAudio`
  (params (Id :type Integer))
  (bind _audio (`self.Audio`))
  (bind _asfake_up_game_instance_base (cast `FakeUpGameInstanceBase` (`GameplayStatics.GetGameInstance`))
    (:`then`
      (bind _returnvalue (/ (`KismetMathLibrary.Conv_IntToDouble` (`FakeUpGameInstanceBase.AudioDialogueLevel` _asfake_up_game_instance_base)) 10.0))
      (if (> _returnvalue 0.0)
        (`AudioComponent.SetVolumeMultiplier` (`self.Audio`) _returnvalue)
        (else
          (`AudioComponent.SetVolumeMultiplier` (`self.Audio`) 0.01 :!label _label))))
    (:`CastFailed`
      (goto _label)))
  ;[1 1 1] Otworzenie Dzwieku
  (if (`AudioComponent.IsPlaying` _audio)
    (`AudioComponent.Stop` _audio))
  (`AudioComponent.SetSound` _audio (`|GetArrayItem` (`self.TablicaWypowiedzi`) Id))
  (`AudioComponent.Play` _audio 0.0))

(fn `UserConstructionScript`)

(fn `WillGetLine`
  (params (CurrentConversation :type Integer) (CurrentLine :type Integer))
  (returns (NewConversation :type Integer) (NewLine :type Integer))
  (switch `int` CurrentConversation
    (:`0`
      _)
    (:`1`
      (return 1 (`KismetMathLibrary.RandomIntegerInRange` 1 4)))
    (:`2`
      _)
    (:`3`
      (return 1 (`KismetMathLibrary.RandomIntegerInRange` 1 4)))
    (:`4`
      _)
    (:`5`
      (return 1 (`KismetMathLibrary.RandomIntegerInRange` 1 4)))
    (:`6`
      _)
    (:`7`
      (return 1 (`KismetMathLibrary.RandomIntegerInRange` 1 4))))
  (return CurrentConversation CurrentLine))