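; Dialogue NPC Blueprint that opens an NPC widget when the player interacts nearby.
; A box overlap enables and disables the actor's input for the player character, so Interact is only handled in range.
; Interacting turns the skeletal mesh toward the player on yaw only, with an offset applied.
; It then creates or reuses the widget, shows the cursor, switches to Game and UI input and adds it to the viewport.
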(event `self.Box.OnComponentBeginOverlap`
  (params (OverlappedComponent :type "PrimitiveComponent Object Reference") (OtherActor :type "Actor Object Reference") (OtherComp :type "PrimitiveComponent Object Reference") (OtherBodyIndex :type Integer) (bFromSweep :type Boolean) (SweepResult :type "HitResult Structure (by ref)"))
  (if (== OtherActor (`GameplayStatics.GetPlayerCharacter` 0))
    (`self.EnableInput` (`GameplayStatics.GetPlayerController` 0))))

(event `self.Box.OnComponentEndOverlap`
  (params (OverlappedComponent :type "PrimitiveComponent Object Reference") (OtherActor :type "Actor Object Reference") (OtherComp :type "PrimitiveComponent Object Reference") (OtherBodyIndex :type Integer))
  (if (== (`GameplayStatics.GetPlayerCharacter` 0) OtherActor)
    (`self.DisableInput` (`GameplayStatics.GetPlayerController` 0))))

(event `InputAction|Interact`
  (params (Key :type "Key Structure"))
  (bind _returnvalue (`GameplayStatics.GetPlayerController` 0))
  (:`Pressed`
    (`SceneComponent.K2_SetRelativeRotation` (`self.SkeletalMesh`) (`KismetMathLibrary.MakeRotator` 0.0 0.0 (- (.yaw (`KismetMathLibrary.FindLookAtRotation` (`self.K2_GetActorLocation`) (`self.K2_GetActorLocation` (`GameplayStatics.GetPlayerCharacter` 0)))) 90.0)) false false)
    (`/Engine/EditorBlueprintResources/StandardMacros.IsValid` (stale _returnvalue_2)
      (:`Is Valid`
        _)
      (:`Is Not Valid`
        (bind _returnvalue_2 (`|CreateWidget` (`self.NPC_Widget`) _returnvalue))))
    (set `PlayerController.bShowMouseCursor` true _returnvalue)
    (if true
      (`WidgetBlueprintLibrary.SetInputMode_GameAndUIEx` _returnvalue _returnvalue_2)
      (`UserWidget.AddToViewport` _returnvalue_2 0))))

(fn `UserConstructionScript`)