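; Dialogue controller that runs branching, data-table-driven NPC conversations, managing the monologue widget, player input, HUD and camera.
; Init caches the NPC's row names; GetLine matches conversation and line IDs, treating SubLineID 0 as speech and others as options.
; CameraID switches the view between the camera target and player pawn.
; Target IDs drive advancing, jumping or ending, while a delegate can redirect lines, play audio and receive progress callbacks.
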(event `Init`
  (params (NPC_ID :type Integer) (CameraTarget :type "Actor Object Reference") (delegate :type "/Game/Blueprints/DialogueNPCs/BP_DialogueControllerDelegate Interface") (DataTable :type "DataTable Object Reference"))
  (set `self.DataBase` DataTable)
  (set `self.CameraTarget` CameraTarget)
  (set `self.Delegate` delegate)
  (bind _outrownames (`DataTableFunctionLibrary.GetDataTableRowNames` (`self.DataBase`)))
  (for _array_element _outrownames
    (bind _returnvalue (`|GetDataTableRow` (`self.DataBase`) _array_element)
      (:`then`
        (if (== (`.NPC_ID_2_9E5F1AFE438861BD878590833A92396C` (break `/Game/Blueprints/DialogueNPCs/S_Monologue` _returnvalue)) NPC_ID)
          (`KismetArrayLibrary.Array_Add` (`self.PossibleDialogues`) _array_element))))))

(event `InputAction|Interact`
  (params (Key :type "Key Structure"))
  (:`Pressed`
    (`self.NextLine`)))

(event `NextLine`
  (bind _targetline (`self.TargetLine`))
  (if (> (`KismetArrayLibrary.Array_Length` (`self.CurrentOptions`)) 0)
    _
    (elif (== _targetline -1)
      (`self.EndConversation`)
      (else
        (if (== _targetline 0)
          (`/Engine/EditorBlueprintResources/StandardMacros.IncrementInt` (`self.CurrentLine`)
            (:`  `
              _))
          (else
            (set `self.CurrentLine` (`self.TargetLine`))))
        (`self.UpdateLines`)))))

(event `BeginConversation`
  (params (ConversationID :type Integer) (LineId :type Integer :default 1))
  (bind _returnvalue (`GameplayStatics.GetPlayerController` 0))
  (set `self.CurrentConversation` ConversationID)
  (set `self.CurrentLine` LineId)
  (set `self.IsOpen` true)
  (set `PlayerController.bShowMouseCursor` true _returnvalue)
  (`self.EnableInput` _returnvalue)
  (bind _asthird_person_character (cast `/Game/ThirdPersonCPP/Blueprints/ThirdPersonCharacter` (`Controller.K2_GetPawn` _returnvalue)))
  (`/Game/ThirdPersonCPP/Blueprints/ThirdPersonCharacter.SetAllCharacterInputs` _asthird_person_character false)
  (`/Engine/EditorBlueprintResources/StandardMacros.IsValid` (`self.Widget`)
    (:`Is Valid`
      _)
    (:`Is Not Valid`
      (bind _returnvalue_2 (`|CreateWidget` "/Game/Blueprints/DialogueNPCs/Widget_Dialogue/W_Monologue.W_Monologue_C" (`GameplayStatics.GetPlayerController` 0)))
      (bind _output_get (set `self.Widget` _returnvalue_2))
      (`UserWidget.AddToViewport` _output_get 0)))
  (`self.UpdateLines`)
  (`self.SetHudVisible` false))

(event `EndConversation`
  (bind _returnvalue (`GameplayStatics.GetPlayerController` 0))
  (bind _returnvalue_2 (`GameplayStatics.GetPlayerController` 0))
  (set `self.IsOpen` false)
  (set `PlayerController.bShowMouseCursor` false _returnvalue)
  (`self.DisableInput` _returnvalue)
  (bind _asthird_person_character (cast `/Game/ThirdPersonCPP/Blueprints/ThirdPersonCharacter` (`Controller.K2_GetPawn` _returnvalue)))
  (`/Game/ThirdPersonCPP/Blueprints/ThirdPersonCharacter.SetAllCharacterInputs` _asthird_person_character true)
  (`Widget.RemoveFromParent` (`self.Widget`))
  (set `self.Widget` null)
  ;[1 1 1] Return back camera
  (if (`self.EndConversationCameraReturn`)
    (`PlayerController.SetViewTargetWithBlend` _returnvalue_2 (`Controller.K2_GetPawn` _returnvalue_2) 0.0 "VTBlend_Linear" 0.0 false))
  (bind _asthird_person_character_2 (cast `/Game/ThirdPersonCPP/Blueprints/ThirdPersonCharacter` (`GameplayStatics.GetPlayerCharacter` 0)))
  (`/Game/ThirdPersonCPP/Blueprints/ThirdPersonCharacter.End conversation` _asthird_person_character_2)
  (`/Game/Blueprints/DialogueNPCs/BP_DialogueControllerDelegate.ConversationDidEnd` (`self.Delegate`))
  (`self.SetHudVisible` true))

(event `/Game/Blueprints/DialogueNPCs/BP_DialogueOptionSelected.OptionSelected`
  (params (Option :type Integer))
  (bind (_text _targetlineid) (break `/Game/Blueprints/DialogueNPCs/BP_DialogueOption` (`|GetArrayItem` (`self.CurrentOptions`) Option)))
  (if (== Option -1)
    (`self.NextLine`)
    (elif (> _targetlineid 0)
      (set `self.CurrentLine` _targetlineid)
      (`self.UpdateLines`)
      (else
        (`self.EndConversation`)))))

(event `UpdateLines`
  (`/Game/Blueprints/DialogueNPCs/BP_DialogueControllerDelegate.DidMoveToNextLine` (`self.Delegate`) (`self.CurrentConversation`) (`self.CurrentLine`))
  (bind (_id_ _valid _line_ _targetline_ _options) (`self.GetLine` (`self.CurrentConversation`) (`self.CurrentLine`)))
  (set `self.CurrentText` (select `bool` (`KismetTextLibrary.TextIsEmpty` _line_) :`false` _line_ :`true` (`self.CurrentText`)))
  (set `self.CurrentOptions` _options)
  (set `self.TargetLine` _targetline_)
  (if _valid
    (`/Game/Blueprints/DialogueNPCs/BP_DialogueControllerDelegate.PlayAudio` (`self.Delegate`) _id_)
    (set `/Game/Blueprints/DialogueNPCs/Widget_Dialogue/W_Monologue.MonologueText` (`self.CurrentText`) (`self.Widget`))
    (`/Game/Blueprints/DialogueNPCs/Widget_Dialogue/W_Monologue.AddOptions` (`self.Widget`) (`self.ConvertOptions` _options) self)
    (else
      (`self.EndConversation`))))

(event `SetData`
  (params (ConversationId :type Integer) (LineId :type Integer))
  (set `self.CurrentConversation` ConversationId)
  (set `self.CurrentLine` LineId))

(event `SetHudVisible`
  (params (Visible :type Boolean))
  (bind _asbp_hud (cast `/Game/Combat/Ui/BP_Hud` (`PlayerController.GetHUD` (`GameplayStatics.GetPlayerController` 0))))
  (`/Game/Combat/Ui/BP_Hud.SetHudVisible` _asbp_hud Visible))

(fn `ConvertOptions`
  (params (options :type "Array of /Game/Blueprints/DialogueNPCs/BP_DialogueOption Structure"))
  (returns (result :type "Array of Text"))
  (locals (Result_ :type "Array of Text"))
  (for _array_element options
    (`KismetArrayLibrary.Array_Add` (`local.Result_`) (`.Text_2_0A8303DF45403A2B60CF75868F2E8FBA` (break `/Game/Blueprints/DialogueNPCs/BP_DialogueOption` _array_element))))
  (return (`local.Result_`)))

(fn `GetLine`
  (params (ConversationId :type Integer) (LineId :type Integer))
  (returns (Id_ :type Integer) (Valid :type Boolean) (Line_ :type Text) (TargetLine_ :type Integer) (Options :type "Array of /Game/Blueprints/DialogueNPCs/BP_DialogueOption Structure"))
  (locals (ResultLines :type "Array of Text") (ResultOptions :type "Array of /Game/Blueprints/DialogueNPCs/BP_DialogueOption Structure") (ResultCameras :type "Array of Integer") (ResultTargetLines :type "Array of Integer") (TempConversation :type Integer) (TempLine :type Integer) (Id :type Integer))
  (bind _returnvalue (`GameplayStatics.GetPlayerController` 0))
  (bind _resultcameras (`local.ResultCameras`))
  (bind _resultlines (`local.ResultLines`))
  (bind (_newconversation _newline) (`/Game/Blueprints/DialogueNPCs/BP_DialogueControllerDelegate.WillGetLine` (`self.Delegate`) ConversationId LineId))
  (set `local.TempConversation` _newconversation)
  (set `local.TempLine` _newline)
  (for _array_element (`self.PossibleDialogues`)
    (bind _returnvalue_2 (`|GetDataTableRow` (`self.DataBase`) _array_element)
      (:`then`
        (bind (_id _npc_id _conversation_id _line_id _subline_id _targetline_id _camera_id _monologue) (break `/Game/Blueprints/DialogueNPCs/S_Monologue` _returnvalue_2))
        (if (and (== (`local.TempConversation`) _conversation_id) (== (`local.TempLine`) _line_id))
          (if (== _subline_id 0)
            (`KismetArrayLibrary.Array_Add` (`local.ResultLines`) _monologue)
            (`KismetArrayLibrary.Array_Add` (`local.ResultCameras`) _camera_id)
            (`KismetArrayLibrary.Array_Add` (`local.ResultTargetLines`) _targetline_id)
            (set `local.Id` _id)
            (else
              (`KismetArrayLibrary.Array_Add` (`local.ResultOptions`) (make `/Game/Blueprints/DialogueNPCs/BP_DialogueOption` _monologue _targetline_id))))))))
  (if (== (`KismetArrayLibrary.Array_Length` _resultcameras) 1)
    (switch `int` (`|GetArrayItem` _resultcameras)
      (:`0`
        (`PlayerController.SetViewTargetWithBlend` _returnvalue (`self.CameraTarget`) 0.0 "VTBlend_Linear" 0.0 false))
      (:`1`
        (`PlayerController.SetViewTargetWithBlend` _returnvalue (`Controller.K2_GetPawn` _returnvalue) 0.0 "VTBlend_Linear" 0.0 false)
        (bind _asthird_person_character (cast `/Game/ThirdPersonCPP/Blueprints/ThirdPersonCharacter` (`GameplayStatics.GetPlayerCharacter` 0)))
        (`/Game/ThirdPersonCPP/Blueprints/ThirdPersonCharacter.Switch camera` _asthird_person_character (`self.CameraTarget`)))))
  (return (`local.Id`) (>= (`KismetArrayLibrary.Array_Length` _resultlines) 1) (`|GetArrayItem` _resultlines) (`|GetArrayItem` (`local.ResultTargetLines`)) (`local.ResultOptions`)))

(fn `UserConstructionScript`)