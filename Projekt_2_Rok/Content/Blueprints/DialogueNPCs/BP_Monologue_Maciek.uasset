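; Monologue NPC for Maciek that plays a voiced one-way dialogue after a cinematic ends, then records mission progress and removes itself.
; It spawns a dialogue controller with itself as delegate and camera target, looping a random talking animation during the conversation.
; Each line's sound plays at the saved dialogue volume, and audio completion advances to the next line.
; A trigger box toggles input and reads the NPC's mission part, though the conversation always starts at ID 0.
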(event `self.ReceiveBeginPlay`
  (bind _returnvalue (`|SpawnActorFromClass` "/Game/Blueprints/DialogueNPCs/BP_DialogueController.BP_DialogueController_C" (`KismetMathLibrary.MakeTransform` (0.0 0.0 0.0)) "Undefined" "OverrideRootScale" null null))
  (bind _output_get (set `self.DialogueController` _returnvalue))
  (`/Game/Blueprints/DialogueNPCs/BP_DialogueController.Init` _output_get (`self.NPC_ID`) self self "/Game/Blueprints/DialogueNPCs/Dialogi/001__Maciek_-_Nieśmiertelna_Klątwa_1.001__Maciek_-_Nieśmiertelna_Klątwa_1")
  (add `AudioComponent.OnAudioFinished` (`self.Audio`) (delegate `AudioFinished`)))

(event `AudioFinished`
  (if (`/Game/Blueprints/DialogueNPCs/BP_DialogueController.IsOpen` (`self.DialogueController`))
    (`/Game/Blueprints/DialogueNPCs/BP_DialogueController.NextLine` (`self.DialogueController`))))

(event `CinematicEnded`
  (bind _gadanieanim (`self.GadanieAnim`))
  (`SkeletalMeshComponent.PlayAnimation` (`self.SkeletalMesh`) (`|GetArrayItem` _gadanieanim (`KismetMathLibrary.RandomIntegerInRange` 0 (- (`KismetArrayLibrary.Array_Length` _gadanieanim) 1))) true)
  (`/Game/Blueprints/DialogueNPCs/BP_DialogueController.BeginConversation` (`self.DialogueController`) 0 1))

(event `/Game/Blueprints/DialogueNPCs/BP_DialogueControllerDelegate.ConversationDidEnd`
  (`AudioComponent.Stop` (`self.Audio`))
  (`SkeletalMeshComponent.Stop` (`self.SkeletalMesh`))
  (`SkeletalMeshComponent.SetAnimationMode` (`self.SkeletalMesh`) "AnimationBlueprint")
  (`/Game/BP_GameInstance.SetMissionPart` (cast `/Game/BP_GameInstance` (`GameplayStatics.GetGameInstance`) :!pure true) (`self.NPC_ID`) 1)
  (`self.K2_DestroyActor` (`self.DialogueController`))
  (`self.K2_DestroyActor`))

(event `self.Box.OnComponentBeginOverlap`
  (params (OverlappedComponent :type "PrimitiveComponent Object Reference") (OtherActor :type "Actor Object Reference") (OtherComp :type "PrimitiveComponent Object Reference") (OtherBodyIndex :type Integer) (bFromSweep :type Boolean) (SweepResult :type "HitResult Structure (by ref)"))
  (bind (_valid _mission) (`/Game/BP_GameInstance.GetMissionForNpc` (cast `/Game/BP_GameInstance` (`GameplayStatics.GetGameInstance`) :!pure true) (`self.NPC_ID`)))
  (if (== OtherActor (`GameplayStatics.GetPlayerCharacter` 0))
    (`self.EnableInput` (`GameplayStatics.GetPlayerController` 0))
    (if _valid
      (set `self.Conversation_ID` (`.KtoraCzescMisji` (break `Misje` _mission))))))

(event `self.Box.OnComponentEndOverlap`
  (params (OverlappedComponent :type "PrimitiveComponent Object Reference") (OtherActor :type "Actor Object Reference") (OtherComp :type "PrimitiveComponent Object Reference") (OtherBodyIndex :type Integer))
  (if (== (`GameplayStatics.GetPlayerCharacter` 0) OtherActor)
    (`self.DisableInput` (`GameplayStatics.GetPlayerController` 0))))

(event `/Game/Blueprints/DialogueNPCs/BP_DialogueControllerDelegate.PlayAudio`
  (params (Id :type Integer))
  (bind _audio (`self.Audio`))
  (bind _asfake_up_game_instance_base (cast `FakeUpGameInstanceBase` (`GameplayStatics.GetGameInstance`))
    (:`then`
      (bind _returnvalue (/ (`KismetMathLibrary.Conv_IntToDouble` (`FakeUpGameInstanceBase.AudioDialogueLevel` _asfake_up_game_instance_base)) 10.0))
      (if (> _returnvalue 0.0)
        (`AudioComponent.SetVolumeMultiplier` (`self.Audio`) _returnvalue)
        (else
          (`AudioComponent.SetVolumeMultiplier` (`self.Audio`) 0.01 :!label _label))))
    (:`CastFailed`
      (goto _label)))
  ;[1 1 1] Otworzenie Dzwieku
  (if (`AudioComponent.IsPlaying` _audio)
    (`AudioComponent.Stop` _audio))
  (`AudioComponent.SetSound` _audio (`|GetArrayItem` (`self.TablicaWypowiedzi`) Id))
  (`AudioComponent.Play` _audio 0.0))

(fn `UserConstructionScript`)

(fn `WillGetLine`
  (params (CurrentConversation :type Integer) (CurrentLine :type Integer))
  (returns (NewConversation :type Integer) (NewLine :type Integer))
  (return CurrentConversation CurrentLine))