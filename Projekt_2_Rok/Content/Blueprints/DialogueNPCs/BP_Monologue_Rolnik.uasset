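; Farmer (Rolnik) quest NPC that talks through a spawned BP_DialogueController and runs a staged fetch mission for crab meat, honey and wood.
; Entering its box enables Interact input and advances the mission stage from GameInstance when PlayerInventory holds the required item.
; Interacting turns the mesh toward the player and opens that stage's conversation; ending it clears delivered items and calls AdvanceEvenMission.
; WillGetLine redirects odd stages to random filler lines in conversation 1.
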(event `self.ReceiveBeginPlay`
  (bind _returnvalue (`|SpawnActorFromClass` "/Game/Blueprints/DialogueNPCs/BP_DialogueController.BP_DialogueController_C" (`KismetMathLibrary.MakeTransform` (0.0 0.0 0.0)) "Undefined" "OverrideRootScale" null null))
  (bind _output_get (set `self.DialogueController` _returnvalue))
  (`/Game/Blueprints/DialogueNPCs/BP_DialogueController.Init` _output_get (`self.NPC_ID`) self self "/Game/Blueprints/DialogueNPCs/Dialogi/06__Zadanie_od_Rolnikiem.06__Zadanie_od_Rolnikiem"))

(event `/Game/Blueprints/DialogueNPCs/BP_DialogueControllerDelegate.ConversationDidEnd`
  (bind _returnvalue (`self.GetComponentByClass` (`GameplayStatics.GetPlayerCharacter` 0) "/Script/Projekt_2_Rok.PlayerInventory"))
  (bind (_valid _mission) (`/Game/Blueprints/DialogueNPCs/NewGameInstance.GetMissionForNpc` (cast `/Game/Blueprints/DialogueNPCs/NewGameInstance` (`GameplayStatics.GetGameInstance`) :!pure true) (`self.NPC_ID`)))
  (if _valid
    (switch `int` (`.KtoraCzescMisji` (break `Misje` _mission))
      (:`0`
        _)
      (:`1`
        _)
      (:`2`
        (`PlayerInventory.RemoveFromInventoryString` _returnvalue "Krab_Mieso" 0))
      (:`3`
        _)
      (:`4`
        (`PlayerInventory.RemoveFromInventoryString` _returnvalue "Miod" 0))
      (:`5`
        _)
      (:`6`
        (`PlayerInventory.RemoveFromInventoryString` _returnvalue "Drewno" 0))
      (:`7`
        _))
    (bind (_valid_2 _mission_2) (`/Game/Blueprints/DialogueNPCs/NewGameInstance.AdvanceEvenMission` (cast `/Game/Blueprints/DialogueNPCs/NewGameInstance` (`GameplayStatics.GetGameInstance`) :!pure true) (`self.NPC_ID`)))
    (if _valid_2
      (set `self.Conversation_ID` (`.KtoraCzescMisji` (break `Misje` _mission_2))))))

(event `InputAction|Interact`
  (params (Key :type "Key Structure"))
  (bind _dialoguecontroller (`self.DialogueController`))
  (:`Pressed`
    (if (not (`/Game/Blueprints/DialogueNPCs/BP_DialogueController.IsOpen` _dialoguecontroller))
      (`/Game/Blueprints/DialogueNPCs/BP_DialogueController.BeginConversation` _dialoguecontroller (`self.Conversation_ID`) 1)
      (`SceneComponent.K2_SetRelativeRotation` (`self.SkeletalMesh`) (`KismetMathLibrary.MakeRotator` 0.0 0.0 (.yaw (`KismetMathLibrary.FindLookAtRotation` (`self.K2_GetActorLocation`) (`self.K2_GetActorLocation` (`GameplayStatics.GetPlayerCharacter` 0))))) false false))))

(event `self.Box.OnComponentBeginOverlap`
  (params (OverlappedComponent :type "PrimitiveComponent Object Reference") (OtherActor :type "Actor Object Reference") (OtherComp :type "PrimitiveComponent Object Reference") (OtherBodyIndex :type Integer) (bFromSweep :type Boolean) (SweepResult :type "HitResult Structure (by ref)"))
  (bind _returnvalue (`self.GetComponentByClass` (`GameplayStatics.GetPlayerCharacter` 0) "/Script/Projekt_2_Rok.PlayerInventory"))
  (bind (_valid _mission) (`/Game/Blueprints/DialogueNPCs/NewGameInstance.GetMissionForNpc` (cast `/Game/Blueprints/DialogueNPCs/NewGameInstance` (`GameplayStatics.GetGameInstance`) :!pure true) (`self.NPC_ID`)))
  (bind (_valid_2 _mission_2) (`/Game/Blueprints/DialogueNPCs/NewGameInstance.GetMissionForNpc` (cast `/Game/Blueprints/DialogueNPCs/NewGameInstance` (`GameplayStatics.GetGameInstance`) :!pure true) (`self.NPC_ID`)))
  (if _valid_2
    (switch `int` (`.KtoraCzescMisji` (break `Misje` _mission_2))
      (:`0`
        _)
      (:`1`
        (bind _returnvalue_2 (`PlayerInventory.CheckIsInInventory` _returnvalue "Krab_Mieso" (`self.Ile_miesa`)))
        (if _returnvalue_2
          (`/Game/Blueprints/DialogueNPCs/NewGameInstance.AdvanceMission` (cast `/Game/Blueprints/DialogueNPCs/NewGameInstance` (`GameplayStatics.GetGameInstance`) :!pure true) (`self.NPC_ID`) :!label _label)))
      (:`2`
        _)
      (:`3`
        (bind _returnvalue_3 (`PlayerInventory.CheckIsInInventory` _returnvalue "Miod" (`self.Ile_miodu`)))
        (if _returnvalue_3
          (goto _label)
          (else
            _)))
      (:`4`
        _)
      (:`5`
        (bind _returnvalue_4 (`PlayerInventory.CheckIsInInventory` _returnvalue "Drewno" (`self.Ile_drewna`)))
        (if _returnvalue_4
          (goto _label)
          (else
            _)))
      (:`6`
        _)
      (:`7`
        _))
    (if (== OtherActor (`GameplayStatics.GetPlayerCharacter` 0))
      (`self.EnableInput` (`GameplayStatics.GetPlayerController` 0))
      (if _valid
        (set `self.Conversation_ID` (`.KtoraCzescMisji` (break `Misje` _mission)))))))

(event `self.Box.OnComponentEndOverlap`
  (params (OverlappedComponent :type "PrimitiveComponent Object Reference") (OtherActor :type "Actor Object Reference") (OtherComp :type "PrimitiveComponent Object Reference") (OtherBodyIndex :type Integer))
  (if (== (`GameplayStatics.GetPlayerCharacter` 0) OtherActor)
    (`self.DisableInput` (`GameplayStatics.GetPlayerController` 0))))

(fn `UserConstructionScript`)

(fn `WillGetLine`
  (params (CurrentConversation :type Integer) (CurrentLine :type Integer))
  (returns (NewConversation :type Integer) (NewLine :type Integer))
  (switch `int` CurrentConversation
    (:`0`
      _)
    (:`1`
      (return 1 (`KismetMathLibrary.RandomIntegerInRange` 1 4)))
    (:`2`
      _)
    (:`3`
      (return 1 (`KismetMathLibrary.RandomIntegerInRange` 1 4)))
    (:`4`
      _)
    (:`5`
      (return 1 (`KismetMathLibrary.RandomIntegerInRange` 1 4)))
    (:`6`
      _)
    (:`7`
      (return 1 (`KismetMathLibrary.RandomIntegerInRange` 1 4))))
  (return CurrentConversation CurrentLine))