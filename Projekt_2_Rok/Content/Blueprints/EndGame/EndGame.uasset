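; EndGame is a trigger actor that shows the end-game screen when the player reaches it at the right mission stage.
; On Box overlap by the player character, it checks through BP_GameInstance that NPC 3's mission is at part 5.
; It then pauses the game, creates or reuses EndGameWidget, adds it to the viewport and switches input to UI only.
; A TODO marks the mission check for review.
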(event `self.Box.OnComponentBeginOverlap`
  (params (OverlappedComponent :type "PrimitiveComponent Object Reference") (OtherActor :type "Actor Object Reference") (OtherComp :type "PrimitiveComponent Object Reference") (OtherBodyIndex :type Integer) (bFromSweep :type Boolean) (SweepResult :type "HitResult Structure (by ref)"))
  (bind _returnvalue (`GameplayStatics.GetPlayerController` 0))
  (if (== OtherActor (`GameplayStatics.GetPlayerCharacter` 0))
    ;[1 1 1] TODO sprawdzić zadanie
    (if (== (`.KtoraCzescMisji` (break `Misje` (`.Mission` (`/Game/BP_GameInstance.GetMissionForNpc` (cast `/Game/BP_GameInstance` (`GameplayStatics.GetGameInstance`) :!pure true) 3)))) 5)
      (`GameplayStatics.SetGamePaused` true)
      (`/Engine/EditorBlueprintResources/StandardMacros.IsValid` (stale _returnvalue_2)
        (:`Is Valid`
          _)
        (:`Is Not Valid`
          (bind _returnvalue_2 (`|CreateWidget` "/Game/Widgets/EndGameW/EndGameWidget.EndGameWidget_C" _returnvalue))))
      (`UserWidget.AddToViewport` _returnvalue_2 0)
      (`WidgetBlueprintLibrary.SetInputMode_UIOnlyEx` _returnvalue _returnvalue_2))))

(fn `UserConstructionScript`)