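; Interactable loot container actor that shows a pickup prompt while the player overlaps its collider and enables input on itself.
; Interact opens a ContainerMain widget seeded with the stored Content, switches to game-and-UI input and plays the chest's opening animation.
; Leaving, pausing or pressing gamepad B copies Content back from the widget, closes it, restores game input and plays the closing animation.
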(event `self.Colider.OnComponentBeginOverlap`
  (params (OverlappedComponent :type "PrimitiveComponent Object Reference") (OtherActor :type "Actor Object Reference") (OtherComp :type "PrimitiveComponent Object Reference") (OtherBodyIndex :type Integer) (bFromSweep :type Boolean) (SweepResult :type "HitResult Structure (by ref)"))
  (if (== OtherActor (`GameplayStatics.GetPlayerCharacter` 0))
    (`/Engine/EditorBlueprintResources/StandardMacros.IsValid` (stale `self.Colider.OnComponentBeginOverlap` _returnvalue)
      (:`Is Valid`
        _)
      (:`Is Not Valid`
        (bind _returnvalue (`|CreateWidget` "/Game/Widgets/Inventory/Press_E_to_Pickup.Press_E_to_Pickup_C" (`GameplayStatics.GetPlayerController` 0)))))
    (`UserWidget.AddToViewport` _returnvalue 0)
    (`self.EnableInput` (`GameplayStatics.GetPlayerController` 0))))

(event `self.Colider.OnComponentEndOverlap`
  (params (OverlappedComponent :type "PrimitiveComponent Object Reference") (OtherActor :type "Actor Object Reference") (OtherComp :type "PrimitiveComponent Object Reference") (OtherBodyIndex :type Integer))
  (if (== OtherActor (`GameplayStatics.GetPlayerCharacter` 0))
    (`/Engine/EditorBlueprintResources/StandardMacros.IsValid` (stale `self.Colider.OnComponentBeginOverlap` _returnvalue)
      (:`Is Valid`
        (`Widget.RemoveFromParent` (stale `self.Colider.OnComponentBeginOverlap` _returnvalue)))
      (:`Is Not Valid`
        _))
    (`self.DisableInput` (`GameplayStatics.GetPlayerController` 0))
    (set `self.content` (`/Game/Widgets/Container/ContainerMain.Content` (stale `InputAction|Interact` _returnvalue)))
    (`/Engine/EditorBlueprintResources/StandardMacros.IsValid` (stale `InputAction|Interact` _returnvalue)
      (:`Is Valid`
        (`Widget.RemoveFromParent` (stale `InputAction|Interact` _returnvalue)))
      (:`Is Not Valid`
        _))
    (`WidgetBlueprintLibrary.SetInputMode_GameOnly` (`GameplayStatics.GetPlayerController` 0))
    (set `self.iscontentset` false)
    (if (`self.isOpen`)
      (`SkeletalMeshComponent.PlayAnimation` (`self.Skszynia`) "/Game/Blueprints/Containers/SM_Skszynia/SM_Skszynia_zamykanie.SM_Skszynia_zamykanie" false)
      (set `self.isOpen` false))))

(event `InputAction|Interact`
  (params (Key :type "Key Structure"))
  (:`Pressed`
    (`/Engine/EditorBlueprintResources/StandardMacros.IsValid` (stale `self.Colider.OnComponentBeginOverlap` _returnvalue)
      (:`Is Valid`
        (`Widget.RemoveFromParent` (stale `self.Colider.OnComponentBeginOverlap` _returnvalue)))
      (:`Is Not Valid`
        _))
    (`/Engine/EditorBlueprintResources/StandardMacros.IsValid` (stale `InputAction|Interact` _returnvalue)
      (:`Is Valid`
        _)
      (:`Is Not Valid`
        (bind _returnvalue (`|CreateWidget` "/Game/Widgets/Container/ContainerMain.ContainerMain_C" (`GameplayStatics.GetPlayerController` 0)))))
    (if (not (`self.iscontentset`))
      (set `/Game/Widgets/Container/ContainerMain.Content` (`self.content`) _returnvalue)
      (set `self.iscontentset` true))
    (`UserWidget.AddToViewport` _returnvalue 0)
    (`WidgetBlueprintLibrary.SetInputMode_GameAndUIEx` (`GameplayStatics.GetPlayerController` 0) _returnvalue "LockAlways")
    (if (not (`self.isOpen`))
      (`SkeletalMeshComponent.PlayAnimation` (`self.Skszynia`) "/Game/Blueprints/Containers/SM_Skszynia/SM_Skszynia_otwieranie_Anim.SM_Skszynia_otwieranie_Anim" false)
      (set `self.isOpen` true))))

(event `InputAction|PauseMenu`
  (params (Key :type "Key Structure"))
  (:`Pressed`
    (`/Engine/EditorBlueprintResources/StandardMacros.IsValid` (stale `self.Colider.OnComponentBeginOverlap` _returnvalue) :!label _label
      (:`Is Valid`
        _)
      (:`Is Not Valid`
        (bind _returnvalue (`|CreateWidget` "/Game/Widgets/Inventory/Press_E_to_Pickup.Press_E_to_Pickup_C" (`GameplayStatics.GetPlayerController` 0)))))
    (`UserWidget.AddToViewport` _returnvalue 0)
    (set `self.content` (`/Game/Widgets/Container/ContainerMain.Content` (stale `InputAction|Interact` _returnvalue)))
    (`/Engine/EditorBlueprintResources/StandardMacros.IsValid` (stale `InputAction|Interact` _returnvalue)
      (:`Is Valid`
        (`Widget.RemoveFromParent` (stale `InputAction|Interact` _returnvalue)))
      (:`Is Not Valid`
        _))
    (set `self.iscontentset` false)
    (`WidgetBlueprintLibrary.SetInputMode_GameOnly` (`GameplayStatics.GetPlayerController` 0))
    (if (`self.isOpen`)
      (`SkeletalMeshComponent.PlayAnimation` (`self.Skszynia`) "/Game/Blueprints/Containers/SM_Skszynia/SM_Skszynia_zamykanie.SM_Skszynia_zamykanie" false)
      (set `self.isOpen` false))))

(event `Key|AnyKey` :consume false :overrideparent false
  (params (Key :type "Key Structure"))
  (:`Pressed`
    (if (== Key "Gamepad_FaceButton_Right")
      (goto _label))))

(fn `UserConstructionScript`)