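; Trigger volume that switches forest and water ambient sound for the player.
; On box overlap by player 0, its two toggles decide which ambient flags are set on FakeUpGameInstanceBase.
; An enabled type calls Ambient on ThirdPersonCharacter, while a disabled one calls its StopForest or StopWater.
; Leaving the box stops both sounds and clears both flags.
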(event `self.Box.OnComponentBeginOverlap`
  (params (OverlappedComponent :type "PrimitiveComponent Object Reference") (OtherActor :type "Actor Object Reference") (OtherComp :type "PrimitiveComponent Object Reference") (OtherBodyIndex :type Integer) (bFromSweep :type Boolean) (SweepResult :type "HitResult Structure (by ref)"))
  (if (== OtherActor (`GameplayStatics.GetPlayerCharacter` 0))
    (if (`self.PlayForestAmbient`)
      (bind _asfake_up_game_instance_base (cast `FakeUpGameInstanceBase` (`GameplayStatics.GetGameInstance`)))
      (set `FakeUpGameInstanceBase.AmbientForest` true _asfake_up_game_instance_base)
      (bind _asthird_person_character (cast `/Game/ThirdPersonCPP/Blueprints/ThirdPersonCharacter` (`GameplayStatics.GetPlayerCharacter` 0)))
      (`/Game/ThirdPersonCPP/Blueprints/ThirdPersonCharacter.Ambient` _asthird_person_character "")
      (else
        (bind _asthird_person_character_2 (cast `/Game/ThirdPersonCPP/Blueprints/ThirdPersonCharacter` (`GameplayStatics.GetPlayerCharacter` 0)))
        (`/Game/ThirdPersonCPP/Blueprints/ThirdPersonCharacter.StopForest` _asthird_person_character_2)
        (bind _asfake_up_game_instance_base_2 (cast `FakeUpGameInstanceBase` (`GameplayStatics.GetGameInstance`)))
        (set `FakeUpGameInstanceBase.AmbientForest` false _asfake_up_game_instance_base_2)))
    (if (`self.PlayWaterAmbient`)
      (bind _asfake_up_game_instance_base_3 (cast `FakeUpGameInstanceBase` (`GameplayStatics.GetGameInstance`)))
      (set `FakeUpGameInstanceBase.AmbientWater` true _asfake_up_game_instance_base_3)
      (bind _asthird_person_character_3 (cast `/Game/ThirdPersonCPP/Blueprints/ThirdPersonCharacter` (`GameplayStatics.GetPlayerCharacter` 0)))
      (`/Game/ThirdPersonCPP/Blueprints/ThirdPersonCharacter.Ambient` _asthird_person_character_3 "")
      (else
        (bind _asthird_person_character_4 (cast `/Game/ThirdPersonCPP/Blueprints/ThirdPersonCharacter` (`GameplayStatics.GetPlayerCharacter` 0)))
        (`/Game/ThirdPersonCPP/Blueprints/ThirdPersonCharacter.StopWater` _asthird_person_character_4)
        (bind _asfake_up_game_instance_base_4 (cast `FakeUpGameInstanceBase` (`GameplayStatics.GetGameInstance`)))
        (set `FakeUpGameInstanceBase.AmbientWater` false _asfake_up_game_instance_base_4)))))

(event `self.Box.OnComponentEndOverlap`
  (params (OverlappedComponent :type "PrimitiveComponent Object Reference") (OtherActor :type "Actor Object Reference") (OtherComp :type "PrimitiveComponent Object Reference") (OtherBodyIndex :type Integer))
  (if (== OtherActor (`GameplayStatics.GetPlayerCharacter` 0))
    (bind _asthird_person_character (cast `/Game/ThirdPersonCPP/Blueprints/ThirdPersonCharacter` (`GameplayStatics.GetPlayerCharacter` 0)))
    (`/Game/ThirdPersonCPP/Blueprints/ThirdPersonCharacter.StopForest` _asthird_person_character)
    (`/Game/ThirdPersonCPP/Blueprints/ThirdPersonCharacter.StopWater` _asthird_person_character)
    (bind _asfake_up_game_instance_base (cast `FakeUpGameInstanceBase` (`GameplayStatics.GetGameInstance`)))
    (set `FakeUpGameInstanceBase.AmbientWater` false _asfake_up_game_instance_base)
    (set `FakeUpGameInstanceBase.AmbientForest` false _asfake_up_game_instance_base)))

(fn `UserConstructionScript`)