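; Interactable chest that the player unlocks with a directional lockpick sequence to reach its contents.
; Interacting while locked pauses the game and shows a panel, where each input is prefix-checked against the stored sequence, filling arrow slots or resetting on a mistake.
; A full match keeps it unlocked, plays the open animation and shows the container widget.
; Pause input or leaving the overlap restores game control and closes an open lid.
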(event `self.ReceiveBeginPlay`
  (bind _slatebrush (make `SlateBrush` (104.0 104.0) (struct) (struct :`SpecifiedColor` (struct :`R` 1.0 :`G` 1.0 :`B` 1.0 :`A` 1.0) :`ColorUseRule` "UseColor_Specified") "/Game/Widgets/ClosedContainer/strzałki/góra.góra"))
  (bind _slatebrush_2 (make `SlateBrush` (104.0 104.0) (struct) (struct :`SpecifiedColor` (struct :`R` 1.0 :`G` 1.0 :`B` 1.0 :`A` 1.0) :`ColorUseRule` "UseColor_Specified") "/Game/Widgets/ClosedContainer/strzałki/prawo.prawo"))
  (bind _slatebrush_3 (make `SlateBrush` (104.0 104.0) (struct) (struct :`SpecifiedColor` (struct :`R` 1.0 :`G` 1.0 :`B` 1.0 :`A` 1.0) :`ColorUseRule` "UseColor_Specified") "/Game/Widgets/ClosedContainer/strzałki/dół.dół"))
  (bind _slatebrush_4 (make `SlateBrush` (104.0 104.0) (struct) (struct :`SpecifiedColor` (struct :`R` 1.0 :`G` 1.0 :`B` 1.0 :`A` 1.0) :`ColorUseRule` "UseColor_Specified") "/Game/Widgets/ClosedContainer/strzałki/lewo.lewo"))
  (`/Game/Blueprints/Interactable/BP_Interactable.Init` (`self.BP_Interactable`) (`self.TriggerBox`) "Naciśnij {0} aby otworzyć")
  ;[1 1 1] Znalezienie gracza
  (set `self.Player` (`GameplayStatics.GetPlayerCharacter` 0))
  ;[1 1 1] Set'owanie obrazkow do odpowiednich znakow
  (set `self.ZnakPolnoc` _slatebrush)
  (set `self.ZnakWschod` _slatebrush_2)
  (set `self.ZnakPoludnie` _slatebrush_3)
  (set `self.ZnakZachod` _slatebrush_4)
  (set `self.DirectionImages` (`|MakeArray` _slatebrush _slatebrush_2 _slatebrush_3 _slatebrush_4)))

(event `self.BP_Interactable.ShouldShowInteract`
  (set `/Game/Blueprints/Interactable/BP_Interactable.Interactable` (not (`self.isOpen`)) (`self.BP_Interactable`)))

(event `self.BP_Interactable.Interacted`
  (if (`self.CzySkrzyniaOtworzona`)
    (`self.OpenUnlockedChest`)
    (else
      (`self.OpenUnlockingView`))))

(event `OpenUnlockingView`
  (set `self.Otwieranie` true)
  ;[1 1 1] Włączenie widget'a panelu otwierania skrzyni
  (`/Engine/EditorBlueprintResources/StandardMacros.IsValid` (`self.PanelOtwierania`)
    (:`Is Valid`
      _)
    (:`Is Not Valid`
      (bind _returnvalue (`|CreateWidget` "/Game/Widgets/ClosedContainer/PanelOtwieraniaSkrzyni.PanelOtwieraniaSkrzyni_C" (`GameplayStatics.GetPlayerController` 0)))
      (bind _output_get (set `self.PanelOtwierania` _returnvalue))))
  (`UserWidget.AddToViewport` _output_get 0)
  ;[1 1 1] Pauza gry, brak mozliwosci poruzania sie postacia
  (`GameplayStatics.SetGamePaused` true)
  (`self.SetHudVisible` false)
  ;[1 1 1] Dodanie kontroli przycisków
  (`self.EnableInput` (`GameplayStatics.GetPlayerController` 0)))

(event `SetHudVisible`
  (params (Visible :type Boolean))
  (bind _asbp_hud (cast `/Game/Combat/Ui/BP_Hud` (`PlayerController.GetHUD` (`GameplayStatics.GetPlayerController` 0))))
  (`/Game/Combat/Ui/BP_Hud.SetHudVisible` _asbp_hud Visible))

(event `InputAction|PauseMenu` :paused true
  (params (Key :type "Key Structure"))
  ;[1 1 1] Wyjscie z interakcji ze skrzynia
  (:`Pressed`
    (`self.Close`)))

(event `self.ReceiveActorEndOverlap`
  (params (OtherActor :type "Actor Object Reference"))
  ;[1 1 1] Odejscie od skrzyni (brak możliwosci interakcja)
  (if (== OtherActor (`self.Player`))
    (`self.Close`)))

(event `Close`
  ;[1 1 1] Usuniecie kontroli przycisków
  (`self.SetHudVisible` true)
  (`self.DisableInput` (`GameplayStatics.GetPlayerController` 0))
  ;[1 1 1] Czyszczenie tablicy i bool'a
  (set `self.Otwieranie` false)
  (`KismetArrayLibrary.Array_Clear` (`self.SekwencjaGracza`))
  ;[1 1 1] Wyłączenie widget'a panelu otwierania skrzyni
  (bind _foundwidgets (`WidgetBlueprintLibrary.GetAllWidgetsOfClass` "/Game/Widgets/ClosedContainer/PanelOtwieraniaSkrzyni.PanelOtwieraniaSkrzyni_C"))
  (if (!= (`KismetArrayLibrary.Array_Length` _foundwidgets) 0)
    (`self.ClearSlots`)
    (`Widget.RemoveFromParent` (`|GetArrayItem` _foundwidgets)))
  (bind _foundwidgets_2 (`WidgetBlueprintLibrary.GetAllWidgetsOfClass` "/Game/Widgets/Container/ContainerMain.ContainerMain_C"))
  (if (!= (`KismetArrayLibrary.Array_Length` _foundwidgets_2) 0)
    (bind _output (`|GetArrayItem` _foundwidgets_2))
    (set `self.content` (`/Game/Widgets/Container/ContainerMain.Content` _output))
    (`Widget.RemoveFromParent` _output))
  (`WidgetBlueprintLibrary.SetInputMode_GameOnly` (`GameplayStatics.GetPlayerController` 0))
  (set `self.iscontentset` false)
  ;[1 1 1] Porwót do sterowania postacia
  (`GameplayStatics.SetGamePaused` false)
  (`WidgetBlueprintLibrary.SetInputMode_GameOnly` (`GameplayStatics.GetPlayerController` 0))
  (if (`self.isOpen`)
    (`SkeletalMeshComponent.PlayAnimation` (`self.Skszynia`) "/Game/Blueprints/Containers/SM_Skszynia/SM_Skszynia_zamykanie.SM_Skszynia_zamykanie" false)
    (set `self.isOpen` false)))

(event `InputAction|LockPickUp` :paused true
  (params (Key :type "Key Structure"))
  (:`Pressed`
    (set `self.LastDirection` 0)
    (if (`self.Otwieranie`) :!label _label
      (`KismetArrayLibrary.Array_Add` (`self.SekwencjaGracza`) (`self.LastDirection`))
      (bind _result (`self.CompareSequence` (`self.Sekwencja`) (`self.SekwencjaGracza`)))
      (if _result
        (if (== (`KismetArrayLibrary.Array_Length` (`self.Sekwencja`)) (`KismetArrayLibrary.Array_Length` (`self.SekwencjaGracza`)))
          (set `self.CzySkrzyniaOtworzona` true)
          (`Widget.RemoveFromParent` (`self.PanelOtwierania`))
          (`self.ClearSequence`)
          (`self.OpenUnlockedChest`)
          (`GameplayStatics.SetGamePaused` false)
          (else
            (for (_array_element _array_index) (`self.SekwencjaGracza`)
              (`Image.SetBrush` (`|GetArrayItem` (`/Game/Widgets/ClosedContainer/PanelOtwieraniaSkrzyni.Slots` (`self.PanelOtwierania`)) _array_index) (`|GetArrayItem` (`self.DirectionImages`) _array_element)))))
        (else
          (`self.ClearSequence`))))))

(event `InputAction|LockPickRight` :paused true
  (params (Key :type "Key Structure"))
  (:`Pressed`
    (set `self.LastDirection` 1)
    (goto _label)))

(event `InputAction|LockPickDown` :paused true
  (params (Key :type "Key Structure"))
  (:`Pressed`
    (set `self.LastDirection` 2)
    (goto _label)))

(event `InputAction|LockPickLeft` :paused true
  (params (Key :type "Key Structure"))
  (:`Pressed`
    (set `self.LastDirection` 3)
    (goto _label)))

(event `ClearSequence`
  (`self.ClearSlots`)
  (set `self.SekwencjaGracza` (`|MakeArray`)))

(event `OpenUnlockedChest`
  (`self.SetHudVisible` true)
  (`/Engine/EditorBlueprintResources/StandardMacros.IsValid` (`self.SkrzyniaMenu`)
    (:`Is Valid`
      _)
    (:`Is Not Valid`
      (bind _returnvalue (`|CreateWidget` "/Game/Widgets/Container/ContainerMain.ContainerMain_C" (`GameplayStatics.GetPlayerController` 0)))
      (set `self.SkrzyniaMenu` _returnvalue)))
  (if (not (`self.iscontentset`))
    (set `/Game/Widgets/Container/ContainerMain.Content` (`self.content`) (`self.SkrzyniaMenu`))
    (set `self.iscontentset` true))
  (`UserWidget.AddToViewport` (`self.SkrzyniaMenu`) 0)
  (`WidgetBlueprintLibrary.SetInputMode_GameAndUIEx` (`GameplayStatics.GetPlayerController` 0) (`self.SkrzyniaMenu`) "LockAlways")
  (if (not (`self.isOpen`))
    (`SkeletalMeshComponent.PlayAnimation` (`self.Skszynia`) "/Game/Blueprints/Containers/SM_Skszynia/SM_Skszynia_otwieranie_Anim.SM_Skszynia_otwieranie_Anim" false)
    (set `self.isOpen` true)
    (`self.EnableInput` (`GameplayStatics.GetPlayerController` 0))))

(fn `ClearSlots`
  (bind _panelotwierania (`self.PanelOtwierania`))
  (`/Engine/EditorBlueprintResources/StandardMacros.IsValid` _panelotwierania
    (:`Is Valid`
      (for _array_element (`/Game/Widgets/ClosedContainer/PanelOtwieraniaSkrzyni.Slots` _panelotwierania)
        (`Image.SetBrush` _array_element (make `SlateBrush` (104.0 104.0) (struct) (struct :`SpecifiedColor` (struct :`R` 1.0 :`G` 1.0 :`B` 1.0 :`A` 1.0) :`ColorUseRule` "UseColor_Specified") "/Game/Widgets/ClosedContainer/strzałki/PustySlot.PustySlot"))))))

(fn `CompareSequence`
  (params (full :type "Array of Integer") (part :type "Array of Integer"))
  (returns (result :type Boolean))
  (for (_array_element _array_index) part
    (if (!= (`|GetArrayItem` full _array_index) _array_element)
      (return false)))
  (return true))

(fn `UserConstructionScript`)