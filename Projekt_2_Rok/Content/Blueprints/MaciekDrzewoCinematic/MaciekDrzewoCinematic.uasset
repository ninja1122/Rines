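; One-time Level 1 cinematic of Maciek, triggered by Play and gated by a GameInstance flag.
; It locks input, hides the HUD and blends to a camera that pans through two timelines.
; In parallel, MaciekRuch uses timelines to move Maciek along a hardcoded offset, turn him around and bring him back.
; After the pans, the view blends to Maciek, control and HUD return, the flag is set and his conversation starts.
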(event `Play`
  (bind _returnvalue (`GameplayStatics.GetPlayerController` 0))
  (bind _camera (`self.Camera`))
  (bind (_returnvalue_roll _returnvalue_pitch _returnvalue_yaw) (`KismetMathLibrary.BreakRotator` (`self.K2_GetActorRotation` _camera)))
  (bind (_returnvalue_roll_2 _returnvalue_pitch_2 _returnvalue_yaw_2) (`KismetMathLibrary.BreakRotator` (`self.K2_GetActorRotation` _camera)))
  (bind _asfake_up_game_instance_base (cast `FakeUpGameInstanceBase` (`GameplayStatics.GetGameInstance`)))
  (if (not (`FakeUpGameInstanceBase.Lvl1MaciejDrzewoCinematic` _asfake_up_game_instance_base))
    (`WidgetBlueprintLibrary.SetInputMode_UIOnlyEx` (`GameplayStatics.GetPlayerController` 0) null)
    (`PlayerController.SetCinematicMode` _returnvalue true false true true true)
    (bind _asbp_hud (cast `/Game/Combat/Ui/BP_Hud` (`PlayerController.GetHUD` _returnvalue)))
    (`/Game/Combat/Ui/BP_Hud.SetHudVisible` _asbp_hud false)
    (`PlayerController.SetViewTargetWithBlend` (`GameplayStatics.GetPlayerController` 0) _camera 1.8 "VTBlend_EaseInOut" 3.0 false)
    (`KismetSystemLibrary.Delay` 1.8)
    (`self.K2_SetActorRotation` (`self.Maciek`) (`self.NewVar_0`) true)
    (`SkeletalMeshComponent.PlayAnimation` (`/Game/Blueprints/DialogueNPCs/NewDialogueNPC/Maciek/NPC_Maciek.SkeletalMesh` (`self.Maciek`)) "/Game/Mesh/Postacie/SM_wiesniaczka/babka_chud_Anim.babka_chud_Anim" true)
    (`self.MaciekRuch`)
    (bind (_direction _x) (`Timeline|RotationTimeline`)
      (:`Update`
        (`self.K2_SetActorRotation` _camera (`KismetMathLibrary.MakeRotator` _returnvalue_roll (+ (* (/ _x 50.0) -1.0) _returnvalue_pitch) (+ (* (/ _x 50.0) -1.0) _returnvalue_yaw)) false))
      (:`Finished`
        (`KismetSystemLibrary.Delay` 1.75)
        (bind (_direction_2 _x_2) (`Timeline|Timeline_0` :!via `PlayFromStart`)
          (:`Update`
            (`self.K2_SetActorRotation` _camera (`KismetMathLibrary.MakeRotator` _returnvalue_roll_2 (+ (* (/ _x_2 20.0) -1.0) _returnvalue_pitch_2) (+ (/ _x_2 30.0) _returnvalue_yaw_2)) false))
          (:`Finished`
            (`KismetSystemLibrary.Delay` 1.0)
            (`PlayerController.SetViewTargetWithBlend` (`GameplayStatics.GetPlayerController` 0) (`self.Maciek`) 3.0 "VTBlend_EaseInOut" 3.0 false)
            (`KismetSystemLibrary.Delay` 3.0)
            (`WidgetBlueprintLibrary.SetInputMode_GameOnly` (`GameplayStatics.GetPlayerController` 0))
            (`PlayerController.SetCinematicMode` (`GameplayStatics.GetPlayerController` 0) false false true true true)
            (`/Game/Combat/Ui/BP_Hud.SetHudVisible` _asbp_hud true)
            (bind _asfake_up_game_instance_base_2 (cast `FakeUpGameInstanceBase` (`GameplayStatics.GetGameInstance`)))
            (set `FakeUpGameInstanceBase.Lvl1MaciejDrzewoCinematic` true _asfake_up_game_instance_base_2)
            (`/Game/Blueprints/DialogueNPCs/NewDialogueNPC/Maciek/NPC_Maciek.PlayConversation1` (`self.Maciek`))))))))

(event `MaciekRuch`
  (bind _temptransform (`self.TempTransform`))
  (bind _temptransform_2 (`self.TempTransform`))
  (bind _temptransform_3 (`self.TempTransform`))
  (set `self.TempTransform` (`self.GetTransform` (`self.Maciek`)))
  ;[1 1 1] Comment
  ;;[1 1 1] 13s
  (bind (_direction _x) (`Timeline|TMaciek` :!via `PlayFromStart`)
    (:`Update`
      (`self.K2_SetActorTransform` (`self.Maciek`) (`KismetMathLibrary.MakeTransform` (`KismetMathLibrary.MakeVector` (- (.x (.location _temptransform_3)) (* _x 1261.0)) (+ (.y (.location _temptransform_3)) (* _x 3499.0)) (- (.z (.location _temptransform_3)) (* _x 4.0))) (.rotation _temptransform_3) (.scale _temptransform_3)) false false))
    (:`Finished`
      (`SkeletalMeshComponent.PlayAnimation` (`/Game/Blueprints/DialogueNPCs/NewDialogueNPC/Maciek/NPC_Maciek.SkeletalMesh` (`self.Maciek`)) "/Game/Mesh/Postacie/SM_wiesniaczka/idle_Anim.idle_Anim" true)
      ;[1 1 1] 1,75s
      (`KismetSystemLibrary.Delay` 1.0)
      (`SkeletalMeshComponent.PlayAnimation` (`/Game/Blueprints/DialogueNPCs/NewDialogueNPC/Maciek/NPC_Maciek.SkeletalMesh` (`self.Maciek`)) "/Game/Mesh/Postacie/SM_wiesniaczka/babka_chud_Anim.babka_chud_Anim" true)
      (set `self.TempTransform` (`self.GetTransform` (`self.Maciek`)))
      (`KismetSystemLibrary.Delay` 0.0)
      (bind (_direction_2 _x_2) (`Timeline|Timeline_2` :!via `PlayFromStart`)
        (:`Update`
          (`self.K2_SetActorTransform` (`self.Maciek`) (`KismetMathLibrary.MakeTransform` (.location _temptransform) (`KismetMathLibrary.MakeRotator` (.roll (.rotation _temptransform)) (.pitch (.rotation _temptransform)) (+ (.yaw (.rotation _temptransform)) (* _x_2 180.0))) (.scale _temptransform)) false false))
        (:`Finished`
          ;[1 1 1] 12s
          (set `self.TempTransform` (`self.GetTransform` (`self.Maciek`)))
          (bind (_direction_3 _x_3) (`Timeline|Timeline_1` :!via `PlayFromStart`)
            (:`Update`
              (`self.K2_SetActorTransform` (`self.Maciek`) (`KismetMathLibrary.MakeTransform` (`KismetMathLibrary.MakeVector` (+ (.x (.location _temptransform_2)) (* _x_3 1261.0)) (- (.y (.location _temptransform_2)) (* _x_3 3499.0)) (+ (.z (.location _temptransform_2)) (* _x_3 4.0))) (.rotation _temptransform_2) (.scale _temptransform_2)) false false))
            (:`Finished`
              (`SkeletalMeshComponent.PlayAnimation` (`/Game/Blueprints/DialogueNPCs/NewDialogueNPC/Maciek/NPC_Maciek.SkeletalMesh` (`self.Maciek`)) "/Game/Mesh/Postacie/SM_wiesniaczka/idle_Anim.idle_Anim" true))))))))

(fn `UserConstructionScript`)