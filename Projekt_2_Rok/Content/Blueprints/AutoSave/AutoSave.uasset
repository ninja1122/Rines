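; Autosave trigger volume that saves the game when the player character overlaps its box.
; The overlap calls SaveGame on the player's SaveGamePlayerComponent using the "Autosave" slot name.
; An autosave notification widget, created on first use and reused afterwards, is added to the viewport before saving and removed after a short delay.
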(event `self.Box.OnComponentBeginOverlap`
  (params (OverlappedComponent :type "PrimitiveComponent Object Reference") (OtherActor :type "Actor Object Reference") (OtherComp :type "PrimitiveComponent Object Reference") (OtherBodyIndex :type Integer) (bFromSweep :type Boolean) (SweepResult :type "HitResult Structure (by ref)"))
  (bind _returnvalue (`GameplayStatics.GetPlayerCharacter` 0))
  (if (== OtherActor _returnvalue)
    (if (`self.DoOnce`)
      (`/Engine/EditorBlueprintResources/StandardMacros.DoOnce` false
        (:`Completed`
          _)))
    (`/Engine/EditorBlueprintResources/StandardMacros.IsValid` (stale _returnvalue_2)
      (:`Is Valid`
        _)
      (:`Is Not Valid`
        (bind _returnvalue_2 (`|CreateWidget` "/Game/Widgets/Autosave/AutosaveWidget.AutosaveWidget_C" (`GameplayStatics.GetPlayerController` 0)))))
    (`UserWidget.AddToViewport` _returnvalue_2 0)
    (`SaveGamePlayerComponent.SaveGame` (`self.GetComponentByClass` _returnvalue "/Script/Projekt_2_Rok.SaveGamePlayerComponent") "Autosave")
    (`KismetSystemLibrary.Delay` 5.0)
    (`Widget.RemoveFromParent` _returnvalue_2)))

(fn `UserConstructionScript`)