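; Honey (Miod) inventory item that heals the player when used.
; On interact, outside the Intro level, it finds the BP_Unit component on the player pawn and heals it by a fifth of maximum health, without resurrecting.
; Each successful use decrements the stack quantity, and the last one removes the item from the inventory.
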(event `self.ItemInteract`
  (bind _returnvalue (`self.GetComponentByClass` (`GameplayStatics.GetPlayerPawn` 0) "/Game/Combat/Blueprints/BP_Unit.BP_Unit_C"))
  (bind (_health_current _health_maximum) (break `/Game/Combat/Blueprints/BP_UnitHealth` (`/Game/Combat/Blueprints/BP_Unit.health` _returnvalue)))
  (bind _returnvalue_2 (`GameplayStatics.GetCurrentLevelName` true))
  (if (not (`KismetStringLibrary.EqualEqual_StrStr` _returnvalue_2 "Intro"))
    (`/Engine/EditorBlueprintResources/StandardMacros.IsValid` _returnvalue
      (:`Is Valid`
        (`/Game/Combat/Blueprints/BP_Unit.Heal` _returnvalue (* _health_maximum 0.2) false)
        (if (> (`self.Quantity`) 1)
          (set `self.Quantity` (- (`self.Quantity`) 1))
          (else
            (`self.RemoveFromInvectory`)))))))

(fn `UserConstructionScript`)