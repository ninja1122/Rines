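; Potion inventory item that heals the player when used.
; ItemInteract finds the BP_Unit component on the first player's pawn and heals it by about a third of maximum health, without resurrection.
; Each use lowers the stack quantity, and using the last one removes the item from the inventory.
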(event `self.ItemInteract`
  (bind _returnvalue (`self.GetComponentByClass` (`GameplayStatics.GetPlayerPawn` 0) "/Game/Combat/Blueprints/BP_Unit.BP_Unit_C"))
  (bind (_health_current _health_maximum) (break `/Game/Combat/Blueprints/BP_UnitHealth` (`/Game/Combat/Blueprints/BP_Unit.health` _returnvalue)))
  (`/Engine/EditorBlueprintResources/StandardMacros.IsValid` _returnvalue
    (:`Is Valid`
      (`/Game/Combat/Blueprints/BP_Unit.Heal` _returnvalue (* _health_maximum 0.33) false)
      (if (> (`self.Quantity`) 1)
        (set `self.Quantity` (- (`self.Quantity`) 1))
        (else
          (`self.RemoveFromInvectory`))))))

(fn `UserConstructionScript`
  (`parent.UserConstructionScript`))