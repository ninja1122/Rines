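; SpellBase is a base pickup actor that grants a spell to the player through the inventory.
; On BeginPlay it binds to the pickup added and removed delegates, then adds or removes its SpellClass in the player pawn's BP_SpellManager spell list.
; The construction script builds its display name from a Polish "Zaklęcie:" (Spell) label and the spell class's default Name.
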(event `self.ReceiveBeginPlay`
  (`parent.ReceiveBeginPlay`)
  (add `self.pickupAddedDelegate` (delegate `PickedUp`))
  (add `self.pickupRemovedDelegate` (delegate `Removed`)))

(event `PickedUp` :!signature `self.pickupAddedDelegate`
  (params (Pickup :type "PickupableActor Object Reference"))
  (bind _returnvalue (`self.GetComponentByClass` (`GameplayStatics.GetPlayerPawn` 0) "/Game/Combat/SpellSystem/BP_SpellManager.BP_SpellManager_C"))
  (bind _newparam (`/Game/Combat/SpellSystem/BP_SpellManager.GetSpells` _returnvalue))
  (`KismetArrayLibrary.Array_AddUnique` _newparam (`self.SpellClass`))
  (`/Game/Combat/SpellSystem/BP_SpellManager.SetSpells` _returnvalue _newparam))

(event `Removed` :!signature `self.pickupRemovedDelegate`
  (params (Pickup :type "PickupableActor Object Reference"))
  (bind _returnvalue (`self.GetComponentByClass` (`GameplayStatics.GetPlayerPawn` 0) "/Game/Combat/SpellSystem/BP_SpellManager.BP_SpellManager_C"))
  (bind _newparam (`/Game/Combat/SpellSystem/BP_SpellManager.GetSpells` _returnvalue))
  (`KismetArrayLibrary.Array_RemoveItem` _newparam (`self.SpellClass`))
  (`/Game/Combat/SpellSystem/BP_SpellManager.SetSpells` _returnvalue _newparam))

(fn `UserConstructionScript`
  (`parent.UserConstructionScript`)
  (set `self.NameShow` (`KismetStringLibrary.Concat_StrStr` "Zaklęcie: " (`KismetTextLibrary.Conv_TextToString` (`.name` (defaults `/Game/Blueprints/Inventory/SpellBase` (`self.SpellClass`)))))))