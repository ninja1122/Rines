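; Mapa is an inventory item Blueprint, named as a map, that shows a full-screen image when interacted with.
; ItemInteract creates a Wiadomosc widget for the first player controller and reuses it while it remains valid.
; It sets that widget's image to a fixed 1920x1080 brush and adds it to the viewport.
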(event `self.ItemInteract`
  (`/Engine/EditorBlueprintResources/StandardMacros.IsValid` (stale _returnvalue)
    (:`Is Valid`
      _)
    (:`Is Not Valid`
      (bind _returnvalue (`|CreateWidget` "/Game/Widgets/Wiadomosc/Wiadomosc.Wiadomosc_C" (`GameplayStatics.GetPlayerController` 0)))))
  (`Image.SetBrush` (`/Game/Widgets/Wiadomosc/Wiadomosc.Image_0` _returnvalue) (make `SlateBrush` (1920.0 1080.0) (struct) (struct :`SpecifiedColor` (struct :`R` 1.0 :`G` 1.0 :`B` 1.0 :`A` 1.0) :`ColorUseRule` "UseColor_Specified") "/Game/Widgets/Trader/2d/3.3"))
  (`UserWidget.AddToViewport` _returnvalue 1))

(fn `UserConstructionScript`
  (`parent.UserConstructionScript`))